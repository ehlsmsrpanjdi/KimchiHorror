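; BP_Illusion is an entity Blueprint that detects fast mouse movement and currently only prints a debug "Hello" in response.
; BeginPlay caches the first player controller and its cursor position.
; Each Tick measures the screen-space distance from the previous cursor position, fires the print when it exceeds a fixed threshold, then stores the new position.
; The overlap event and construction script are empty.
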(event `self.ReceiveBeginPlay`
  (bind _returnvalue (`GameplayStatics.GetPlayerController` 0))
  (bind (_locationx _locationy) (`PlayerController.GetMousePosition` _returnvalue))
  (set `self.PlayerMousePos` (`KismetMathLibrary.MakeVector2D` _locationx _locationy))
  (set `self.Player` _returnvalue))

(event `self.ReceiveTick`
  (params (DeltaSeconds :type "Float (single-precision)"))
  (bind (_locationx _locationy) (`PlayerController.GetMousePosition` (`self.Player`)))
  (bind _returnvalue (`KismetMathLibrary.MakeVector2D` _locationx _locationy))
  (if (< 100.0 (`KismetMathLibrary.Distance2D` _returnvalue (`self.PlayerMousePos`)))
    (`KismetSystemLibrary.PrintString` "Hello"))
  (set `self.PlayerMousePos` _returnvalue))

(fn `UserConstructionScript`)