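; Spawner actor that creates a single BP_Illusion once it has line of sight to the player.
; BeginPlay caches the player pawn, then each Tick runs an object line trace from the spawner to the player until it hits BP_MainPlayer.
; It then spawns the illusion at its Arrow component's location and rotation and sets IsSpawn so it fires only once.
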(event `self.ReceiveBeginPlay`
  (set `self.Player` (`GameplayStatics.GetPlayerPawn` 0)))

(event `self.ReceiveTick`
  (params (DeltaSeconds :type "Float (single-precision)"))
  (bind _arrow (`self.Arrow`))
  (if (not (`self.IsSpawn`))
    (bind _outhit (`KismetSystemLibrary.LineTraceSingleForObjects` :`Start` (`self.K2_GetActorLocation`) :`End` (`self.K2_GetActorLocation` (`self.Player`)) :`ObjectTypes` (`self.Object Types`) :`DrawDebugType` "ForOneFrame"))
    (cast `/Game/Level/Stage_1Element/BP_MainPlayer` (`.HitActor` (`GameplayStatics.BreakHitResult` _outhit)))
    (`|SpawnActorFromClass` "/Game/BP/BP_Entity/Illusion/BP_Illusion.BP_Illusion_C" (`KismetMathLibrary.MakeTransform` (`SceneComponent.K2_GetComponentLocation` _arrow) (`SceneComponent.K2_GetComponentRotation` _arrow)) "Undefined" "MultiplyWithRoot" null null)
    (set `self.IsSpawn` true)))

(fn `UserConstructionScript`)