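; BP_TopFloor is a top floor actor with left and right lights whose blinking can be switched on and off.
; On BeginPlay it creates one dynamic instance of MT_Light and assigns it to both LLight and RLight.
; OnBlink and OffBlink set that shared material's IsBlink scalar parameter to 1 or 0, so both lights change together.
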(event `self.ReceiveBeginPlay`
  (bind _returnvalue (`KismetMaterialLibrary.CreateDynamicMaterialInstance` "/Game/CustomMT/MT_Light.MT_Light"))
  (bind _output_get (set `self.BlinkMT` _returnvalue))
  (`PrimitiveComponent.SetMaterial` (`self.L_Light`) 0 _output_get)
  (`PrimitiveComponent.SetMaterial` (`self.R_Light`) 0 _output_get))

(event `OnBlink`
  (`MaterialInstanceDynamic.SetScalarParameterValue` (`self.BlinkMT`) "IsBlink" 1.0))

(event `OffBlink`
  (`MaterialInstanceDynamic.SetScalarParameterValue` (`self.BlinkMT`) "IsBlink" 0.0))

(fn `UserConstructionScript`)