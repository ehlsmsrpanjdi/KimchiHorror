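; Base interactable door that either swings open or, on its matching game day with its quest complete, acts as a story transition.
; The transition runs a sequence or loads DoorLevel, optionally advancing DayCount through the game instance.
; Otherwise, timelines swing it away from the player or entity using a forward-vector dot product, then auto-close after a delay.
; Forced opening stays open; CloseDoor shuts it and disables CanOpen.
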(event `InteractionInterface.OnInteract`
  (params (Interactor :type "Actor Object Reference"))
  (bind _isadddaycount (`self.IsAddDayCount`))
  (bind _doorlevel (`self.DoorLevel`))
  (bind _asbp_game_instance (cast `/Game/BP/BP_GameInstance` (`GameplayStatics.GetGameInstance`)))
  (if (== (`C_GameInstance.DayCount` _asbp_game_instance) (`self.DoorDayCount`))
    (if (`self.IsQuestComplete`)
      (if (`self.IsSequencer`)
        (if _isadddaycount
          (bind _asbp_game_instance_2 (cast `/Game/BP/BP_GameInstance` (`GameplayStatics.GetGameInstance`)))
          (set `C_GameInstance.DayCount` (+ (`C_GameInstance.DayCount` _asbp_game_instance_2) 1) _asbp_game_instance_2))
        (`/Game/Sequence/BP_SequenceHelper.RunSequence` (`self.As BP Squence Helper`))
        (elif _isadddaycount
          (`/Game/BP/BP_GameInstance.RespawnAddDayCount` _asbp_game_instance _doorlevel)
          (else
            (`GameplayStatics.OpenLevelBySoftObjectPtr` _doorlevel)))))
    (else
      (`self.OpenCloseEvent`))))

(event `self.ReceiveBeginPlay`
  (set `self.Rotation` (`self.K2_GetActorRotation`)))

(event `OpenCloseEvent`
  (bind (_rotation_roll _rotation_pitch _rotation_yaw) (`KismetMathLibrary.BreakRotator` (`self.Rotation`)))
  (bind (_rotation_roll_2 _rotation_pitch_2 _rotation_yaw_2) (`KismetMathLibrary.BreakRotator` (`self.Rotation`)))
  (if (`self.CanOpen`)
    (if (not (`self.IsOpening`))
      (`self.PlaySound` "/Game/Sound/Door/door_open.door_open")
      (set `self.IsOpening` true)
      (if (> (`KismetMathLibrary.Dot_VectorVector` (`self.GetActorForwardVector`) (`self.GetActorForwardVector` (`GameplayStatics.GetPlayerPawn` 0))) 0.0)
        (set `self.doorDirection` -1)
        (bind (_direction _alpha) (`Timeline|타임라인` :!via `PlayFromStart` :!label _label)
          (:`Update`
            (`self.K2_SetActorRotation` (`KismetMathLibrary.MakeRotator` 0.0 0.0 (+ (* _alpha 100.0 (`self.doorDirection`)) _rotation_yaw_2))))
          (:`Finished`
            (`KismetSystemLibrary.Delay` 3.0)
            (`self.PlaySound` "/Game/Sound/Door/door_close3.door_close3")
            (bind (_direction_2 _alpha_2) (`Timeline|타임라인_0` :!via `ReverseFromEnd`)
              (:`Update`
                (`self.K2_SetActorRotation` (`KismetMathLibrary.MakeRotator` 0.0 0.0 (+ (* _alpha_2 100.0 (`self.doorDirection`)) _rotation_yaw))))
              (:`Finished`
                (set `self.IsOpening` false)))))
        (else
          (set `self.doorDirection` 1)
          (goto _label :!via `PlayFromStart`))))))

(event `EntityOpen`
  (params (`타깃` :type "Actor Object Reference"))
  (bind (_rotation_roll _rotation_pitch _rotation_yaw) (`KismetMathLibrary.BreakRotator` (`self.Rotation`)))
  (bind (_rotation_roll_2 _rotation_pitch_2 _rotation_yaw_2) (`KismetMathLibrary.BreakRotator` (`self.Rotation`)))
  (if (not (`self.IsOpening`))
    (`self.PlaySound` "/Game/Sound/Door/door_open.door_open")
    (set `self.IsOpening` true)
    (if (> (`KismetMathLibrary.Dot_VectorVector` (`self.GetActorForwardVector`) (`self.GetActorForwardVector` `타깃`)) 0.0)
      (set `self.doorDirection` -1)
      (bind (_direction _alpha) (`Timeline|타임라인_1` :!via `PlayFromStart` :!label _label_2)
        (:`Update`
          (`self.K2_SetActorRotation` (`KismetMathLibrary.MakeRotator` 0.0 0.0 (+ (* _alpha 100.0 (`self.doorDirection`)) _rotation_yaw))))
        (:`Finished`
          (`KismetSystemLibrary.Delay` 3.0)
          (`self.PlaySound` "/Game/Sound/Door/door_close3.door_close3")
          (bind (_direction_2 _alpha_2) (`Timeline|타임라인_2` :!via `ReverseFromEnd`)
            (:`Update`
              (`self.K2_SetActorRotation` (`KismetMathLibrary.MakeRotator` 0.0 0.0 (+ (* _alpha_2 100.0 (`self.doorDirection`)) _rotation_yaw_2))))
            (:`Finished`
              (set `self.IsOpening` false)))))
      (else
        (set `self.doorDirection` 1)
        (goto _label_2 :!via `PlayFromStart`)))))

(event `OpenForce`
  (bind (_rotation_roll _rotation_pitch _rotation_yaw) (`KismetMathLibrary.BreakRotator` (`self.Rotation`)))
  (if (not (`self.IsOpening`))
    (`self.PlaySound` "/Game/Sound/Door/door_open.door_open")
    (set `self.IsOpening` true)
    (if (> (`KismetMathLibrary.Dot_VectorVector` (`self.GetActorForwardVector`) (`self.GetActorForwardVector`)) 0.0)
      (set `self.doorDirection` 1)
      (bind (_direction _alpha) (`Timeline|타임라인_3` :!via `PlayFromStart` :!label _label_3)
        (:`Update`
          (`self.K2_SetActorRotation` (`KismetMathLibrary.MakeRotator` 0.0 0.0 (+ (* _alpha 100.0 (`self.doorDirection`)) _rotation_yaw)))))
      (else
        (set `self.doorDirection` -1)
        (goto _label_3 :!via `PlayFromStart`)))))

(event `PlaySound`
  (params (NewSound :type "SoundBase Object Reference"))
  (bind _audio (`self.Audio`))
  (`AudioComponent.SetSound` _audio NewSound)
  (`AudioComponent.Play` _audio 0.0))

(event `CloseDoor`
  (bind (_rotation_roll _rotation_pitch _rotation_yaw) (`KismetMathLibrary.BreakRotator` (`self.Rotation`)))
  (`self.PlaySound` "/Game/Sound/Door/door_close3.door_close3")
  (bind (_direction _alpha) (`Timeline|타임라인_4` :!via `ReverseFromEnd`)
    (:`Update`
      (`self.K2_SetActorRotation` (`KismetMathLibrary.MakeRotator` 0.0 0.0 (+ (* _alpha 100.0 (`self.doorDirection`)) _rotation_yaw)))
      (set `self.CanOpen` false))
    (:`Finished`
      (set `self.IsOpening` false))))

(event `InteractionInterface.SetQuestComplete`
  (params (Interactor :type "Actor Object Reference"))
  (set `self.IsQuestComplete` true))

(fn `GetCurrentQuestLineName`
  (params (Interactor :type "Actor Object Reference"))
  (returns (ReturnValue :type Name))
  (return (`self.DoorQuestLine`)))

(fn `IsQuestObject`
  (params (Interactor :type "Actor Object Reference"))
  (returns (ReturnValue :type Boolean))
  (return (`self.IsQuestObj`)))

(fn `UserConstructionScript`)