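; BP_FocusActor is an interactable actor that takes over the player's view and shows an explanation UI.
; Interacting calls View, which switches the view target to itself, moves input from the pawn to the actor and creates a BP_ExplainUI widget.
; Pressing E calls UnView, which restores pawn input and view and removes the widget.
; Its quest query functions report that it is not a quest object.
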(event `View`
  (params (Interactor :type "Actor Object Reference"))
  (bind _returnvalue (`GameplayStatics.GetPlayerController` 0))
  (`PlayerController.SetViewTargetWithBlend` _returnvalue self 0.0 "VTBlend_Linear" 0.0 false)
  (`self.EnableInput` _returnvalue)
  (`self.DisableInput` (`GameplayStatics.GetPlayerPawn` 0) _returnvalue)
  (bind _returnvalue_2 (`|CreateWidget` "/Game/BP/UI/Common/BP_ExplainUI.BP_ExplainUI_C" (`GameplayStatics.GetPlayerController` 0)))
  (bind _output_get (set `self.ExplainUI` _returnvalue_2))
  (`UserWidget.AddToViewport` _output_get 0))

(event `UnView`
  (bind _returnvalue (`GameplayStatics.GetPlayerController` 0))
  (bind _returnvalue_2 (`GameplayStatics.GetPlayerPawn` 0))
  (`self.EnableInput` _returnvalue_2 _returnvalue)
  (`self.DisableInput` _returnvalue)
  (`PlayerController.SetViewTargetWithBlend` _returnvalue _returnvalue_2 0.0 "VTBlend_Linear" 0.0 false)
  (`Widget.RemoveFromParent` (`self.ExplainUI`)))

(event `Key|E`
  (params (Key :type "Key Structure"))
  (:`Pressed`
    (`self.UnView`)))

(event `InteractionInterface.OnInteract`
  (params (Interactor :type "Actor Object Reference"))
  (`self.View` null))

(fn `GetCurrentQuestLineName`
  (params (Interactor :type "Actor Object Reference"))
  (returns (ReturnValue :type Name))
  (return "None"))

(fn `IsQuestObject`
  (params (Interactor :type "Actor Object Reference"))
  (returns (ReturnValue :type Boolean))
  (return false))

(fn `UserConstructionScript`)