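; BP_LastLevelDoor is an interactable door, named for the last level, that opens or closes only on a specific day.
; On interact, it casts the game instance to BP_GameInstance and calls OpenCloseEvent when DayCount equals the door's DoorDayCount.
; Leftover checks for quest completion and day-count increment are unconnected and never run.
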(event `InteractionInterface.OnInteract`
  (params (Interactor :type "Actor Object Reference"))
  (bind _asbp_game_instance (cast `/Game/BP/BP_GameInstance` (`GameplayStatics.GetGameInstance`)))
  (if (== (`C_GameInstance.DayCount` _asbp_game_instance) (`self.DoorDayCount`))
    (`self.OpenCloseEvent`)))

(fn `UserConstructionScript`
  (`parent.UserConstructionScript`))