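; Level-placed trigger actor that advances the player's quest line when the player walks into it.
; Shortly after BeginPlay it teleports itself to its Arrow component's world location.
; When BP_MainPlayer overlaps the Box, it writes its CurrentQuestLine into the player's BP_QuestComponent, destroys itself and prints a quest-update debug message.
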(event `self.ReceiveBeginPlay`
  (`KismetSystemLibrary.Delay` 0.2)
  (`self.K2_SetActorLocation` (`SceneComponent.K2_GetComponentLocation` (`self.Arrow`))))

(event `self.Box.OnComponentBeginOverlap`
  (params (OverlappedComponent :type "PrimitiveComponent Object Reference") (OtherActor :type "Actor Object Reference") (OtherComp :type "PrimitiveComponent Object Reference") (OtherBodyIndex :type Integer) (bFromSweep :type Boolean) (SweepResult :type "HitResult Structure (by ref)"))
  (bind _asbp_main_player (cast `/Game/Level/Stage_1Element/BP_MainPlayer` OtherActor))
  (set `C_QuestComponent.CurrentQuestLine` (`self.Current Quest Line`) (`self.GetComponentByClass` _asbp_main_player "/Game/Level/Stage_1Element/BP_QuestComponent.BP_QuestComponent_C"))
  (`self.K2_DestroyActor`)
  (`KismetSystemLibrary.PrintString` "퀘스트갱신"))

(fn `UserConstructionScript`)