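; Interactable main door that serves as the "GoMainGate" quest object and stages the Stage 1 nurse jump scare.
; Once SetQuestComplete arms it, the next interaction spawns the nurse at a world-space offset from the player, oriented by the Arrow, and clears the flag.
; When the player begins overlapping the Box while the nurse exists, both the nurse and the trigger are destroyed.
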(event `InteractionInterface.OnInteract`
  (params (Interactor :type "Actor Object Reference"))
  (bind (_returnvalue_location _returnvalue_rotation) (`KismetMathLibrary.BreakTransform` (`SceneComponent.K2_GetComponentToWorld` (`self.Arrow`))))
  (if (`self.QuestComplete`)
    (bind _returnvalue (`|SpawnActorFromClass` "/Game/BP/Stage1/Jumps/BP_Stage_1JumpScareNurse.BP_Stage_1JumpScareNurse_C" (`KismetMathLibrary.MakeTransform` (+ (`self.K2_GetActorLocation` (`GameplayStatics.GetPlayerPawn` 0)) (0.0 200.0 0.0)) _returnvalue_rotation) "Undefined" "MultiplyWithRoot" null null))
    (set `self.Nurse` _returnvalue)
    (set `self.QuestComplete` false)))

(event `InteractionInterface.SetQuestComplete`
  (params (Interactor :type "Actor Object Reference"))
  (set `self.QuestComplete` true))

(event `self.Box.OnComponentBeginOverlap`
  (params (OverlappedComponent :type "PrimitiveComponent Object Reference") (OtherActor :type "Actor Object Reference") (OtherComp :type "PrimitiveComponent Object Reference") (OtherBodyIndex :type Integer) (bFromSweep :type Boolean) (SweepResult :type "HitResult Structure (by ref)"))
  (bind _nurse (`self.Nurse`))
  (cast `/Game/Level/Stage_1Element/BP_MainPlayer` OtherActor)
  (if (`KismetSystemLibrary.IsValid` _nurse)
    (`self.K2_DestroyActor` _nurse)
    (`ActorComponent.K2_DestroyComponent` (`self.Box`))))

(fn `GetCurrentQuestLineName`
  (params (Interactor :type "Actor Object Reference"))
  (returns (ReturnValue :type Name))
  (return "GoMainGate"))

(fn `IsQuestObject`
  (params (Interactor :type "Actor Object Reference"))
  (returns (ReturnValue :type Boolean))
  (return true))

(fn `UserConstructionScript`)