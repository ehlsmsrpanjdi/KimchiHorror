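; BP_MoveObstacleBase is a base obstacle Blueprint that moves its static mesh to an Arrow component's position when the player pawn enters its trigger Box.
; The overlap calls MoveEvent, which destroys the Box so it fires only once, then plays a timeline.
; Each update lerps the mesh from its current location toward the Arrow, compounding the timeline alpha, and completion snaps it exactly onto the Arrow.
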(event `self.Box.OnComponentBeginOverlap`
  (params (OverlappedComponent :type "PrimitiveComponent Object Reference") (OtherActor :type "Actor Object Reference") (OtherComp :type "PrimitiveComponent Object Reference") (OtherBodyIndex :type Integer) (bFromSweep :type Boolean) (SweepResult :type "HitResult Structure (by ref)"))
  (if (== OtherActor (`GameplayStatics.GetPlayerPawn` 0))
    (`self.MoveEvent`)))

(event `MoveEvent`
  (bind _returnvalue (`SceneComponent.K2_GetComponentLocation` (`self.Arrow`)))
  (`ActorComponent.K2_DestroyComponent` (`self.Box`))
  (bind (_direction `_새_트랙_0`) (`Timeline|타임라인` :!via `PlayFromStart`)
    (:`Update`
      (`SceneComponent.K2_SetWorldLocation` (`self.StaticMesh`) (`KismetMathLibrary.VLerp` (`SceneComponent.K2_GetComponentLocation` (`self.StaticMesh`)) _returnvalue `_새_트랙_0`) false false))
    (:`Finished`
      (`SceneComponent.K2_SetWorldLocation` (`self.StaticMesh`) _returnvalue false false))))

(fn `UserConstructionScript`)