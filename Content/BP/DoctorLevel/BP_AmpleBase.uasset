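; BP_AmpleBase is the base interactable drug ampoule in the Doctor level, using the player's BP_DoctorLevelComponent to decide what interaction does.
; If a syringe is held and OnAmple is false, it adds the drug, disables input and animates a temporary syringe along two spline points via timeline.
; Without a syringe, an empty-handed player gains the ampoule, notifying its Crate if valid.
; An outline overlay material shows interactability.
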(event `InteractionInterface.OnInteract`
  (params (Interactor :type "Actor Object Reference"))
  (bind _crate (`self.Crate`))
  (bind _returnvalue (`self.GetComponentByClass` (`GameplayStatics.GetPlayerPawn` 0) "/Game/BP/DoctorLevel/BP_DoctorLevelComponent.BP_DoctorLevelComponent_C"))
  (bind _syringe (`/Game/BP/DoctorLevel/BP_DoctorLevelComponent.Syringe` _returnvalue))
  ;[1 1 1] Ample이 들어간 상태?
  (if (`/Game/BP/DoctorLevel/BP_DoctorLevelComponent.OnAmple` _returnvalue)
    (`KismetSystemLibrary.PrintString` "주사기가없거나 약물을 이미 주입함")
    (else
      ;[1 1 1] 주사기 있음?
      (if (`KismetSystemLibrary.IsValid` _syringe)
        ;[1 1 1] Ample안들어갔고 주사기 있음
        (`/Game/BP/DoctorLevel/BP_DoctorLevelComponent.AddDrug` _returnvalue self)
        (`self.SetActorHiddenInGame` _syringe true)
        (`self.DisableInput` (`GameplayStatics.GetPlayerPawn` 0) (`GameplayStatics.GetPlayerController` 0))
        (bind _returnvalue_2 (`|SpawnActorFromClass` "/Game/BP/DoctorLevel/BP_Syringe.BP_Syringe_C" (`KismetMathLibrary.MakeTransform` (`SplineComponent.GetLocationAtSplinePoint` (`self.Spline`) 0 "World") (struct :`Roll` 90.0)) "Undefined" "MultiplyWithRoot" null null))
        (bind (_direction _syringetimeline) (`Timeline|Syringe` :!via `PlayFromStart`)
          (:`Update`
            (`self.K2_SetActorLocation` _returnvalue_2 (`KismetMathLibrary.VLerp` (`SplineComponent.GetLocationAtSplinePoint` (`self.Spline`) 0 "World") (`SplineComponent.GetLocationAtSplinePoint` (`self.Spline`) 1 "World") _syringetimeline) false false))
          (:`Finished`
            (`self.K2_DestroyActor` _returnvalue_2)
            (`self.SetActorHiddenInGame` _syringe false)
            (`self.EnableInput` (`GameplayStatics.GetPlayerPawn` 0) (`GameplayStatics.GetPlayerController` 0))))
        (else
          ;[1 1 1] 앰플 들고있음?
          (if (`KismetSystemLibrary.IsValid` (`/Game/BP/DoctorLevel/BP_DoctorLevelComponent.Ample` _returnvalue))
            (`KismetSystemLibrary.PrintString` "약품 이미 들고있음")
            (else
              (if (`KismetSystemLibrary.IsValid` _crate)
                (`/Game/BP/DoctorLevel/BP_Crate.TakeAmple` _crate (`self.CrateIndex`)))
              ;[1 1 1] 약품얻기
              (`/Game/BP/DoctorLevel/BP_DoctorLevelComponent.GainAmple` _returnvalue self))))))))

(event `InteractionInterface.CanInteract`
  (params (Interactor :type "Actor Object Reference"))
  (`MeshComponent.SetOverlayMaterial` (`self.StaticMesh`) "/Game/BP/Material/MT_OutLine.MT_OutLine"))

(event `InteractionInterface.CanNotInteract`
  (params (Interactor :type "Actor Object Reference"))
  (`MeshComponent.SetOverlayMaterial` (`self.StaticMesh`) null))

(fn `GetCurrentQuestLineName`
  (params (Interactor :type "Actor Object Reference"))
  (returns (ReturnValue :type Name))
  (return "None"))

(fn `IsQuestObject`
  (params (Interactor :type "Actor Object Reference"))
  (returns (ReturnValue :type Boolean))
  (return false))

(fn `UserConstructionScript`)