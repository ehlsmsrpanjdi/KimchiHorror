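; BP_AngryEntity is an interactable entity in the doctor level that the player can inject with an ampoule.
; On interact, if the player's BP_DoctorLevelComponent has OnAmple set, it uses the ampoule and caches the selected drug index.
; SyringeEvent disables input and animates a spawned BP_Syringe between two spline points via a timeline.
; When finished, it destroys the syringe, restores input and calls GoBackEvent for one specific drug.
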(event `InteractionInterface.OnInteract`
  (params (Interactor :type "Actor Object Reference"))
  (bind _returnvalue (`self.GetComponentByClass` (`GameplayStatics.GetPlayerPawn` 0) "/Game/BP/DoctorLevel/BP_DoctorLevelComponent.BP_DoctorLevelComponent_C"))
  ;[1 1 1] 상호작용
  (if (`C_DocLevelComponent.bOnAmple` _returnvalue)
    (`C_DocLevelComponent.UseAmple` _returnvalue)
    (set `self.CachedIndex` (`C_DocLevelComponent.SelectedDrugIndex` _returnvalue))
    (`self.SyringeEvent`)))

(event `SyringeEvent`
  (bind _returnvalue (`SplineComponent.GetLocationAtSplinePoint` (`self.Spline`) 0 "World"))
  ;[1 1 1] 주사바늘놓기
  (`self.DisableInput` (`GameplayStatics.GetPlayerPawn` 0) (`GameplayStatics.GetPlayerController` 0))
  (bind _returnvalue_2 (`|SpawnActorFromClass` "/Game/BP/DoctorLevel/BP_Syringe.BP_Syringe_C" (`KismetMathLibrary.MakeTransform` _returnvalue (`KismetMathLibrary.ComposeRotators` (`KismetMathLibrary.FindLookAtRotation` _returnvalue (`SplineComponent.GetLocationAtSplinePoint` (`self.Spline`) 1 "World")) (struct :`Yaw` -90.0))) "Undefined" "MultiplyWithRoot" null null))
  (bind (_direction _syringetimeline) (`Timeline|타임라인` :!via `PlayFromStart`)
    (:`Update`
      (`self.K2_SetActorLocation` _returnvalue_2 (`KismetMathLibrary.VLerp` (`SplineComponent.GetLocationAtSplinePoint` (`self.Spline`) 0 "World") (`SplineComponent.GetLocationAtSplinePoint` (`self.Spline`) 1 "World") _syringetimeline) false false))
    (:`Finished`
      (`self.K2_DestroyActor` _returnvalue_2)
      (`self.EnableInput` (`GameplayStatics.GetPlayerPawn` 0) (`GameplayStatics.GetPlayerController` 0))
      (if (== (`self.CachedIndex`) 2)
        (`self.GoBackEvent`)))))

(fn `UserConstructionScript`
  (`parent.UserConstructionScript`))