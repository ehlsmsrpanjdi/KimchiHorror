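; BP_DocDoor is an interactable doctor-level door that runs a knock event the player must answer in time.
; Two minutes after BeginPlay, Tick starts polling a cooldown check that triggers the knock sound and turns on a spotlight.
; Interacting during the knock silences it and switches the light off.
; If the sound finishes first, a fail handler prints a debug message and stops further knocks.
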(event `self.ReceiveBeginPlay`
  (`LightComponent.SetIntensity` (`self.SpotLight`) 0.0)
  (`KismetSystemLibrary.Delay` 120.0)
  (set `self.IsWalking` true))

(event `self.ReceiveTick`
  (params (DeltaSeconds :type "Float (single-precision)"))
  (if (`self.IsWalking`)
    (bind _returnvalue (`self.CalculateCoolTime` DeltaSeconds))
    (if _returnvalue
      (`self.DoorOpenEvent`)
      (`LightComponent.SetIntensity` (`self.SpotLight`) 30.0))))

(event `DoorOpenEvent`
  (bind _audiocomponent (`self.AudioComponent`))
  (`AudioComponent.SetSound` _audiocomponent "/Game/Sound/DocLevel/SO_DoorKnock.SO_DoorKnock")
  (`AudioComponent.Play` _audiocomponent 0.0)
  (add `AudioComponent.OnAudioFinished` _audiocomponent (delegate `FailDoorCheck`)))

(event `FailDoorCheck`
  (bind _audiocomponent (`self.AudioComponent`))
  (clear `AudioComponent.OnAudioFinished` _audiocomponent)
  (`AudioComponent.Stop` _audiocomponent)
  (`AudioComponent.SetSound` _audiocomponent null)
  (`KismetSystemLibrary.PrintString` "느조쓰")
  (set `self.IsWalking` false))

(event `InteractionInterface.OnInteract`
  (params (Interactor :type "Actor Object Reference"))
  (bind _audiocomponent (`self.AudioComponent`))
  (if (`AudioComponent.IsPlaying` _audiocomponent)
    (clear `AudioComponent.OnAudioFinished` _audiocomponent)
    (`AudioComponent.Stop` _audiocomponent)
    (`AudioComponent.SetSound` _audiocomponent null)
    (`LightComponent.SetIntensity` (`self.SpotLight`) 0.0)))

(fn `GetCurrentQuestLineName`
  (params (Interactor :type "Actor Object Reference"))
  (returns (ReturnValue :type Name))
  (return "None"))

(fn `IsQuestObject`
  (params (Interactor :type "Actor Object Reference"))
  (returns (ReturnValue :type Boolean))
  (return false))

(fn `UserConstructionScript`)