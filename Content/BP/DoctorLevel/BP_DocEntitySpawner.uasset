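; Spawner for the doctor level that periodically spawns a random entity at a random free point and sends it walking toward a patient.
; BeginPlay sets up the points and widens the entity pool over time, adding angry, then sad entities after successive delays.
; A Delay on Tick paces spawning; each spawn casts to BP_SmileEntity and receives a forward-offset target, the spawner and point index, while no valid point prints a "full" message.
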(event `self.ReceiveBeginPlay`
  (`self.SetupPointPos` 1200.0)
  (`KismetSystemLibrary.Delay` 120.0)
  (`KismetArrayLibrary.Array_Add` (`self.EntityArray`) "/Game/BP/DoctorLevel/BP_AngryEntity.BP_AngryEntity_C")
  (`KismetSystemLibrary.Delay` 120.0)
  (`KismetArrayLibrary.Array_Add` (`self.EntityArray`) "/Game/BP/DoctorLevel/BP_SadEntity.BP_SadEntity_C"))

(event `self.ReceiveTick`
  (params (DeltaSeconds :type "Float (single-precision)"))
  (`KismetSystemLibrary.Delay` 10.0)
  (bind _returnvalue (`self.GetRandomPoint`))
  (if (`KismetSystemLibrary.IsValid` _returnvalue)
    (bind _returnvalue_2 (`self.GetRandomCharacter`))
    (bind (_returnvalue_location _returnvalue_rotation _returnvalue_scale) (`KismetMathLibrary.BreakTransform` (`SceneComponent.K2_GetComponentToWorld` _returnvalue)))
    (bind _returnvalue_3 (`|SpawnActorFromClass` _returnvalue_2 (`KismetMathLibrary.MakeTransform` _returnvalue_location _returnvalue_rotation _returnvalue_scale) "Undefined" "MultiplyWithRoot" null null))
    (bind _asbp_smile_entity (cast `/Game/BP/DoctorLevel/BP_SmileEntity` _returnvalue_3))
    (`/Game/BP/DoctorLevel/BP_SmileEntity.MoveToPatient` _asbp_smile_entity (+ _returnvalue_location (* (`SceneComponent.GetForwardVector` _returnvalue) 800.0)) self (`self.currentSelectedIndex`))
    (else
      (`KismetSystemLibrary.PrintString` "꽉참"))))

(fn `UserConstructionScript`)