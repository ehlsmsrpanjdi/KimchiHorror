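; Patient character for the doctor level that raises medical emergencies the player must treat by syringe before a death timer fires.
; Tick triggers one of four events (eye opening, seizure, fast or slow pulse), binds death and starts the timer; only the pulse events change audio, the others just print.
; Interacting with an ampoule animates a syringe along a spline and checks the cure, unbinding death on success.
; Interface events drive face, head-tilt and body animation.
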(event `self.ISetFaceMove`
  (params (Pose :type "C_FacePoseEnum Enum" :default "Idle") (Mood :type "C_FaceMoodEnum Enum" :default "Normal") (Interval :type "Float (double-precision)"))
  (bind _asbp_entity_face_anim (cast `/Game/BP/Stage1/InteractiveEntity/AnimIns/Face/BP_EntityFaceAnim` (`SkeletalMeshComponent.GetAnimInstance` (`self.Face`)))
    (:`then`
      (`C_AnimBPBase.SetFacePose` _asbp_entity_face_anim Pose Mood Interval))
    (:`CastFailed`
      (`KismetSystemLibrary.PrintString` "FaceMissing"))))

(event `self.ISetHeadTilting`
  (params (DesVector :type "Vector Structure") (RotateSpeed :type "Float (double-precision)"))
  (bind _asbp_male_entity_body_anim (cast `/Game/BP/Stage1/InteractiveEntity/AnimIns/Body/BP_MaleEntityBodyAnim` (`SkeletalMeshComponent.GetAnimInstance` (`self.Mesh`)))
    (:`then`
      (`C_EntityAnimBase.LerfTiltHead` _asbp_male_entity_body_anim DesVector RotateSpeed))
    (:`CastFailed`
      (`KismetSystemLibrary.PrintString` "TiltingMissing"))))

(event `self.ISetBodyMove`
  (params (Move :type "C_EntityMoveEnum Enum" :default "Idle"))
  (bind _asbp_male_entity_body_anim (cast `/Game/BP/Stage1/InteractiveEntity/AnimIns/Body/BP_MaleEntityBodyAnim` (`SkeletalMeshComponent.GetAnimInstance` (`self.Mesh`)))
    (:`then`
      (`C_EntityAnimBase.SetBodyMove` _asbp_male_entity_body_anim Move))
    (:`CastFailed`
      (`KismetSystemLibrary.PrintString` "BodyMissing"))))

(event `OpenEyeEvent`
  (`KismetSystemLibrary.PrintString` "눈뜨기"))

(event `self.ReceiveBeginPlay`
  (bind _heartbeatcomponent (`self.HeartBeatComponent`))
  (`parent.ReceiveBeginPlay`)
  (set `self.MyFace` (`self.Face`))
  (`SceneComponent.K2_AttachToComponent` (`self.Noise`) (`self.Mesh`) "headSocket" "KeepRelative" "KeepRelative" "KeepRelative" true)
  (`AudioComponent.SetSound` _heartbeatcomponent "/Game/Sound/DocLevel/SO_HeartBeat.SO_HeartBeat")
  (`AudioComponent.Play` _heartbeatcomponent 0.0))

(event `SeizureEvent`
  (`KismetSystemLibrary.PrintString` "발작"))

(event `PulseSlowEvent`
  (bind _heartbeatcomponent (`self.HeartBeatComponent`))
  (`AudioComponent.Stop` _heartbeatcomponent)
  (`AudioComponent.SetSound` _heartbeatcomponent "/Game/Sound/DocLevel/SO_HeartBeatSlow.SO_HeartBeatSlow")
  (`AudioComponent.Play` _heartbeatcomponent 0.0)
  (`KismetSystemLibrary.PrintString` "심장느려지기"))

(event `PulseQuickEvent`
  (bind _heartbeatcomponent (`self.HeartBeatComponent`))
  (`AudioComponent.Stop` _heartbeatcomponent)
  (`AudioComponent.SetSound` _heartbeatcomponent "/Game/Sound/DocLevel/SO_HeartBeatFast.SO_HeartBeatFast")
  (`AudioComponent.Play` _heartbeatcomponent 0.0)
  (`KismetSystemLibrary.PrintString` "심장빨라지기"))

(event `self.ReceiveTick`
  (params (DeltaSeconds :type "Float (single-precision)"))
  (bind _returnvalue (`self.OnEvent` DeltaSeconds))
  (if _returnvalue
    (switch `int` (`self.CurrentEventIndex`)
      (:`0`
        (`self.OpenEyeEvent`))
      (:`1`
        (`self.SeizureEvent`))
      (:`2`
        (`self.PulseQuickEvent`))
      (:`3`
        (`self.PulseSlowEvent`)))
    (add `self.OnAction` (delegate `DeadEvent`))
    (`self.DeadTimer`)))

(event `DeadTimer`
  (`KismetSystemLibrary.Delay` 15.0)
  (`self.ActiveAllEvent`))

(event `DeadEvent`
  (`KismetSystemLibrary.PrintString` "환자 사망 및 플레이어 사망"))

(event `InteractionInterface.OnInteract`
  (params (Interactor :type "Actor Object Reference"))
  (bind _returnvalue (`self.GetComponentByClass` (`GameplayStatics.GetPlayerPawn` 0) "/Game/BP/DoctorLevel/BP_DoctorLevelComponent.BP_DoctorLevelComponent_C"))
  (if (`/Game/BP/DoctorLevel/BP_DoctorLevelComponent.OnAmple` _returnvalue)
    (`self.SyringeEvent`)
    (bind _newparam (`/Game/BP/DoctorLevel/BP_DoctorLevelComponent.UseSyringe` _returnvalue))
    (bind _returnvalue_2 (`self.OnCurePatient` _newparam))
    (if _returnvalue_2
      (`KismetSystemLibrary.PrintString` "맞춤")
      (clear `self.OnAction`)
      (else
        (`KismetSystemLibrary.PrintString` "틀림")))))

(event `SyringeEvent`
  (`self.DisableInput` (`GameplayStatics.GetPlayerPawn` 0) (`GameplayStatics.GetPlayerController` 0))
  (bind _returnvalue (`|SpawnActorFromClass` "/Game/BP/DoctorLevel/BP_Syringe.BP_Syringe_C" (`KismetMathLibrary.MakeTransform` (`SplineComponent.GetLocationAtSplinePoint` (`self.Spline`) 0 "World") (struct :`Yaw` 90.0)) "Undefined" "MultiplyWithRoot" null null))
  (bind (_direction _syringetimeline) (`Timeline|Syringe` :!via `PlayFromStart`)
    (:`Update`
      (`self.K2_SetActorLocation` _returnvalue (`KismetMathLibrary.VLerp` (`SplineComponent.GetLocationAtSplinePoint` (`self.Spline`) 0 "World") (`SplineComponent.GetLocationAtSplinePoint` (`self.Spline`) 1 "World") _syringetimeline) false false))
    (:`Finished`
      (`self.K2_DestroyActor` _returnvalue)
      (`self.EnableInput` (`GameplayStatics.GetPlayerPawn` 0) (`GameplayStatics.GetPlayerController` 0)))))

(event `self.CanInteract`
  (params (Interactor :type "Actor Object Reference"))
  (cast `/Game/Level/Stage_1Element/BP_MainPlayer` Interactor)
  (`/Game/BP/UI/Common/Text/BP_InterMassage.OnInteraction` (`self.As BP Inter Massage`) (`self.InteractionMassage`))
  (`C_UIManager.OnUI` (`C_UIManager.GetUIManager`) "/Script/HorrorProtoKimchi.C_InterUI"))

(event `self.CanNotInteract`
  (params (Interactor :type "Actor Object Reference"))
  (`/Game/BP/UI/Common/Text/BP_InterMassage.OffInteraction` (`self.As BP Inter Massage`)))

(fn `UserConstructionScript`
  (`SkinnedMeshComponent.SetLeaderPoseComponent` (`self.Clothes`) (`self.Mesh`) false false)
  (`SkinnedMeshComponent.SetLeaderPoseComponent` (`self.Arms`) (`self.Mesh`) false false)
  (`SkinnedMeshComponent.SetLeaderPoseComponent` (`self.Pants`) (`self.Mesh`) false false)
  (`SkinnedMeshComponent.SetLeaderPoseComponent` (`self.Hair_1`) (`self.Mesh`) false false))