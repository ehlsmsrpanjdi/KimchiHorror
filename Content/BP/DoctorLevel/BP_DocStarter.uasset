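; BP_DocStarter is the timed game-flow controller for the Doctor level, running the round from start to victory.
; On BeginPlay, a chain of Delays clears IsEnd on the patient, crate and entity spawner references, then later on the door.
; After the final delay it sets IsEnd on all four and prints a Korean victory message, with no condition checked.
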(event `self.ReceiveBeginPlay`
  (`KismetSystemLibrary.Delay` 30.0)
  (`KismetSystemLibrary.PrintString` "게임시작")
  (set `C_DocPatient.isEnd` false (`self.Patient`))
  (set `C_Crate.isEnd` false (`self.As BP Crate`))
  (set `C_DocEntitySpawner.isEnd` false (`self.As BP Doc Entity Spawner`))
  (`KismetSystemLibrary.Delay` 120.0)
  (set `C_DoctorDoorKnockObj.isEnd` false (`self.As BP Doc Door`))
  (`KismetSystemLibrary.Delay` 240.0)
  (set `C_DocPatient.isEnd` true (`self.Patient`))
  (set `C_Crate.isEnd` true (`self.As BP Crate`))
  (set `C_DocEntitySpawner.isEnd` true (`self.As BP Doc Entity Spawner`))
  (set `C_DoctorDoorKnockObj.isEnd` true (`self.As BP Doc Door`))
  (`KismetSystemLibrary.PrintString` "승리"))

(fn `UserConstructionScript`)