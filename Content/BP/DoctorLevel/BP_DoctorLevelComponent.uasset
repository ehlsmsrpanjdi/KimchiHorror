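; BP_DoctorLevelComponent tracks the syringe and drug ampoule the player holds in the doctor level.
; GainSyringe spawns a syringe at the owning player's hand, while GainAmple replaces the given ampoule with a fresh copy of its class attached below the hand.
; AddDrug stores the ampoule's drug index when a syringe exists.
; UseSyringe destroys the syringe, resets drug state and returns the stored index.
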(event `self.ReceiveTick`
  (params (DeltaSeconds :type "Float (single-precision)"))
  (if (`KismetSystemLibrary.IsValid` (`self.Syringe`))
    _))

(event `GainSyringe`
  (bind _returnvalue (`self.GetOwner`))
  (bind _returnvalue_2 (`|SpawnActorFromClass` "/Game/BP/DoctorLevel/BP_Syringe.BP_Syringe_C" (`KismetMathLibrary.MakeTransform` (0.0 0.0 0.0) (struct :`Roll` -90.0)) "Undefined" "MultiplyWithRoot" null null))
  (bind _asbp_main_player (cast `/Game/Level/Stage_1Element/BP_MainPlayer` _returnvalue))
  (set `self.Syringe` _returnvalue_2)
  (`Actor.K2_AttachToActor` _returnvalue_2 _returnvalue "None" "KeepRelative" "KeepRelative" "KeepRelative" false)
  (`Actor.K2_SetActorLocation` _returnvalue_2 (`SceneComponent.K2_GetComponentLocation` (`/Game/Level/Stage_1Element/BP_MainPlayer.HandPos` _asbp_main_player)) false false))

(event `AddDrug`
  (params (Ample :type "/Game/BP/DoctorLevel/BP_AmpleBase Object Reference"))
  (if (`KismetSystemLibrary.IsValid` (`self.Syringe`))
    (set `self.DrugIndex` (`/Game/BP/DoctorLevel/BP_AmpleBase.DrugIndex` Ample))
    (set `self.OnAmple` true)))

(event `GainAmple`
  (params (Ample :type "/Game/BP/DoctorLevel/BP_AmpleBase Object Reference"))
  (bind _returnvalue (`|SpawnActorFromClass` (`GameplayStatics.GetObjectClass` Ample) (`KismetMathLibrary.MakeTransform` (0.0 0.0 0.0)) "Undefined" "MultiplyWithRoot" null null))
  (`Actor.K2_DestroyActor` Ample)
  (set `self.Ample` _returnvalue)
  (bind _asbp_main_player (cast `/Game/Level/Stage_1Element/BP_MainPlayer` (`GameplayStatics.GetPlayerPawn` 0)))
  (`Actor.K2_AttachToActor` _returnvalue _asbp_main_player "None" "KeepRelative" "KeepRelative" "KeepRelative" false)
  (`Actor.K2_SetActorLocation` _returnvalue (- (`SceneComponent.K2_GetComponentLocation` (`/Game/Level/Stage_1Element/BP_MainPlayer.HandPos` _asbp_main_player)) (0.0 0.0 30.0)) false false))

(fn `UseSyringe`
  (returns (NewParam :type Integer))
  (`Actor.K2_DestroyActor` (`self.Syringe`))
  (set `self.Syringe` null)
  (set `self.CachedIndex` (`self.DrugIndex`))
  (set `self.DrugIndex` -1)
  (set `self.OnAmple` false)
  (return (`self.CachedIndex`)))