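; BP_MaskObj is an interactable mask in the Doctor level that starts and times the level's survival-style round.
; It shows an outline overlay when interactable; interacting plays a sequence whose completion triggers GameStart.
; GameStart uses chained delays to clear IsEnd on the patient, crate and entity spawner, then later the door.
; After the last delay EndGame sets those flags again and a second, victory sequence runs.
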(event `InteractionInterface.CanNotInteract`
  (params (Interactor :type "Actor Object Reference"))
  (`MeshComponent.SetOverlayMaterial` (`self.StaticMesh`) null))

(event `InteractionInterface.CanInteract`
  (params (Interactor :type "Actor Object Reference"))
  (`MeshComponent.SetOverlayMaterial` (`self.StaticMesh`) "/Game/BP/Material/MT_OutLine.MT_OutLine")
  (`KismetSystemLibrary.PrintString` "Hello"))

(event `InteractionInterface.OnInteract`
  (params (Interactor :type "Actor Object Reference"))
  (bind _as_bp_sequence_helper_1 (`self.As BP Sequence Helper_1`))
  (add `C_SequenceHelper.OnSequenceFinished` _as_bp_sequence_helper_1 (delegate `GameStart`))
  (`/Game/Sequence/BP_SequenceHelper.RunSequence` _as_bp_sequence_helper_1))

(event `GameStart`
  (`KismetSystemLibrary.Delay` 30.0)
  (`KismetSystemLibrary.PrintString` "게임시작")
  (set `C_DocPatient.isEnd` false (`self.Patient`))
  (set `C_Crate.isEnd` false (`self.As BP Crate`))
  (set `C_DocEntitySpawner.isEnd` false (`self.As BP Doc Entity Spawner`))
  (`KismetSystemLibrary.Delay` 120.0)
  (set `C_DoctorDoorKnockObj.isEnd` false (`self.As BP Doc Door`))
  (`KismetSystemLibrary.Delay` 240.0)
  (`self.EndGame`)
  (`KismetSystemLibrary.PrintString` "승리")
  (cast `/Game/BP/BP_GameInstance` (`GameplayStatics.GetGameInstance`))
  (`/Game/Sequence/BP_SequenceHelper.RunSequence` (`self.As BP Sequence Helper_2`)))

(event `EndGame`
  (set `C_DocPatient.isEnd` true (`self.Patient`))
  (set `C_Crate.isEnd` true (`self.As BP Crate`))
  (set `C_DocEntitySpawner.isEnd` true (`self.As BP Doc Entity Spawner`))
  (set `C_DoctorDoorKnockObj.isEnd` true (`self.As BP Doc Door`)))

(fn `GetCurrentQuestLineName`
  (params (Interactor :type "Actor Object Reference"))
  (returns (ReturnValue :type Name))
  (return "None"))

(fn `IsQuestObject`
  (params (Interactor :type "Actor Object Reference"))
  (returns (ReturnValue :type Boolean))
  (return false))

(fn `UserConstructionScript`)