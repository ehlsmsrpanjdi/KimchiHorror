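; BP_SadEntity is a Doctor level entity that walks to a patient, lingers, then leaves.
; MovetoPatient stores its spawner and index, runs AI MoveTo to the target and, on success, calls GoBackEvent after a delay.
; Interaction only prints a Korean debug message saying this entity should not be touched.
; The move and leave override events are empty.
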(event `self.MoveToPatient`
  (params (TargetLocation :type "Vector Structure (by ref)") (`As BP Doc Entity Spawner` :type "/Game/BP/DoctorLevel/BP_DocEntitySpawner Object Reference") (_index :type Integer))
  (set `self.Index` _index)
  (set `self.As BP Doc Entity Spawner` `As BP Doc Entity Spawner`)
  (`|AIMoveTo` self TargetLocation null
    (:`OnSuccess`
      (`KismetSystemLibrary.Delay` 10.0)
      (`self.GoBackEvent`))))

(event `InteractionInterface.OnInteract`
  (params (Interactor :type "Actor Object Reference"))
  (`KismetSystemLibrary.PrintString` "얘는 건들면 안됨 오히려"))

(event `self.OverrideMoveEvent`)

(event `self.OverrideLeaveEvent`)

(fn `UserConstructionScript`
  (`parent.UserConstructionScript`))