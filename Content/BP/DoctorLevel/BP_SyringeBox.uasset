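; BP_SyringeBox is an interactable box in the doctor level that gives the player a syringe.
; On interact, it reads the BP_DoctorLevelComponent on BP_MainPlayer and calls GainSyringe only if neither its Ample nor Syringe reference is valid.
; Otherwise it prints a Korean debug message saying the player holds medicine or already has a syringe.
; The CanInteract and CanNotInteract events are empty.
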(event `InteractionInterface.CanInteract`
  (params (Interactor :type "Actor Object Reference")))

(event `InteractionInterface.OnInteract`
  (params (Interactor :type "Actor Object Reference"))
  (bind _asbp_main_player (cast `/Game/Level/Stage_1Element/BP_MainPlayer` (`GameplayStatics.GetPlayerPawn` 0)))
  (bind _returnvalue (`self.GetComponentByClass` _asbp_main_player "/Game/BP/DoctorLevel/BP_DoctorLevelComponent.BP_DoctorLevelComponent_C"))
  (if (`KismetSystemLibrary.IsValid` (`/Game/BP/DoctorLevel/BP_DoctorLevelComponent.Ample` _returnvalue))
    (`KismetSystemLibrary.PrintString` "약을 들고있음")
    (elif (`KismetSystemLibrary.IsValid` (`/Game/BP/DoctorLevel/BP_DoctorLevelComponent.Syringe` _returnvalue))
      (`KismetSystemLibrary.PrintString` "이미 주사기가 있음")
      (else
        (`/Game/BP/DoctorLevel/BP_DoctorLevelComponent.GainSyringe` _returnvalue)))))

(event `InteractionInterface.CanNotInteract`
  (params (Interactor :type "Actor Object Reference")))

(fn `UserConstructionScript`)