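; BP_SyringeWaste is an interactable syringe disposal prop in the doctor level.
; On interact, it finds the player pawn's BP_DoctorLevelComponent and, if valid, calls WasteSyringe on it, leaving the disposal logic to that component.
; Interaction availability toggles an outline overlay material on its static mesh.
; It reports itself as a non-quest object with no quest line.
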(event `InteractionInterface.OnInteract`
  (params (Interactor :type "Actor Object Reference"))
  (bind _returnvalue (`self.GetComponentByClass` (`GameplayStatics.GetPlayerPawn` 0) "/Game/BP/DoctorLevel/BP_DoctorLevelComponent.BP_DoctorLevelComponent_C"))
  (if (`KismetSystemLibrary.IsValid` _returnvalue)
    (`C_DocLevelComponent.WasteSyringe` _returnvalue)))

(event `InteractionInterface.CanInteract`
  (params (Interactor :type "Actor Object Reference"))
  (`MeshComponent.SetOverlayMaterial` (`self.StaticMesh`) "/Game/BP/Material/MT_OutLine.MT_OutLine"))

(event `InteractionInterface.CanNotInteract`
  (params (Interactor :type "Actor Object Reference"))
  (`MeshComponent.SetOverlayMaterial` (`self.StaticMesh`) null))

(fn `GetCurrentQuestLineName`
  (params (Interactor :type "Actor Object Reference"))
  (returns (ReturnValue :type Name))
  (return "None"))

(fn `IsQuestObject`
  (params (Interactor :type "Actor Object Reference"))
  (returns (ReturnValue :type Boolean))
  (return false))

(fn `UserConstructionScript`)