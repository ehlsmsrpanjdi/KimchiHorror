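; BP_DocInteractiveInterface is a doctor-level interactable actor that shows an interaction prompt and a doubt-driven noise effect.
; On BeginPlay it caches the BP_InterMassage widget from the UI manager, then shows its message when BP_MainPlayer can interact and turns it off when interaction ends.
; SetNoise creates a Test_Noise dynamic material on Noise, scaling NoiseIntensity from Doubt.
; Quest queries return stub values, marking it as a non-quest object.
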(event `self.SetNoise`
  (params (Doubt :type Integer))
  (bind _returnvalue (`PrimitiveComponent.CreateDynamicMaterialInstance` (`self.Noise`) 0 "/Game/BP/Stage1/InteractiveEntity/Test_Noise.Test_Noise" "None"))
  (`MaterialInstanceDynamic.SetScalarParameterValue` _returnvalue "NoiseIntensity" (/ (`KismetMathLibrary.Conv_IntToDouble` Doubt) 100.0)))

(event `self.ReceiveBeginPlay`
  (bind _returnvalue (`C_UIManager.GetUI` (`C_UIManager.GetUIManager`) "/Game/BP/UI/Common/Text/BP_InterMassage.BP_InterMassage_C"))
  (bind _asbp_inter_massage (cast `/Game/BP/UI/Common/Text/BP_InterMassage` _returnvalue))
  (set `self.As BP Inter Massage` _asbp_inter_massage))

(event `self.CanInteract`
  (params (Interactor :type "Actor Object Reference"))
  (`KismetSystemLibrary.PrintString` "상호 시작")
  (cast `/Game/Level/Stage_1Element/BP_MainPlayer` Interactor)
  (`/Game/BP/UI/Common/Text/BP_InterMassage.OnInteraction` (`self.As BP Inter Massage`) (`self.InteractionMassage`))
  (`C_UIManager.OnUI` (`C_UIManager.GetUIManager`) "/Script/HorrorProtoKimchi.C_InterUI"))

(event `self.CanNotInteract`
  (params (Interactor :type "Actor Object Reference"))
  (`KismetSystemLibrary.PrintString` "상호 끝")
  (`/Game/BP/UI/Common/Text/BP_InterMassage.OffInteraction` (`self.As BP Inter Massage`)))

(fn `GetCurrentQuestLineName`
  (params (Interactor :type "Actor Object Reference"))
  (returns (ReturnValue :type Name))
  (return "None"))

(fn `IsQuestObject`
  (params (Interactor :type "Actor Object Reference"))
  (returns (ReturnValue :type Boolean))
  (return false))

(fn `UserConstructionScript`)