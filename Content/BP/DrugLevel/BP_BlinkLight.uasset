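; BP_BlinkLight is a spot light actor for the drug level that can switch into a flickering state.
; While blinking is on, Tick sets the light's intensity from a flicker noise function.
; OnBlink starts the flicker, and OffBlink stops it and resets a fixed intensity.
; An alternative using a dynamic light-function material with an IsBlink parameter is left unconnected and never runs.
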(event `self.ReceiveBeginPlay`)

(event `self.ReceiveTick`
  (params (DeltaSeconds :type "Float (single-precision)"))
  (if (`self.IsBlinking`)
    (bind _returnvalue (`self.GetFlickerNoise` 0.0 100.0 10.0))
    (`LightComponent.SetIntensity` (`self.SpotLight`) _returnvalue)))

(event `OnBlink`
  (set `self.IsBlinking` true))

(event `OffBlink`
  (set `self.IsBlinking` false)
  (`LightComponent.SetIntensity` (`self.SpotLight`) 100.0))

(fn `UserConstructionScript`)