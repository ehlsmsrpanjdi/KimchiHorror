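; BP_CheatCheck is a trigger volume in the drug level that punishes the player for reaching it while the light index is wrong.
; When BP_MainPlayer overlaps its Box, it compares its own LightIndex to the one in BP_DrugGameState.
; On a mismatch it calls JumpScare on the player with BP_JumpScareDarkEntity.
; It prints the game state's LightIndex for debugging at BeginPlay and after each triggered scare.
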(event `self.ReceiveBeginPlay`
  (bind _asbp_drug_game_state (cast `/Game/BP/DrugLevel/BP_DrugGameState` (`GameplayStatics.GetGameState`)))
  (`KismetSystemLibrary.PrintString` (`KismetStringLibrary.Conv_IntToString` (`C_DrugLevelGameState.LightIndex` _asbp_drug_game_state))))

(event `self.Box.OnComponentBeginOverlap`
  (params (OverlappedComponent :type "PrimitiveComponent Object Reference") (OtherActor :type "Actor Object Reference") (OtherComp :type "PrimitiveComponent Object Reference") (OtherBodyIndex :type Integer) (bFromSweep :type Boolean) (SweepResult :type "HitResult Structure (by ref)"))
  (bind _asbp_main_player (cast `/Game/Level/Stage_1Element/BP_MainPlayer` OtherActor))
  (bind _asbp_drug_game_state (cast `/Game/BP/DrugLevel/BP_DrugGameState` (`GameplayStatics.GetGameState`)))
  (bind _lightindex (`C_DrugLevelGameState.LightIndex` _asbp_drug_game_state))
  (if (!= _lightindex (`self.LightIndex`))
    (`/Game/Level/Stage_1Element/BP_MainPlayer.JumpScare` _asbp_main_player "/Game/BP/JumpScare/BP_JumpScareDarkEntity.BP_JumpScareDarkEntity_C" null)
    (`KismetSystemLibrary.PrintString` (`KismetStringLibrary.Conv_IntToString` _lightindex))))

(fn `UserConstructionScript`)