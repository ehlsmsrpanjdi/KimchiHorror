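; BP_DifferentColorLight is a drug-level spotlight that turns dark red when the player walks into its Box trigger.
; It registers itself with BP_DrugGameState on BeginPlay.
; Its OnLight and OffLight events switch the spotlight intensity between very bright and zero, with switching on gated by the CanLight flag.
; The color change has no reset in this graph.
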(event `self.ReceiveBeginPlay`
  (bind _asbp_drug_game_state (cast `/Game/BP/DrugLevel/BP_DrugGameState` (`GameplayStatics.GetGameState`)))
  (`C_DrugLevelGameState.AddLight` _asbp_drug_game_state self))

(event `self.Box.OnComponentBeginOverlap`
  (params (OverlappedComponent :type "PrimitiveComponent Object Reference") (OtherActor :type "Actor Object Reference") (OtherComp :type "PrimitiveComponent Object Reference") (OtherBodyIndex :type Integer) (bFromSweep :type Boolean) (SweepResult :type "HitResult Structure (by ref)"))
  (cast `/Game/Level/Stage_1Element/BP_MainPlayer` OtherActor)
  (`LightComponent.SetLightColor` (`self.SpotLight`) (struct :`R` 0.328125 :`A` 1.0) true))

(event `self.OnLight`
  (if (`self.CanLight`)
    (`LightComponent.SetIntensity` (`self.SpotLight`) 100000.0)))

(event `self.OffLight`
  (`LightComponent.SetIntensity` (`self.SpotLight`) 0.0))

(fn `UserConstructionScript`)