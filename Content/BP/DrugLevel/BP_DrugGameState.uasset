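; BP_DrugGameState is the drug level's game state Blueprint and acts as a central switch for a group of lights.
; TurnOnLight and TurnOffLight loop over the AllLight array, skip invalid entries, set each light's CanLight flag and call its OnLight or OffLight.
; Nothing in this Blueprint fills AllLight or triggers either event, and the construction script is empty.
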(event `TurnOnLight`
  (for _array_element (`self.AllLight`)
    (if (`KismetSystemLibrary.IsValid` _array_element)
      (set `C_BlinkLight.CanLight` true _array_element)
      (`C_BlinkLight.OnLight` _array_element))))

(event `TurnOffLight`
  (for _array_element (`self.AllLight`)
    (if (`KismetSystemLibrary.IsValid` _array_element)
      (set `C_BlinkLight.CanLight` false _array_element)
      (`C_BlinkLight.OffLight` _array_element))))

(fn `UserConstructionScript`)