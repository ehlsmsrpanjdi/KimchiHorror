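; BP_FaceWall is an advancing wall hazard in the drug level that starts moving once a sequence finishes.
; BeginPlay binds StartEntity to the sequence helper's finished event, which enables a constant-speed Tick move along the Arrow's forward vector without sweep.
; Its Box overlap hides any BP_PathLight it reaches and, for BP_MainPlayer, only prints a player-death message without applying any death logic.
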(event `StartEntity`
  (set `self.MoveStart` true))

(event `self.ReceiveBeginPlay`
  (add `C_SequenceHelper.OnSequenceFinished` (`self.As BP Sequence Helper`) (delegate `StartEntity`)))

(event `self.ReceiveTick`
  (params (DeltaSeconds :type "Float (single-precision)"))
  (if (`self.MoveStart`)
    (`self.K2_AddActorWorldOffset` (* (`SceneComponent.GetForwardVector` (`self.Arrow`)) (* DeltaSeconds 20.0)))))

(event `self.Box.OnComponentBeginOverlap`
  (params (OverlappedComponent :type "PrimitiveComponent Object Reference") (OtherActor :type "Actor Object Reference") (OtherComp :type "PrimitiveComponent Object Reference") (OtherBodyIndex :type Integer) (bFromSweep :type Boolean) (SweepResult :type "HitResult Structure (by ref)"))
  (bind _asbp_path_light (cast `/Game/BP/DrugLevel/BP_PathLight` OtherActor)
    (:`then`
      (`self.SetActorHiddenInGame` _asbp_path_light true))
    (:`CastFailed`
      (cast `/Game/Level/Stage_1Element/BP_MainPlayer` OtherActor)
      (`KismetSystemLibrary.PrintString` "플레이어 사망"))))

(fn `UserConstructionScript`)