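; BP_LightEntity is an entity in the DrugLevel folder that makes nearby BP_BlinkLight actors blink.
; Its LightBox component acts as the trigger, calling OnBlink on each blink light it begins overlapping and OffBlink when that overlap ends.
; BeginPlay is empty, and unconnected debug nodes for unhiding the box and capsule and printing the actor's location never run.
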(event `self.ReceiveBeginPlay`)

(event `self.LightBox.OnComponentBeginOverlap`
  (params (OverlappedComponent :type "PrimitiveComponent Object Reference") (OtherActor :type "Actor Object Reference") (OtherComp :type "PrimitiveComponent Object Reference") (OtherBodyIndex :type Integer) (bFromSweep :type Boolean) (SweepResult :type "HitResult Structure (by ref)"))
  (bind _asbp_blink_light (cast `/Game/BP/DrugLevel/BP_BlinkLight` OtherActor))
  (`/Game/BP/DrugLevel/BP_BlinkLight.OnBlink` _asbp_blink_light))

(event `self.LightBox.OnComponentEndOverlap`
  (params (OverlappedComponent :type "PrimitiveComponent Object Reference") (OtherActor :type "Actor Object Reference") (OtherComp :type "PrimitiveComponent Object Reference") (OtherBodyIndex :type Integer))
  (bind _asbp_blink_light (cast `/Game/BP/DrugLevel/BP_BlinkLight` OtherActor))
  (`/Game/BP/DrugLevel/BP_BlinkLight.OffBlink` _asbp_blink_light))

(fn `UserConstructionScript`)