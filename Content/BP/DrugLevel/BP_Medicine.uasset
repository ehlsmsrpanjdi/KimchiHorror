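; BP_Medicine is a quest-object actor in the drug level that animates one of its components on BeginPlay.
; It caches that component's world location, then a timeline lerps it toward the Arrow component's location.
; Its quest functions return true for IsQuestObject and QuestLine as the current quest line name.
; The interaction events are placeholders that only print "Hello".
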(event `self.ReceiveBeginPlay`
  (set `self.NewVar` (`SceneComponent.K2_GetComponentLocation` (`self.cum`)))
  (`self.LetsCum`))

(event `self.ReceiveTick`
  (params (DeltaSeconds :type "Float (single-precision)")))

(event `LetsCum`
  (bind (_direction `_새_트랙_0`) (`Timeline|타임라인`)
    (:`Update`
      (`SceneComponent.K2_SetWorldLocation` (`self.cum`) (`KismetMathLibrary.VLerp` (`self.NewVar`) (`SceneComponent.K2_GetComponentLocation` (`self.Arrow`)) `_새_트랙_0`) false false))))

(event `InteractionInterface.OnInteract`
  (params (Interactor :type "Actor Object Reference"))
  (`KismetSystemLibrary.PrintString` "Hello"))

(event `InteractionInterface.CanInteract`
  (params (Interactor :type "Actor Object Reference"))
  (`KismetSystemLibrary.PrintString` "Hello"))

(event `InteractionInterface.CanNotInteract`
  (params (Interactor :type "Actor Object Reference"))
  (`KismetSystemLibrary.PrintString` "Hello"))

(fn `GetCurrentQuestLineName`
  (params (Interactor :type "Actor Object Reference"))
  (returns (ReturnValue :type Name))
  (return (`self.QuestLine`)))

(fn `IsQuestObject`
  (params (Interactor :type "Actor Object Reference"))
  (returns (ReturnValue :type Boolean))
  (return true))

(fn `UserConstructionScript`)