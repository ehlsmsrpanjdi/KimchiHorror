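; BP_NormalLight is a spotlight in the drug level that acts as a safe zone, halting the game state's LightEntity while the player stands in it.
; It registers itself with BP_DrugGameState on BeginPlay.
; Its box overlap stops the entity on entry and sends it toward the player on exit.
; OffLight and OnLight switch the intensity, with OffLight releasing the entity and OnLight re-stopping it if CanLight and overlap are set.
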(event `self.ReceiveBeginPlay`
  (bind _asbp_drug_game_state (cast `/Game/BP/DrugLevel/BP_DrugGameState` (`GameplayStatics.GetGameState`)))
  (`C_DrugLevelGameState.AddLight` _asbp_drug_game_state self))

(event `self.Box.OnComponentBeginOverlap`
  (params (OverlappedComponent :type "PrimitiveComponent Object Reference") (OtherActor :type "Actor Object Reference") (OtherComp :type "PrimitiveComponent Object Reference") (OtherBodyIndex :type Integer) (bFromSweep :type Boolean) (SweepResult :type "HitResult Structure (by ref)"))
  (cast `/Game/Level/Stage_1Element/BP_MainPlayer` OtherActor)
  (set `self.IsOverlap` true)
  (bind _asbp_drug_game_state (cast `/Game/BP/DrugLevel/BP_DrugGameState` (`GameplayStatics.GetGameState`)))
  (`/Game/BP/DrugLevel/BP_LightEntity.StopMove` (`/Game/BP/DrugLevel/BP_DrugGameState.LightEntity` _asbp_drug_game_state)))

(event `self.Box.OnComponentEndOverlap`
  (params (OverlappedComponent :type "PrimitiveComponent Object Reference") (OtherActor :type "Actor Object Reference") (OtherComp :type "PrimitiveComponent Object Reference") (OtherBodyIndex :type Integer))
  (cast `/Game/Level/Stage_1Element/BP_MainPlayer` OtherActor)
  (set `self.IsOverlap` false)
  (bind _asbp_drug_game_state (cast `/Game/BP/DrugLevel/BP_DrugGameState` (`GameplayStatics.GetGameState`)))
  (`/Game/BP/DrugLevel/BP_LightEntity.MoveToPlayer` (`/Game/BP/DrugLevel/BP_DrugGameState.LightEntity` _asbp_drug_game_state)))

(event `self.OffLight`
  (`LightComponent.SetIntensity` (`self.SpotLight`) 0.0)
  (if (`self.IsOverlap`)
    (bind _asbp_drug_game_state (cast `/Game/BP/DrugLevel/BP_DrugGameState` (`GameplayStatics.GetGameState`)))
    (`/Game/BP/DrugLevel/BP_LightEntity.MoveToPlayer` (`/Game/BP/DrugLevel/BP_DrugGameState.LightEntity` _asbp_drug_game_state))
    (set `self.IsOverlap` false)))

(event `self.OnLight`
  (`LightComponent.SetIntensity` (`self.SpotLight`) 100000.0)
  (if (`self.CanLight`)
    (if (`self.IsOverlap`)
      (bind _asbp_drug_game_state (cast `/Game/BP/DrugLevel/BP_DrugGameState` (`GameplayStatics.GetGameState`)))
      (`/Game/BP/DrugLevel/BP_LightEntity.StopMove` (`/Game/BP/DrugLevel/BP_DrugGameState.LightEntity` _asbp_drug_game_state)))))

(fn `UserConstructionScript`)