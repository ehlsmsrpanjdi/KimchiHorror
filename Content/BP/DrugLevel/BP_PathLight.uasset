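; BP_PathLight is a spotlight in the drug level's path sequence, hidden at start unless marked as a starter.
; When the player enters its box, it reports to BP_DrugGameState, checking its index if it is a correct light or calling InCorrect otherwise.
; It then shows the spotlight in the game state's current color.
; Only an accepted index locks it against further overlaps.
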(event `self.ReceiveBeginPlay`
  (if (not (`self.Starter`))
    (`SceneComponent.SetHiddenInGame` (`self.SpotLight`) true false)))

(event `self.Box.OnComponentBeginOverlap`
  (params (OverlappedComponent :type "PrimitiveComponent Object Reference") (OtherActor :type "Actor Object Reference") (OtherComp :type "PrimitiveComponent Object Reference") (OtherBodyIndex :type Integer) (bFromSweep :type Boolean) (SweepResult :type "HitResult Structure (by ref)"))
  (if (not (`self.IsOverlaped`))
    (cast `/Game/Level/Stage_1Element/BP_MainPlayer` OtherActor)
    (bind _asbp_drug_game_state (cast `/Game/BP/DrugLevel/BP_DrugGameState` (`GameplayStatics.GetGameState`)))
    (if (`self.IsCorrect`)
      (bind _returnvalue (`C_DrugLevelGameState.CheckIndex` _asbp_drug_game_state (`self.LightIndex`)))
      (if _returnvalue
        (set `self.bIsOverlaped` true))
      (else
        (`/Game/BP/DrugLevel/BP_DrugGameState.InCorrect` _asbp_drug_game_state)))
    (bind _returnvalue_2 (`C_DrugLevelGameState.GetColor` _asbp_drug_game_state))
    (`LightComponent.SetLightColor` (`self.SpotLight`) _returnvalue_2 true)
    (`SceneComponent.SetHiddenInGame` (`self.SpotLight`) false false)))

(fn `UserConstructionScript`)