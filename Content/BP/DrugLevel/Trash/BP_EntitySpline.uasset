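; BP_EntitySpline is a spline actor that spawns a BP_LightEntity_2 when play begins and hands it the path data.
; SpawnEntity places the entity at the Arrow component's world location, printing that location as debug output.
; It then passes its Spline and MoveClock to the new entity and calls StartMachine on it.
; The actor holds no movement logic itself.
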(event `self.ReceiveBeginPlay`
  (`self.SpawnEntity`))

(event `SpawnEntity`
  (bind _returnvalue (`SceneComponent.K2_GetComponentLocation` (`self.Arrow`)))
  (`KismetSystemLibrary.PrintString` (`KismetStringLibrary.Conv_VectorToString` _returnvalue))
  (bind _returnvalue_2 (`|SpawnActorFromClass` "/Game/BP/DrugLevel/Trash/BP_LightEntity_2.BP_LightEntity_2_C" (`KismetMathLibrary.MakeTransform` _returnvalue) "Undefined" "MultiplyWithRoot" null null))
  (set `C_BlinkEntity.Spline` (`self.Spline`) _returnvalue_2)
  (set `C_BlinkEntity.MoveClock` (`self.MoveClock`) _returnvalue_2)
  (`C_BlinkEntity.StartMachine` _returnvalue_2))

(fn `UserConstructionScript`)