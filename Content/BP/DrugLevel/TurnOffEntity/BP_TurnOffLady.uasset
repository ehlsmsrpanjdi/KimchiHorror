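; Female entity character in the drug level that walks off to switch off the light when the player enters its trigger box, then removes itself.
; The one-shot overlap starts an AI move toward the light button; timed delays stop it, call TurnOffLight on BP_DrugGameState and destroy the actor.
; Interface events forward face, head-tilt and body poses to its anim blueprints.
; Modular outfit meshes follow the body as leader pose.
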(event `self.ReceiveBeginPlay`
  (`parent.ReceiveBeginPlay`)
  (set `self.MyFace` (`self.Face`))
  (`SceneComponent.K2_AttachToComponent` (`self.Noise`) (`self.Mesh`) "headSocket" "KeepRelative" "KeepRelative" "KeepRelative" true))

(event `self.ISetFaceMove`
  (params (Pose :type "C_FacePoseEnum Enum" :default "Idle") (Mood :type "C_FaceMoodEnum Enum" :default "Normal") (Interval :type "Float (double-precision)"))
  (bind _asbp_entity_face_anim (cast `/Game/BP/Stage1/InteractiveEntity/AnimIns/Face/BP_EntityFaceAnim` (`SkeletalMeshComponent.GetAnimInstance` (`self.Face`)))
    (:`then`
      (`C_AnimBPBase.SetFacePose` _asbp_entity_face_anim Pose Mood Interval))
    (:`CastFailed`
      (`KismetSystemLibrary.PrintString` "FaceMissing"))))

(event `self.ISetHeadTilting`
  (params (DesVector :type "Vector Structure") (RotateSpeed :type "Float (double-precision)"))
  (bind _asbp_female_entity_body_anim (cast `/Game/BP/Stage1/InteractiveEntity/AnimIns/Body/BP_FemaleEntityBodyAnim` (`SkeletalMeshComponent.GetAnimInstance` (`self.Mesh`)))
    (:`then`
      (`C_EntityAnimBase.LerfTiltHead` _asbp_female_entity_body_anim DesVector RotateSpeed))
    (:`CastFailed`
      (`KismetSystemLibrary.PrintString` "TiltingMissing"))))

(event `self.ISetBodyMove`
  (params (Move :type "C_EntityMoveEnum Enum" :default "Idle"))
  (bind _asbp_female_entity_body_anim (cast `/Game/BP/Stage1/InteractiveEntity/AnimIns/Body/BP_FemaleEntityBodyAnim` (`SkeletalMeshComponent.GetAnimInstance` (`self.Mesh`)))
    (:`then`
      (`C_EntityAnimBase.SetBodyMove` _asbp_female_entity_body_anim Move))
    (:`CastFailed`
      (`KismetSystemLibrary.PrintString` "BodyMissing"))))

(event `self.Box.OnComponentBeginOverlap`
  (params (OverlappedComponent :type "PrimitiveComponent Object Reference") (OtherActor :type "Actor Object Reference") (OtherComp :type "PrimitiveComponent Object Reference") (OtherBodyIndex :type Integer) (bFromSweep :type Boolean) (SweepResult :type "HitResult Structure (by ref)"))
  (cast `/Game/Level/Stage_1Element/BP_MainPlayer` OtherActor)
  (`self.TurnOffLight`)
  (`ActorComponent.K2_DestroyComponent` (`self.Box`)))

(event `TurnOffLight`
  (`C_KimchiHelper.MoveToActorAndCheckArrival` self (`self.As BP Turn On Light Btn`))
  (`KismetSystemLibrary.Delay` 2.0)
  (`Controller.StopMovement` (`AIBlueprintHelperLibrary.GetAIController` self))
  (bind _asbp_drug_game_state (cast `/Game/BP/DrugLevel/BP_DrugGameState` (`GameplayStatics.GetGameState`)))
  (`/Game/BP/DrugLevel/BP_DrugGameState.TurnOffLight` _asbp_drug_game_state)
  (`KismetSystemLibrary.Delay` 1.0)
  (`self.K2_DestroyActor`))

(fn `UserConstructionScript`
  (`SkinnedMeshComponent.SetLeaderPoseComponent` (`self.Clothes`) (`self.Mesh`) false false)
  (`SkinnedMeshComponent.SetLeaderPoseComponent` (`self.Gloves`) (`self.Mesh`) false false)
  (`SkinnedMeshComponent.SetLeaderPoseComponent` (`self.Hat`) (`self.Mesh`) false false)
  (`SkinnedMeshComponent.SetLeaderPoseComponent` (`self.Arms`) (`self.Mesh`) false false)
  (`SkinnedMeshComponent.SetLeaderPoseComponent` (`self.Pants`) (`self.Mesh`) false false)
  (`SkinnedMeshComponent.SetLeaderPoseComponent` (`self.Helmet`) (`self.Mesh`) false false))