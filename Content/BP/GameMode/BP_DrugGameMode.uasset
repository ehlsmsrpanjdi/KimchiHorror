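; BP_DrugGameMode is a game mode that resets manager state and builds the UI when play begins.
; BeginPlay empties the CDoubtsManager array and clears the UI manager's dictionary.
; If the game instance casts to BP_GameInstance, it then creates the interaction message, dialog, menu, pop-up message and eye-blink widgets through the UI manager.
; Tick and the construction script are empty.
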(event `self.ReceiveBeginPlay`
  (bind _returnvalue (`C_UIManager.GetUIManager`))
  (`C_DoubtsManager.EmptyArrayfuckyou` (subsystem `C_DoubtsManager`))
  (`C_UIManager.ClearDictionary` _returnvalue)
  (cast `/Game/BP/BP_GameInstance` (`GameplayStatics.GetGameInstance`))
  (`C_UIManager.CreateAndAddUI` _returnvalue "/Game/BP/UI/Common/Text/BP_InterMassage.BP_InterMassage_C")
  (`C_UIManager.CreateAndAddUI` _returnvalue "/Game/BP/UI/Common/Text/BP_Dialog.BP_Dialog_C")
  (`C_UIManager.CreateAndAddUI` _returnvalue "/Game/BP/UI/Common/Stash/BP_MenuUI.BP_MenuUI_C")
  (`C_UIManager.CreateAndAddUI` _returnvalue "/Game/BP/UI/Common/Text/BP_PopUpMassage.BP_PopUpMassage_C")
  (`C_UIManager.CreateAndAddUI` _returnvalue "/Game/BP/UI/Common/FunctionUI/BP_BlinkEye.BP_BlinkEye_C"))

(fn `UserConstructionScript`)