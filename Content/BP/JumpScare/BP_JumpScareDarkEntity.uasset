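; BP_JumpScareDarkEntity is a jump scare actor that shows a dark entity and then respawns the player.
; On BeginPlay it starts a camera shake and runs a delay chain that clears Move, calls FadeIn on the player controller, then calls ReSpawnPlayer on the game instance.
; While Move is true, Tick slides the skeletal mesh along the Arrow component's forward vector at constant speed, without sweep.
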(event `self.ReceiveBeginPlay`
  (`PlayerCameraManager.StartCameraShake` :`self` (`GameplayStatics.GetPlayerCameraManager` 0) :`ShakeClass` "/Game/BP/Common/BP_JumpScareShake.BP_JumpScareShake_C")
  (`KismetSystemLibrary.Delay` 0.5)
  (set `self.Move` false)
  (`KismetSystemLibrary.Delay` 0.5)
  (bind _asbp_main_player_controller (cast `/Game/Level/Stage_1Element/BP_MainPlayerController` (`GameplayStatics.GetPlayerController` 0)))
  (`/Game/Level/Stage_1Element/BP_MainPlayerController.FadeIn` _asbp_main_player_controller 4.0)
  (`KismetSystemLibrary.Delay` 1.0)
  (bind _asbp_game_instance (cast `/Game/BP/BP_GameInstance` (`GameplayStatics.GetGameInstance`)))
  (`C_GameInstance.ReSpawnPlayer` _asbp_game_instance))

(event `self.ReceiveTick`
  (params (DeltaSeconds :type "Float (single-precision)"))
  (if (`self.Move`)
    (`SceneComponent.K2_AddWorldOffset` (`self.SkeletalMesh`) (* (* (`SceneComponent.GetForwardVector` (`self.Arrow`)) DeltaSeconds) 370.0) false false)))

(fn `UserConstructionScript`)