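; BP_EscapeKey is an interactable key object for the last level.
; Interacting with it runs a sequence through a referenced BPSequenceHelper.
; It shows an outline overlay material on its static mesh while interaction is available and clears it otherwise.
; Its quest queries report that it is not a quest object and has no quest line.
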(event `InteractionInterface.OnInteract`
  (params (Interactor :type "Actor Object Reference"))
  (`/Game/Sequence/BP_SequenceHelper.RunSequence` (`self.As BP Sequence Helper`)))

(event `InteractionInterface.CanNotInteract`
  (params (Interactor :type "Actor Object Reference"))
  (`MeshComponent.SetOverlayMaterial` (`self.StaticMesh`) null))

(event `InteractionInterface.CanInteract`
  (params (Interactor :type "Actor Object Reference"))
  (`MeshComponent.SetOverlayMaterial` (`self.StaticMesh`) "/Game/BP/Material/MT_OutLine.MT_OutLine"))

(fn `GetCurrentQuestLineName`
  (params (Interactor :type "Actor Object Reference"))
  (returns (ReturnValue :type Name))
  (return "None"))

(fn `IsQuestObject`
  (params (Interactor :type "Actor Object Reference"))
  (returns (ReturnValue :type Boolean))
  (return false))

(fn `UserConstructionScript`)