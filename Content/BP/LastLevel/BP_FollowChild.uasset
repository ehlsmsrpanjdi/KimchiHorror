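; BP_FollowChild is an AI-moved child character in the last level that follows the player once triggered.
; Player overlap with MoveStartCollision destroys that trigger and sets MoveStart, after which Tick repeatedly calls MoveToActorAndCheckArrival toward the player.
; DoorCollision calls EntityOpen on any BP_Door it overlaps, passing itself.
; Tick also stores velocity magnitude as Speed, and player overlap with PlayerCol only prints the player's name.
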(event `self.ReceiveTick`
  (params (DeltaSeconds :type "Float (single-precision)"))
  (set `self.Speed` (`KismetMathLibrary.VSize` (`MovementComponent.Velocity` (`self.CharacterMovement`))))
  (if (`self.MoveStart`)
    (`C_KimchiHelper.MoveToActorAndCheckArrival` self (`self.Player`))))

(event `self.doorCollision.OnComponentBeginOverlap`
  (params (OverlappedComponent :type "PrimitiveComponent Object Reference") (OtherActor :type "Actor Object Reference") (OtherComp :type "PrimitiveComponent Object Reference") (OtherBodyIndex :type Integer) (bFromSweep :type Boolean) (SweepResult :type "HitResult Structure (by ref)"))
  (bind _asbp_door (cast `/Game/BP/Common/BP_Door` OtherActor))
  (`/Game/BP/Common/BP_DoorBase.EntityOpen` _asbp_door self))

(event `self.PlayerCol.OnComponentBeginOverlap`
  (params (OverlappedComponent :type "PrimitiveComponent Object Reference") (OtherActor :type "Actor Object Reference") (OtherComp :type "PrimitiveComponent Object Reference") (OtherBodyIndex :type Integer) (bFromSweep :type Boolean) (SweepResult :type "HitResult Structure (by ref)"))
  (if (== OtherActor (`self.Player`))
    (`KismetSystemLibrary.PrintString` (`KismetSystemLibrary.GetDisplayName` OtherActor))))

(event `self.MoveStartCollision.OnComponentBeginOverlap`
  (params (OverlappedComponent :type "PrimitiveComponent Object Reference") (OtherActor :type "Actor Object Reference") (OtherComp :type "PrimitiveComponent Object Reference") (OtherBodyIndex :type Integer) (bFromSweep :type Boolean) (SweepResult :type "HitResult Structure (by ref)"))
  (if (== OtherActor (`self.Player`))
    (`ActorComponent.K2_DestroyComponent` (`self.MoveStartCollision`))
    (set `self.MoveStart` true)))

(fn `UserConstructionScript`)