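; BP_NumberPad is an interactable keypad puzzle that clears a linked puzzle door when the correct code is entered.
; Interacting switches view and input to the pad with a mouse cursor, and E returns control to the pawn.
; Clicks trace to box components whose name's last character selects the key: digits spawn number actors up to four, # clears, and * checks the answer and fires success events.
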(event `self.ReceiveBeginPlay`
  (`self.CalculateDirection`))

(event `InteractionInterface.OnInteract`
  (params (Interactor :type "Actor Object Reference"))
  (bind _returnvalue (`GameplayStatics.GetPlayerController` 0))
  (`PlayerController.SetViewTargetWithBlend` _returnvalue self 0.0 "VTBlend_Linear" 0.0 false)
  (`self.EnableInput` _returnvalue)
  (`self.DisableInput` (`GameplayStatics.GetPlayerPawn` 0) _returnvalue)
  (set `PlayerController.bShowMouseCursor` true _returnvalue))

(event `Key|LeftMouseButton`
  (params (Key :type "Key Structure"))
  (bind _bp_puzzledoor (`self.BP_PuzzleDoor`))
  (:`Pressed`
    (bind `_as박스_콜리전` (cast `BoxComponent` (`.HitComponent` (`GameplayStatics.BreakHitResult` (`PlayerController.GetHitResultUnderCursorByChannel` (`GameplayStatics.GetPlayerController` 0) "TraceTypeQuery1" true)))))
    (bind _returnvalue (`self.CalculateCurrentPos` 2.5))
    (bind _returnvalue_2 (`KismetStringLibrary.Right` (`KismetSystemLibrary.GetDisplayName` `_as박스_콜리전`) 1))
    (if (`KismetStringLibrary.EqualEqual_StrStr` _returnvalue_2 "#")
      (`self.ClearNumber`)
      (elif (`KismetStringLibrary.EqualEqual_StrStr` _returnvalue_2 "*")
        (bind _returnvalue_3 (`self.CheckAnswer`))
        (if _returnvalue_3
          (`self.ActiveAllEvent`)
          (if (`KismetSystemLibrary.IsValid` _bp_puzzledoor)
            (`/Game/BP/PuzzleLevel/BP_PuzzleDoor.ClearEvent` _bp_puzzledoor)))
        (elif (not (>= (`KismetArrayLibrary.Array_Length` (`self.CurrentArrayValue`)) 4))
          (bind _returnvalue_4 (`KismetStringLibrary.Conv_StringToInt` _returnvalue_2))
          (`KismetArrayLibrary.Array_Add` (`self.CurrentArrayValue`) _returnvalue_4)
          (bind _returnvalue_5 (`|SpawnActorFromClass` (`|GetArrayItem` (`self.NumberAssetArray`) _returnvalue_4) (`KismetMathLibrary.MakeTransform` _returnvalue (`SceneComponent.K2_GetComponentRotation` (`self.DirectionComponent`))) "Undefined" "MultiplyWithRoot" null null))
          (`KismetArrayLibrary.Array_Add` (`self.NumberArray`) _returnvalue_5))))))

(event `Key|E`
  (params (Key :type "Key Structure"))
  (bind _returnvalue (`GameplayStatics.GetPlayerController` 0))
  (bind _returnvalue_2 (`GameplayStatics.GetPlayerPawn` 0))
  (:`Pressed`
    (`self.EnableInput` _returnvalue_2 _returnvalue)
    (`self.DisableInput` _returnvalue)
    (`PlayerController.SetViewTargetWithBlend` _returnvalue _returnvalue_2 0.0 "VTBlend_Linear" 0.0 false)
    (set `PlayerController.bShowMouseCursor` false _returnvalue)))

(fn `GetCurrentQuestLineName`
  (params (Interactor :type "Actor Object Reference"))
  (returns (ReturnValue :type Name))
  (return "None"))

(fn `IsQuestObject`
  (params (Interactor :type "Actor Object Reference"))
  (returns (ReturnValue :type Boolean))
  (return false))

(fn `UserConstructionScript`)