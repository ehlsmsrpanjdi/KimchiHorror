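; BP_PuzzleCabinet is a puzzle-level cabinet whose door swings open when the puzzle is cleared.
; BeginPlay caches the door's world rotation as the closed pose.
; ClearEvent plays the DoorOpen timeline, lerping the door from that rotation to a combined 120-degree rotated offset.
; The interact and can/cannot-interact events are empty, so direct interaction does nothing here.
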(event `self.ReceiveBeginPlay`
  (set `self.CabinetRotation` (`SceneComponent.K2_GetComponentRotation` (`self.Door`))))

(event `InteractionInterface.OnInteract`
  (params (Interactor :type "Actor Object Reference")))

(event `self.ClearEvent`
  (bind (_direction `_새_트랙_0`) (`Timeline|DoorOpen`)
    (:`Update`
      (`SceneComponent.K2_SetWorldRotation` (`self.Door`) (`KismetMathLibrary.RLerp` (`self.CabinetRotation`) (`KismetMathLibrary.ComposeRotators` (`self.CabinetRotation`) (struct :`Yaw` -120.0)) `_새_트랙_0`) false false))))

(event `InteractionInterface.CanNotInteract`
  (params (Interactor :type "Actor Object Reference")))

(event `InteractionInterface.CanInteract`
  (params (Interactor :type "Actor Object Reference")))

(fn `UserConstructionScript`
  (`parent.UserConstructionScript`))