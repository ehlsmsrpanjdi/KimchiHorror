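; BP_PuzzleKey is an interactable key in the puzzle level that advances the player's mortuary-key quest when picked up.
; On interact, it casts the player pawn to BP_MainPlayer, notifies the quest component with "FindMortuaryKey", then destroys itself.
; CanInteract and CanNotInteract toggle an outline overlay material on the static mesh.
; Its quest queries report no quest line and a non-quest object, despite that notification.
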(event `InteractionInterface.OnInteract`
  (params (Interactor :type "Actor Object Reference"))
  (bind _asbp_main_player (cast `/Game/Level/Stage_1Element/BP_MainPlayer` (`GameplayStatics.GetPlayerPawn` 0)))
  (`HorrorProtoKimchiCharacter.NotifyQuestComponent` _asbp_main_player "FindMortuaryKey")
  (`self.K2_DestroyActor`))

(event `InteractionInterface.CanNotInteract`
  (params (Interactor :type "Actor Object Reference"))
  (`MeshComponent.SetOverlayMaterial` (`self.StaticMesh`) null))

(event `InteractionInterface.CanInteract`
  (params (Interactor :type "Actor Object Reference"))
  (`MeshComponent.SetOverlayMaterial` (`self.StaticMesh`) "/Game/BP/Material/MT_OutLine.MT_OutLine"))

(fn `GetCurrentQuestLineName`
  (params (Interactor :type "Actor Object Reference"))
  (returns (ReturnValue :type Name))
  (return "None"))

(fn `IsQuestObject`
  (params (Interactor :type "Actor Object Reference"))
  (returns (ReturnValue :type Boolean))
  (return false))

(fn `UserConstructionScript`
  (`parent.UserConstructionScript`))