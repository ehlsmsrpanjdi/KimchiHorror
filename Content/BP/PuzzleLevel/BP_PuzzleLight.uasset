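; BP_PuzzleLight is an interactable puzzle actor that shows an outline overlay while interactable and rotates in fixed steps on each interaction.
; Its Box, made visible at BeginPlay, sets IsCorrect while BP_MainPlayer overlaps it and clears it on exit.
; It binds CheckAnswer to BindButton's action event, which prints a "correct" message (정답) when IsCorrect is true.
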(event `InteractionInterface.CanInteract`
  (params (Interactor :type "Actor Object Reference"))
  (`MeshComponent.SetOverlayMaterial` (`self.Mesh`) "/Game/BP/Material/MT_OutLine.MT_OutLine"))

(event `InteractionInterface.OnInteract`
  (params (Interactor :type "Actor Object Reference"))
  (`self.K2_AddActorWorldRotation` (struct :`Yaw` 30.0)))

(event `InteractionInterface.CanNotInteract`
  (params (Interactor :type "Actor Object Reference"))
  (`MeshComponent.SetOverlayMaterial` (`self.Mesh`) null))

(event `self.ReceiveBeginPlay`
  (`SceneComponent.SetHiddenInGame` (`self.Box`) false false)
  (add `C_Button.OnAction` (`self.BindButton`) (delegate `CheckAnswer`)))

(event `CheckAnswer`
  (if (`self.IsCorrect`)
    (`KismetSystemLibrary.PrintString` "정답")))

(event `self.Box.OnComponentBeginOverlap`
  (params (OverlappedComponent :type "PrimitiveComponent Object Reference") (OtherActor :type "Actor Object Reference") (OtherComp :type "PrimitiveComponent Object Reference") (OtherBodyIndex :type Integer) (bFromSweep :type Boolean) (SweepResult :type "HitResult Structure (by ref)"))
  (cast `/Game/Level/Stage_1Element/BP_MainPlayer` OtherActor)
  (set `self.IsCorrect` true))

(event `self.Box.OnComponentEndOverlap`
  (params (OverlappedComponent :type "PrimitiveComponent Object Reference") (OtherActor :type "Actor Object Reference") (OtherComp :type "PrimitiveComponent Object Reference") (OtherBodyIndex :type Integer))
  (cast `/Game/Level/Stage_1Element/BP_MainPlayer` OtherActor)
  (set `self.IsCorrect` false))

(fn `UserConstructionScript`)