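; BP_Telephone is an interactable phone in the puzzle level that rings on a timer after the player enters a start trigger.
; StartColl arms the delayed ring and removes itself; overlapping EndColl after that cancels the timer and destroys the audio.
; Interacting while audio plays swaps the ring for a one-time end sound, then destroys the audio component after a short delay.
; Its quest query functions report that it is not a quest object.
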(event `InteractionInterface.OnInteract`
  (params (Interactor :type "Actor Object Reference"))
  (bind _audio (`self.Audio`))
  (if (`AudioComponent.IsPlaying` _audio)
    (if (not (`self.bIsInteracted`))
      (`AudioComponent.Stop` _audio)
      (`AudioComponent.SetSound` _audio "/Game/Sound/PuzzleLevel/SO_PhoneEnd.SO_PhoneEnd")
      (`AudioComponent.Play` _audio 0.0)
      (set `self.bIsInteracted` true)
      (`KismetSystemLibrary.Delay` 3.0)
      (`ActorComponent.K2_DestroyComponent` _audio))))

(event `self.EndColl.OnComponentBeginOverlap`
  (params (OverlappedComponent :type "PrimitiveComponent Object Reference") (OtherActor :type "Actor Object Reference") (OtherComp :type "PrimitiveComponent Object Reference") (OtherBodyIndex :type Integer) (bFromSweep :type Boolean) (SweepResult :type "HitResult Structure (by ref)"))
  (cast `/Game/Level/Stage_1Element/BP_MainPlayer` OtherActor)
  (if (`self.bStarted`)
    (`KismetSystemLibrary.K2_ClearAndInvalidateTimerHandle` (`self.CallTimeHandle`))
    (`ActorComponent.K2_DestroyComponent` (`self.Audio`))))

(event `self.StartColl.OnComponentBeginOverlap`
  (params (OverlappedComponent :type "PrimitiveComponent Object Reference") (OtherActor :type "Actor Object Reference") (OtherComp :type "PrimitiveComponent Object Reference") (OtherBodyIndex :type Integer) (bFromSweep :type Boolean) (SweepResult :type "HitResult Structure (by ref)"))
  (cast `/Game/Level/Stage_1Element/BP_MainPlayer` OtherActor)
  (set `self.bStarted` true)
  (bind _returnvalue (`KismetSystemLibrary.K2_SetTimerDelegate` (delegate `TimeEvent`) 15.0))
  (set `self.CallTimeHandle` _returnvalue)
  (`ActorComponent.K2_DestroyComponent` (`self.StartColl`)))

(event `TimeEvent`
  (bind _audio (`self.Audio`))
  (`AudioComponent.SetSound` _audio "/Game/Sound/PuzzleLevel/SO_PhoneRing.SO_PhoneRing")
  (`AudioComponent.Play` _audio 0.0))

(fn `GetCurrentQuestLineName`
  (params (Interactor :type "Actor Object Reference"))
  (returns (ReturnValue :type Name))
  (return "None"))

(fn `IsQuestObject`
  (params (Interactor :type "Actor Object Reference"))
  (returns (ReturnValue :type Boolean))
  (return false))

(fn `UserConstructionScript`)