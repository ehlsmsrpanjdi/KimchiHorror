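; Trigger-volume actor that activates and later removes a linked counter nurse in the puzzle level.
; While its Trigger flag is set, the player entering Box passes their forward vector to the nurse, sets its Trigger, calls Check, then destroys Box.
; With the flag set, leaving OutBox, which is made visible at BeginPlay, destroys both the nurse and this actor.
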(event `self.ReceiveBeginPlay`
  (`SceneComponent.SetHiddenInGame` (`self.OutBox`) false false))

(event `self.Box.OnComponentBeginOverlap`
  (params (OverlappedComponent :type "PrimitiveComponent Object Reference") (OtherActor :type "Actor Object Reference") (OtherComp :type "PrimitiveComponent Object Reference") (OtherBodyIndex :type Integer) (bFromSweep :type Boolean) (SweepResult :type "HitResult Structure (by ref)"))
  (bind _as_bp_puzzle_counter_nurse (`self.As BP Puzzle Counter Nurse`))
  (if (`self.Trigger`)
    (cast `/Game/Level/Stage_1Element/BP_MainPlayer` OtherActor)
    (set `/Game/BP/PuzzleLevel/CounterNurse/BP_PuzzleCounterNurse.Trigger` true _as_bp_puzzle_counter_nurse)
    (set `/Game/BP/PuzzleLevel/CounterNurse/BP_PuzzleCounterNurse.CachedPlayerForward` (`self.GetActorForwardVector` (`GameplayStatics.GetPlayerPawn` 0)) _as_bp_puzzle_counter_nurse)
    (`/Game/BP/PuzzleLevel/CounterNurse/BP_PuzzleCounterNurse.Check` _as_bp_puzzle_counter_nurse)
    (`ActorComponent.K2_DestroyComponent` (`self.Box`))))

(event `self.OutBox.OnComponentEndOverlap`
  (params (OverlappedComponent :type "PrimitiveComponent Object Reference") (OtherActor :type "Actor Object Reference") (OtherComp :type "PrimitiveComponent Object Reference") (OtherBodyIndex :type Integer))
  (cast `/Game/Level/Stage_1Element/BP_MainPlayer` OtherActor)
  (if (`self.Trigger`)
    (`self.K2_DestroyActor` (`self.As BP Puzzle Counter Nurse`))
    (`self.K2_DestroyActor`)))

(fn `UserConstructionScript`)