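; Interactable puzzle light that outlines when it can be interacted with and rotates by a fixed step on each interaction.
; Its Box, shown in game, marks the answer correct while the player overlaps it.
; The bound button triggers the check: success fires clear events on the light manager and door, then unbinds the button.
; Failure calls the manager's normal jump scare, preceded by a unique one on a random roll.
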(event `InteractionInterface.CanInteract`
  (params (Interactor :type "Actor Object Reference"))
  (`MeshComponent.SetOverlayMaterial` (`self.Mesh`) "/Game/BP/Material/MT_OutLine.MT_OutLine"))

(event `InteractionInterface.OnInteract`
  (params (Interactor :type "Actor Object Reference"))
  (`self.K2_AddActorWorldRotation` (struct :`Yaw` 30.0)))

(event `InteractionInterface.CanNotInteract`
  (params (Interactor :type "Actor Object Reference"))
  (`MeshComponent.SetOverlayMaterial` (`self.Mesh`) null))

(event `self.ReceiveBeginPlay`
  (bind _bindbutton (`self.BindButton`))
  (`SceneComponent.SetHiddenInGame` (`self.Box`) false false)
  (if (`KismetSystemLibrary.IsValid` _bindbutton)
    (add `C_Button.OnAction` _bindbutton (delegate `CheckAnswer`))))

(event `CheckAnswer`
  (bind _bp_puzzledoor (`self.BP_PuzzleDoor`))
  (bind _as_bp_puzzle_light_manager (`self.As BP Puzzle Light Manager`))
  (if (`self.IsCorrect`)
    (if (`KismetSystemLibrary.IsValid` _bp_puzzledoor)
      (`/Game/BP/PuzzleLevel/PuzzleLight/BP_PuzzleLightManager.ClearEvent` (`self.As BP Puzzle Light Manager`))
      (`/Game/BP/PuzzleLevel/BP_PuzzleDoor.ClearEvent` _bp_puzzledoor)
      (clear `C_Button.OnAction` (`self.BindButton`)))
    (else
      (bind _returnvalue (`C_KimchiHelper.GetRandomInteger` 1 5))
      (if (== _returnvalue 1)
        (`/Game/BP/PuzzleLevel/PuzzleLight/BP_PuzzleLightManager.UniqueJumpScare` _as_bp_puzzle_light_manager))
      (`/Game/BP/PuzzleLevel/PuzzleLight/BP_PuzzleLightManager.NormalJumpScare` _as_bp_puzzle_light_manager))))

(event `self.Box.OnComponentBeginOverlap`
  (params (OverlappedComponent :type "PrimitiveComponent Object Reference") (OtherActor :type "Actor Object Reference") (OtherComp :type "PrimitiveComponent Object Reference") (OtherBodyIndex :type Integer) (bFromSweep :type Boolean) (SweepResult :type "HitResult Structure (by ref)"))
  (cast `/Game/Level/Stage_1Element/BP_MainPlayer` OtherActor)
  (set `self.IsCorrect` true))

(event `self.Box.OnComponentEndOverlap`
  (params (OverlappedComponent :type "PrimitiveComponent Object Reference") (OtherActor :type "Actor Object Reference") (OtherComp :type "PrimitiveComponent Object Reference") (OtherBodyIndex :type Integer))
  (cast `/Game/Level/Stage_1Element/BP_MainPlayer` OtherActor)
  (set `self.IsCorrect` false))

(fn `GetCurrentQuestLineName`
  (params (Interactor :type "Actor Object Reference"))
  (returns (ReturnValue :type Name))
  (return "None"))

(fn `IsQuestObject`
  (params (Interactor :type "Actor Object Reference"))
  (returns (ReturnValue :type Boolean))
  (return false))

(fn `UserConstructionScript`)