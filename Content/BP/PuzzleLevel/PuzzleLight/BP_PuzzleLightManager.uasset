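; Manager actor for the light puzzle that tracks registered light entities and handles the puzzle's clear, disable and jump scare events.
; AddEntity fills the entity list, and the clear event snaps each entity to the location and rotation of the matching one of five arrow markers by index.
; The disable event deactivates every entity.
; The unique jump scare spawns through the player and is destroyed after a delay, while the normal one only prints.
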(event `self.ReceiveBeginPlay`
  (`KismetArrayLibrary.Array_Add` (`self.ArrowArray`) (`self.Arrow`))
  (`KismetArrayLibrary.Array_Add` (`self.ArrowArray`) (`self.Arrow1`))
  (`KismetArrayLibrary.Array_Add` (`self.ArrowArray`) (`self.Arrow2`))
  (`KismetArrayLibrary.Array_Add` (`self.ArrowArray`) (`self.Arrow3`))
  (`KismetArrayLibrary.Array_Add` (`self.ArrowArray`) (`self.Arrow4`)))

(event `AddEntity`
  (params (NewItem :type "/Game/BP/PuzzleLevel/PuzzleLight/BP_PuzzleLightEntity Object Reference (by ref)"))
  (`KismetArrayLibrary.Array_Add` (`self.As BP Puzzle Light Entity`) NewItem))

(event `NormalJumpScare`
  (`KismetSystemLibrary.PrintString` "노말"))

(event `UniqueJumpScare`
  (bind _asbp_main_player (cast `/Game/Level/Stage_1Element/BP_MainPlayer` (`GameplayStatics.GetPlayerPawn` 0)))
  (`KismetSystemLibrary.PrintString` "유니크")
  (bind _returnvalue (`/Game/Level/Stage_1Element/BP_MainPlayer.JumpScare` _asbp_main_player null null))
  (`KismetSystemLibrary.Delay` 2.0)
  (`self.K2_DestroyActor` _returnvalue))

(event `ClearEvent`
  (for (_array_element _array_index) (`self.ArrowArray`)
    (bind _output (`|GetArrayItem` (`self.As BP Puzzle Light Entity`) _array_index))
    (`self.K2_SetActorLocation` _output (`SceneComponent.K2_GetComponentLocation` _array_element) false false)
    (`self.K2_SetActorRotation` _output (`SceneComponent.K2_GetComponentRotation` _array_element) false)))

(event `DisableEvent`
  (for _array_element (`self.As BP Puzzle Light Entity`)
    (`C_EntityBase.SetActiveFalse` _array_element)))

(fn `UserConstructionScript`)