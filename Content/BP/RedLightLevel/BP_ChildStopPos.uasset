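; BP_ChildStopPos is a trigger actor in the Red Light level that ends the child encounter when the player reaches it.
; When the player pawn overlaps its box, it destroys the referenced Child actor and itself, then calls CloseDoor on a referenced door.
; It finally casts the player to BP_MainPlayer and notifies its quest component with the "SurviveChild" key.
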(event `self.Box.OnComponentBeginOverlap`
  (params (OverlappedComponent :type "PrimitiveComponent Object Reference") (OtherActor :type "Actor Object Reference") (OtherComp :type "PrimitiveComponent Object Reference") (OtherBodyIndex :type Integer) (bFromSweep :type Boolean) (SweepResult :type "HitResult Structure (by ref)"))
  (if (== OtherActor (`GameplayStatics.GetPlayerPawn` 0))
    (`self.K2_DestroyActor` (`self.Child`))
    (`self.K2_DestroyActor`)
    (`/Game/BP/Common/BP_DoorBase.CloseDoor` (`self.CloseDoor`))
    (bind _asbp_main_player (cast `/Game/Level/Stage_1Element/BP_MainPlayer` (`GameplayStatics.GetPlayerPawn` 0)))
    (`HorrorProtoKimchiCharacter.NotifyQuestComponent` _asbp_main_player "SurviveChild")))

(fn `UserConstructionScript`)