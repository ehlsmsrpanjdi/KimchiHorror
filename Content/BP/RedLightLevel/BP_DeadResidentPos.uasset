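; BP_DeadResidentPos is a trigger volume in the RedLightLevel that repositions a resident when the player enters it.
; On the first overlap by the player pawn with its Box, it sets TempStop on a referenced Child and calls MoveActor on the Resident with the Arrow component's world location.
; An IsOverlap flag makes it fire only once.
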(event `self.Box.OnComponentBeginOverlap`
  (params (OverlappedComponent :type "PrimitiveComponent Object Reference") (OtherActor :type "Actor Object Reference") (OtherComp :type "PrimitiveComponent Object Reference") (OtherBodyIndex :type Integer) (bFromSweep :type Boolean) (SweepResult :type "HitResult Structure (by ref)"))
  (if (`self.IsOverlap`)
    _
    (elif (== OtherActor (`GameplayStatics.GetPlayerPawn` 0))
      (set `self.IsOverlap` true)
      (set `C_RedLightChild.TempStop` true (`self.Child`))
      (`/Game/BP/RedLightLevel/BP_RedLightResident.MoveActor` (`self.Resident`) (`SceneComponent.K2_GetComponentLocation` (`self.Arrow`))))))

(fn `UserConstructionScript`)