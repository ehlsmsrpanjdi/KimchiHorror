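; Child character that runs a Red Light, Green Light (Mugunghwa) game against the player, starting shortly after BeginPlay.
; Until touched, Tick polls the player movement check and prints a debug message when it fails.
; Interacting stops the game, flags the child as touched and sets EndGame on its AnimBP, after which Tick moves it toward the player.
; Player collision overlap only prints a caught message, and destruction also stops the game.
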(event `self.ReceiveBeginPlay`
  (`KismetSystemLibrary.Delay` 5.0)
  (`self.PlayRedLight`)
  (`self.SetDirectionToForward`))

(event `self.ReceiveTick`
  (params (DeltaSeconds :type "Float (single-precision)"))
  (set `self.Speed` (`KismetMathLibrary.VSize` (`MovementComponent.Velocity` (`self.CharacterMovement`))))
  (if (`self.IsTouch`)
    (`C_KimchiHelper.MoveToActorAndCheckArrival` self (`self.Player`))
    (`self.SetDirectionToForward`)
    (else
      (bind _returnvalue (`self.CheckPlayerMove`))
      (if (not _returnvalue)
        (`KismetSystemLibrary.PrintString` "무궁화 중 움직임")))))

(event `self.ReceiveDestroyed`
  (`self.StopRedLightGame`))

(event `InteractionInterface.OnInteract`
  (params (Interactor :type "Actor Object Reference"))
  (if (not (`self.IsTouch`))
    (`self.StopRedLightGame`)
    (`KismetSystemLibrary.Delay` 0.5)
    (set `self.IsTouch` true)
    (`self.SetDirectionToForward`)
    (bind _asabp_red_light_child (cast `/Game/BP/RedLightLevel/RedLightChild/ABP_RedLightChild` (`SkeletalMeshComponent.GetAnimInstance` (`self.Mesh`))))
    (set `/Game/BP/RedLightLevel/RedLightChild/ABP_RedLightChild.EndGame` true _asabp_red_light_child)))

(event `InteractionInterface.CanInteract`
  (params (Interactor :type "Actor Object Reference"))
  (`KismetSystemLibrary.PrintString` "닿음"))

(event `self.PlayerCol.OnComponentBeginOverlap`
  (params (OverlappedComponent :type "PrimitiveComponent Object Reference") (OtherActor :type "Actor Object Reference") (OtherComp :type "PrimitiveComponent Object Reference") (OtherBodyIndex :type Integer) (bFromSweep :type Boolean) (SweepResult :type "HitResult Structure (by ref)"))
  (if (== OtherActor (`self.Player`))
    (`KismetSystemLibrary.PrintString` "잡힘")))

(event `InteractionInterface.CanNotInteract`
  (params (Interactor :type "Actor Object Reference"))
  (`KismetSystemLibrary.PrintString` "안닿음"))

(fn `UserConstructionScript`)