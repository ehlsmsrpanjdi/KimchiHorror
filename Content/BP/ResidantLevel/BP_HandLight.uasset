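; BP_HandLight is a hand light actor whose Box volume switches BP_InterNurseHalusi actors between ticking and dormant.
; On begin overlap it enables tick on that actor, its Face and its Mesh; on end overlap it disables all three, halting their per-frame updates outside the box.
; BeginPlay makes the Box visible in game, and each switch prints a debug string.
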(event `self.ReceiveBeginPlay`
  (`SceneComponent.SetHiddenInGame` (`self.Box`) false false))

(event `self.Box.OnComponentBeginOverlap`
  (params (OverlappedComponent :type "PrimitiveComponent Object Reference") (OtherActor :type "Actor Object Reference") (OtherComp :type "PrimitiveComponent Object Reference") (OtherBodyIndex :type Integer) (bFromSweep :type Boolean) (SweepResult :type "HitResult Structure (by ref)"))
  (bind _asbp_inter_nurse_halusi (cast `/Game/BP/ResidantLevel/BP_InterNurseHalusi` OtherActor))
  (`ActorComponent.SetComponentTickEnabled` (`/Game/BP/ResidantLevel/BP_InterNurseHalusi.Face` _asbp_inter_nurse_halusi) true)
  (`self.SetActorTickEnabled` _asbp_inter_nurse_halusi true)
  (`ActorComponent.SetComponentTickEnabled` (`Character.Mesh` _asbp_inter_nurse_halusi) true)
  (`KismetSystemLibrary.PrintString` "닿음"))

(event `self.Box.OnComponentEndOverlap`
  (params (OverlappedComponent :type "PrimitiveComponent Object Reference") (OtherActor :type "Actor Object Reference") (OtherComp :type "PrimitiveComponent Object Reference") (OtherBodyIndex :type Integer))
  (bind _asbp_inter_nurse_halusi (cast `/Game/BP/ResidantLevel/BP_InterNurseHalusi` OtherActor))
  (`ActorComponent.SetComponentTickEnabled` (`/Game/BP/ResidantLevel/BP_InterNurseHalusi.Face` _asbp_inter_nurse_halusi) false)
  (`self.SetActorTickEnabled` _asbp_inter_nurse_halusi false)
  (`ActorComponent.SetComponentTickEnabled` (`Character.Mesh` _asbp_inter_nurse_halusi) false)
  (`KismetSystemLibrary.PrintString` "비활성화"))

(fn `UserConstructionScript`)