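; Interactable hallucination nurse for the resident level, with correct and wrong reveal reactions that change face, gaze, materials and, when wrong, body pose.
; On BeginPlay it picks a chair, bed or default pose, closes its eyes, registers with BP_ResidentState by phase and goes dormant.
; Tick runs face and shake timers, with Shake alternating head tilts.
; Expressions, eye movement and look-at route through face, post-process and body AnimBPs, while clothing follows the body via leader pose.
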(event `self.ReceiveBeginPlay`
  (bind _dormantincludemeshes (`self.DormantIncludeMeshes`))
  (bind _as_bp_sequence_helper (`self.As BP Sequence Helper`))
  (`parent.ReceiveBeginPlay`)
  (bind _asbp_main_player (cast `/Game/Level/Stage_1Element/BP_MainPlayer` (`GameplayStatics.GetPlayerPawn` 0)))
  (set `self.Player` _asbp_main_player)
  (if (`self.IsChair`)
    (`self.SetBody` "NewEnumerator0")
    (elif (`self.IsBed`)
      (`self.SetBody` "NewEnumerator1")
      (else
        (`self.SetBody` "NewEnumerator2"))))
  (`/Game/BP/Stage1/InteractiveEntity/AnimIns/BPI_EntityMoveInter.ISetFaceMove` "CloseEye")
  (bind _asbp_entity_face_anim (cast `/Game/BP/Stage1/InteractiveEntity/AnimIns/Face/BP_EntityFaceAnim` (`SkeletalMeshComponent.GetAnimInstance` (`self.Face`))))
  (set `/Game/BP/Stage1/InteractiveEntity/AnimIns/Face/BP_EntityFaceAnim.IsTingle` false _asbp_entity_face_anim)
  (`/Game/BP/Stage1/InteractiveEntity/AnimIns/Face/BP_EntityFaceAnim.SetMoodIntensity` _asbp_entity_face_anim 0.9)
  (bind _asbp_resident_state (cast `/Game/BP/ResidantLevel/BP_ResidentState` (`GameplayStatics.GetGameState`)))
  (bind _output_get (set `self.GameState` _asbp_resident_state))
  (`C_ResidentGameState.AddNurseAboutPhaseNumber` _output_get self)
  (`self.Eye` "NewEnumerator1")
  (`SceneComponent.K2_AttachToComponent` (`self.Medicine`) (`self.Mesh`) "ItemSocket" "KeepRelative" "KeepRelative" "KeepRelative" true)
  (`KismetArrayLibrary.Array_Add` _dormantincludemeshes (`self.Mesh`))
  (`KismetArrayLibrary.Array_Add` _dormantincludemeshes (`self.Face`))
  (`self.SleepMode`)
  (if (`KismetSystemLibrary.IsValid` _as_bp_sequence_helper)
    (set `self.SequenceHelper` _as_bp_sequence_helper)))

(event `FollowP`
  (`self.SetBody` "NewEnumerator3")
  (`/Game/BP/Stage1/InteractiveEntity/AnimIns/BPI_EntityMoveInter.ISetFaceMove` "MadLaugh" "MadLaugh"))

(event `self.ReceiveTick`
  (params (DeltaSeconds :type "Float (single-precision)"))
  (`self.CalculateFace` DeltaSeconds)
  (bind _returnvalue (`self.CalculateShaking` DeltaSeconds))
  (if _returnvalue
    (`self.Shake`)))

(event `self.ISetFaceMove`
  (params (Pose :type "C_FacePoseEnum Enum" :default "Idle") (Mood :type "C_FaceMoodEnum Enum" :default "Normal") (Interval :type "Float (double-precision)"))
  ;[1 1 1] 기본 ㅅ
  (bind _asbp_entity_face_anim (cast `/Game/BP/Stage1/InteractiveEntity/AnimIns/Face/BP_EntityFaceAnim` (`SkeletalMeshComponent.GetAnimInstance` (`self.Face`)))
    (:`then`
      (`C_AnimBPBase.SetFacePose` _asbp_entity_face_anim Pose Mood Interval))
    (:`CastFailed`
      (`KismetSystemLibrary.PrintString` "FaceMissing"))))

(event `self.ISetHeadTilting`
  (params (DesVector :type "Vector Structure") (RotateSpeed :type "Float (double-precision)"))
  ;[1 1 1] 기본 ㅅ
  (bind _asbp_hnurse_body_anim (cast `/Game/BP/ResidantLevel/BP_HNurseBodyAnim` (`SkeletalMeshComponent.GetAnimInstance` (`self.Mesh`)))
    (:`then`
      (`C_EntityAnimBase.LerfTiltHead` _asbp_hnurse_body_anim DesVector RotateSpeed))
    (:`CastFailed`
      (`KismetSystemLibrary.PrintString` "TiltingMissing"))))

(event `Eye`
  (params (`On/Off` :type "/Game/BP/Stage1/InteractiveEntity/AnimIns/Body/BP_LookAtEnum Enum" :default "NewEnumerator0"))
  ;[1 1 1] 눈 목 돌리기
  (bind _asabp_face_post_process (cast `/Game/MetaHumans/Common/Face/ABP_Face_PostProcess` (`SkeletalMeshComponent.GetPostProcessInstance` (`self.Face`))))
  (`/Game/MetaHumans/Common/Face/ABP_Face_PostProcess.EyeMoveOnOff` _asabp_face_post_process `On/Off`))

(event `self.ISetBodyMove`
  (params (Move :type "C_EntityMoveEnum Enum" :default "Idle"))
  ;[1 1 1] 기본 ㅅ
)

(event `Look`
  (params (`On/Off` :type "/Game/BP/Stage1/InteractiveEntity/AnimIns/Body/BP_LookAtEnum Enum" :default "NewEnumerator0"))
  ;[1 1 1] 눈 목 돌리기
  (bind _asbp_hnurse_body_anim (cast `/Game/BP/ResidantLevel/BP_HNurseBodyAnim` (`SkeletalMeshComponent.GetAnimInstance` (`self.Mesh`))))
  (`/Game/BP/ResidantLevel/BP_HNurseBodyAnim.LookAtSwitch` _asbp_hnurse_body_anim `On/Off`))

(event `SetBody`
  (params (Enum :type "/Game/BP/ResidantLevel/BP_HNurseBodyEnum Enum" :default "NewEnumerator0"))
  ;[1 1 1] 기본 ㅅ
  (bind _asbp_hnurse_body_anim (cast `/Game/BP/ResidantLevel/BP_HNurseBodyAnim` (`SkeletalMeshComponent.GetAnimInstance` (`self.Mesh`))))
  (set `/Game/BP/ResidantLevel/BP_HNurseBodyAnim.Enum` Enum _asbp_hnurse_body_anim))

(event `self.Shake`
  ;[1 1 1] 대가리 쉐이킷
  (if (`self.bCanShake`)
    (set `self.bCanShake` false)
    (`/Game/BP/Stage1/InteractiveEntity/AnimIns/BPI_EntityMoveInter.ISetHeadTilting` (1800.0 1800.0 1800.0) 3.0)
    (set `self.CurrentTime` 4.0)
    (else
      (set `self.bCanShake` true)
      (`/Game/BP/Stage1/InteractiveEntity/AnimIns/BPI_EntityMoveInter.ISetHeadTilting` (-1800.0 -1800.0 -1800.0) 3.0)
      (set `self.CurrentTime` 4.0)))
  (`/Game/BP/Stage1/InteractiveEntity/AnimIns/BPI_EntityMoveInter.ISetFaceMove` "CloseEye")
  (set `self.FaceCurrentTime` 0.0))

(event `self.FaceFunction`
  ;[1 1 1] 대가리 쉐이킷
  (if (`self.bIsTrueNS`)
    (`/Game/BP/Stage1/InteractiveEntity/AnimIns/BPI_EntityMoveInter.ISetFaceMove` "Idle" "Anger")
    (else
      (`/Game/BP/Stage1/InteractiveEntity/AnimIns/BPI_EntityMoveInter.ISetFaceMove` "Idle" "MadLaugh"))))

(event `InteractionInterface.OnInteract`
  (params (Interactor :type "Actor Object Reference"))
  ;[1 1 1] 상호작용
  (`self.InteractionEvent`))

(event `self.Sneer`
  ;[1 1 1] 대가리 쉐이킷
  (`/Game/BP/Stage1/InteractiveEntity/AnimIns/BPI_EntityMoveInter.ISetHeadTilting` (-3600.0 3600.0 3600.0) 3.0)
  (`self.ISetFaceMove` "MadLaugh" "MadLaugh"))

(event `self.CorrectNurse`
  (`self.ISetFaceMove` "Talk" "Anger")
  (`self.Eye` "NewEnumerator0")
  (`self.Look` "NewEnumerator1")
  (for _index (range 1 3)
    (`PrimitiveComponent.SetMaterial` (`self.Face`) _index "/Game/ArtWorkOnGit/Object/MT_Hanger.MT_Hanger")
    (set `self.InteractionMassage` "" :!label _label)))

(event `self.WrongNurse`
  (`self.SetBody` "NewEnumerator4")
  (`self.ISetFaceMove` "MadLaugh" "MadLaugh")
  (`self.Eye` "NewEnumerator0")
  (`self.Look` "NewEnumerator1")
  (for _index (range 1 3)
    (`PrimitiveComponent.SetMaterial` (`self.Face`) _index "/Game/ArtWorkOnGit/Object/MT_Hanger.MT_Hanger")
    (goto _label)))

(fn `CloseEye`
  (`self.ISetHeadTilting` (-1800.0 -1800.0 -1800.0) 3.0)
  (`/Game/BP/Stage1/InteractiveEntity/AnimIns/BPI_EntityMoveInter.ISetFaceMove` "CloseEye"))

(fn `OpenEye`
  (`self.ISetHeadTilting` (1800.0 1800.0 1800.0) 3.0)
  (`/Game/BP/Stage1/InteractiveEntity/AnimIns/BPI_EntityMoveInter.ISetFaceMove` "Idle" "MadLaugh"))

(fn `UserConstructionScript`
  (`SkinnedMeshComponent.SetLeaderPoseComponent` (`self.Clothes`) (`self.Mesh`) false false)
  (`SkinnedMeshComponent.SetLeaderPoseComponent` (`self.Gloves`) (`self.Mesh`) false false)
  (`SkinnedMeshComponent.SetLeaderPoseComponent` (`self.Arms`) (`self.Mesh`) false false)
  (`SkinnedMeshComponent.SetLeaderPoseComponent` (`self.Pants`) (`self.Mesh`) false false))