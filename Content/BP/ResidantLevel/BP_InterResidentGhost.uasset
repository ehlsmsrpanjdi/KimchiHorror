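; Resident-level ghost character that chases the player every tick and prints a caught message on arrival.
; Once Phase1Start fires, timers escalate it through four phases, each pausing for a scream before switching to a new looping animation and higher walk speed.
; It registers itself with BP_ResidentState; body-move calls reach the anim blueprint, but face and head-tilt logic is disconnected.
; The construction script makes modular outfit meshes follow the body's pose.
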(event `self.ReceiveBeginPlay`
  (`parent.ReceiveBeginPlay`)
  (set `self.MyFace` (`self.Face`))
  (`self.ISetFaceMove` "AngerYelling" "Anger")
  (bind _asbp_resident_state (cast `/Game/BP/ResidantLevel/BP_ResidentState` (`GameplayStatics.GetGameState`)))
  (set `/Game/BP/ResidantLevel/BP_ResidentState.Resi` self _asbp_resident_state))

(event `self.ISetFaceMove`
  (params (Pose :type "C_FacePoseEnum Enum" :default "Idle") (Mood :type "C_FaceMoodEnum Enum" :default "Normal") (Interval :type "Float (double-precision)")))

(event `Phase 1 Start`
  (bind _charactermovement (`self.CharacterMovement`))
  (bind _mesh (`self.Mesh`))
  (set `CharacterMovementComponent.MaxWalkSpeed` 0.0 _charactermovement)
  (`SkeletalMeshComponent.PlayAnimation` _mesh "/Game/BP/ResidantLevel/Zombie_Scream.Zombie_Scream" false)
  (`KismetSystemLibrary.Delay` 3.0)
  (`SkeletalMeshComponent.PlayAnimation` _mesh "/Game/BP/ResidantLevel/SlowUpsetWalking.SlowUpsetWalking" true)
  (set `CharacterMovementComponent.MaxWalkSpeed` 100.0 _charactermovement)
  (`KismetSystemLibrary.K2_SetTimerDelegate` (delegate `Phase2`) 120.0))

(event `self.ISetHeadTilting`
  (params (DesVector :type "Vector Structure") (RotateSpeed :type "Float (double-precision)")))

(event `Phase2`
  (bind _charactermovement (`self.CharacterMovement`))
  (bind _mesh (`self.Mesh`))
  (set `CharacterMovementComponent.MaxWalkSpeed` 0.0 _charactermovement)
  (`SkeletalMeshComponent.PlayAnimation` _mesh "/Game/BP/ResidantLevel/Zombie_Scream.Zombie_Scream" false)
  (`KismetSystemLibrary.Delay` 3.0)
  (`SkeletalMeshComponent.PlayAnimation` _mesh "/Game/BP/ResidantLevel/NormalUpsetWalking.NormalUpsetWalking" true)
  (set `CharacterMovementComponent.MaxWalkSpeed` 200.0 _charactermovement)
  (`KismetSystemLibrary.K2_SetTimerDelegate` (delegate `Phase3`) 120.0))

(event `self.ReceiveTick`
  (params (DeltaSeconds :type "Float (single-precision)"))
  (bind _returnvalue (`C_KimchiHelper.MoveToActorAndCheckArrival` self (`GameplayStatics.GetPlayerPawn` 0) 50.0 true))
  (if _returnvalue
    (`KismetSystemLibrary.PrintString` "당신은 아이엠규민에게 당했습니다")))

(event `Phase3`
  (bind _charactermovement (`self.CharacterMovement`))
  (bind _mesh (`self.Mesh`))
  (set `CharacterMovementComponent.MaxWalkSpeed` 0.0 _charactermovement)
  (`SkeletalMeshComponent.PlayAnimation` _mesh "/Game/BP/ResidantLevel/Zombie_Scream.Zombie_Scream" false)
  (`KismetSystemLibrary.Delay` 3.0)
  (`SkeletalMeshComponent.PlayAnimation` _mesh "/Game/BP/ResidantLevel/FastUpsetWalking.FastUpsetWalking" true)
  (set `CharacterMovementComponent.MaxWalkSpeed` 300.0 _charactermovement)
  (`KismetSystemLibrary.K2_SetTimerDelegate` (delegate `EndPhase`) 120.0))

(event `self.ISetBodyMove`
  (params (Move :type "C_EntityMoveEnum Enum" :default "Idle"))
  (bind _asbp_male_entity_body_anim (cast `/Game/BP/Stage1/InteractiveEntity/AnimIns/Body/BP_MaleEntityBodyAnim` (`SkeletalMeshComponent.GetAnimInstance` (`self.Mesh`)))
    (:`then`
      (`C_EntityAnimBase.SetBodyMove` _asbp_male_entity_body_anim Move))
    (:`CastFailed`
      (`KismetSystemLibrary.PrintString` "BodyMissing"))))

(event `EndPhase`
  (bind _charactermovement (`self.CharacterMovement`))
  (bind _mesh (`self.Mesh`))
  (set `CharacterMovementComponent.MaxWalkSpeed` 0.0 _charactermovement)
  (`SkeletalMeshComponent.PlayAnimation` _mesh "/Game/BP/ResidantLevel/Zombie_Scream.Zombie_Scream" false)
  (`KismetSystemLibrary.Delay` 3.0)
  (`SkeletalMeshComponent.PlayAnimation` _mesh "/Game/BP/ResidantLevel/TopBlade.TopBlade" true)
  (set `CharacterMovementComponent.MaxWalkSpeed` 400.0 _charactermovement))

(fn `UserConstructionScript`
  (`SkinnedMeshComponent.SetLeaderPoseComponent` (`self.Clothes`) (`self.Mesh`) false false)
  (`SkinnedMeshComponent.SetLeaderPoseComponent` (`self.Backpack`) (`self.Mesh`) false false)
  (`SkinnedMeshComponent.SetLeaderPoseComponent` (`self.Armor`) (`self.Mesh`) false false)
  (`SkinnedMeshComponent.SetLeaderPoseComponent` (`self.Gloves`) (`self.Mesh`) false false)
  (`SkinnedMeshComponent.SetLeaderPoseComponent` (`self.Arm_Module_Right`) (`self.Mesh`) false false)
  (`SkinnedMeshComponent.SetLeaderPoseComponent` (`self.Patch_L_Arm`) (`self.Mesh`) false false)
  (`SkinnedMeshComponent.SetLeaderPoseComponent` (`self.Hip_Right`) (`self.Mesh`) false false)
  (`SkinnedMeshComponent.SetLeaderPoseComponent` (`self.Gasmask`) (`self.Mesh`) false false)
  (`SkinnedMeshComponent.SetLeaderPoseComponent` (`self.Balaclava`) (`self.Mesh`) false false)
  (`SkinnedMeshComponent.SetLeaderPoseComponent` (`self.Hat`) (`self.Mesh`) false false)
  (`SkinnedMeshComponent.SetLeaderPoseComponent` (`self.Hip_Left`) (`self.Mesh`) false false)
  (`SkinnedMeshComponent.SetLeaderPoseComponent` (`self.Patch_Cap`) (`self.Mesh`) false false)
  (`SkinnedMeshComponent.SetLeaderPoseComponent` (`self.Helmet_Drops`) (`self.Mesh`) false false)
  (`SkinnedMeshComponent.SetLeaderPoseComponent` (`self.Scarf`) (`self.Mesh`) false false)
  (`SkinnedMeshComponent.SetLeaderPoseComponent` (`self.Patch_Helmetn`) (`self.Mesh`) false false)
  (`SkinnedMeshComponent.SetLeaderPoseComponent` (`self.Bulletproof`) (`self.Mesh`) false false)
  (`SkinnedMeshComponent.SetLeaderPoseComponent` (`self.Arms`) (`self.Mesh`) false false)
  (`SkinnedMeshComponent.SetLeaderPoseComponent` (`self.Preset`) (`self.Mesh`) false false)
  (`SkinnedMeshComponent.SetLeaderPoseComponent` (`self.Bulletproof_Drops`) (`self.Mesh`) false false)
  (`SkinnedMeshComponent.SetLeaderPoseComponent` (`self.Helmet_Headphones`) (`self.Mesh`) false false)
  (`SkinnedMeshComponent.SetLeaderPoseComponent` (`self.Helmet_Module`) (`self.Mesh`) false false)
  (`SkinnedMeshComponent.SetLeaderPoseComponent` (`self.Tactical_Belt`) (`self.Mesh`) false false)
  (`SkinnedMeshComponent.SetLeaderPoseComponent` (`self.Pants`) (`self.Mesh`) false false)
  (`SkinnedMeshComponent.SetLeaderPoseComponent` (`self.Helmet`) (`self.Mesh`) false false)
  (`SkinnedMeshComponent.SetLeaderPoseComponent` (`self.Glasses`) (`self.Mesh`) false false)
  (`SkinnedMeshComponent.SetLeaderPoseComponent` (`self.Headphones`) (`self.Mesh`) false false)
  (`SkinnedMeshComponent.SetLeaderPoseComponent` (`self.Patch_Back`) (`self.Mesh`) false false)
  (`SkinnedMeshComponent.SetLeaderPoseComponent` (`self.Patch_R_Arm`) (`self.Mesh`) false false)
  (`SkinnedMeshComponent.SetLeaderPoseComponent` (`self.Hair_1`) (`self.Mesh`) false false)
  (`SkinnedMeshComponent.SetLeaderPoseComponent` (`self.Watch`) (`self.Mesh`) false false))