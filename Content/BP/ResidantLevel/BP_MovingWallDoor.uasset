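; BP_MovingWallDoor is a wall door for the resident level that slides a cube between its starting position and an arrow marker.
; OpenDoor plays a timeline that lerps the cube from the location cached at BeginPlay to the arrow, and CloseDoor reverses it.
; InitSelf casts the game state to BP_ResidentState and switches on MyNum, but its door-reference assignments are disconnected.
; A separate MoveVertical function sets the cube's world Y, zeroing X and Z.
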(event `self.ReceiveBeginPlay`
  (`self.InitSelf`)
  (set `self.DefaultLoca` (`SceneComponent.K2_GetComponentLocation` (`self.Cube`))))

(event `InitSelf`
  (cast `/Game/BP/ResidantLevel/BP_ResidentState` (`GameplayStatics.GetGameState`))
  (switch `/Game/BP/ResidantLevel/BP_ResiNsPhaseEnum` (`self.MyNum`)))

(event `OpenDoor`
  (bind (_direction `_새_트랙_0`) (`Timeline|타임라인` :!via `PlayFromStart` :!label _label)
    (:`Update`
      (`SceneComponent.K2_SetWorldLocation` (`self.Cube`) (`KismetMathLibrary.VLerp` (`self.DefaultLoca`) (`SceneComponent.K2_GetComponentLocation` (`self.Arrow`)) `_새_트랙_0`) false false))))

(event `CloseDoor`
  (goto _label :!via `ReverseFromEnd`))

(fn `MoveVertical`
  (params (NewParam :type "Float (double-precision)"))
  (`SceneComponent.K2_SetWorldLocation` (`self.Cube`) (`KismetMathLibrary.MakeVector` 0.0 NewParam) false false))

(fn `UserConstructionScript`)