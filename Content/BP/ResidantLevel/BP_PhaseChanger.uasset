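; BP_PhaseChanger is a one-shot overlap trigger that advances the Resident level to a configured phase when the player enters it.
; On the first overlap by BP_MainPlayer, it sets IsWorked, closes the linked MyDoor if valid, and passes MyPhase to BP_ResidentState's ChangePhase through the game state.
; Overlaps by other actors before it fires only print a debug string.
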(event `self.ReceiveActorBeginOverlap`
  (params (OtherActor :type "Actor Object Reference"))
  (bind _mydoor (`self.MyDoor`))
  (if (not (`self.IsWorked`))
    (cast `/Game/Level/Stage_1Element/BP_MainPlayer` OtherActor
      (:`then`
        (set `self.IsWorked` true)
        (`/Engine/EditorBlueprintResources/StandardMacros.IsValid` _mydoor
          (:`Is Valid`
            (`/Game/BP/ResidantLevel/BP_MovingWallDoor.CloseDoor` _mydoor))
          (:`Is Not Valid`
            _))
        (bind _asbp_resident_state (cast `/Game/BP/ResidantLevel/BP_ResidentState` (`GameplayStatics.GetGameState`)))
        (`/Game/BP/ResidantLevel/BP_ResidentState.ChangePhase` _asbp_resident_state (`self.MyPhase`)))
      (:`CastFailed`
        (`KismetSystemLibrary.PrintString` "이거여?")))))

(fn `UserConstructionScript`)