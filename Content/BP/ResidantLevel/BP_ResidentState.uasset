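; Resident level state manager that runs the phased search for angry nurses.
; Game start activates phase one, randomly flags three via SetRandomThreeSetTrue and sets the angry nurse count.
; When all are found, it force-opens the phase one or two door, then advances the phase and repeats that setup.
; Restart clears the doubts manager and reloads the level, while losing all lives only prints a death message.
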(event `self.GameStart`
  (`self.SetRandomThreeSetTrue` 1)
  (`self.SetNextPhase` 1)
  (set `self.CurrentPhase` 1)
  (set `self.AngryNurseCount` 3))

(event `self.FindAllAngry`
  (bind _currentphase (`self.CurrentPhase`))
  (bind _returnvalue (+ _currentphase 1))
  ;[1 1 1] 모든 화난놈찾기
  (switch `int` (`self.CurrentPhase`)
    (:`1`
      (`/Game/BP/Common/BP_DoorBase.OpenForce` (`self.Phase_1Door`)))
    (:`2`
      (`/Game/BP/Common/BP_DoorBase.OpenForce` (`self.Phase_2Door`))))
  (`self.SetRandomThreeSetTrue` _returnvalue)
  (`self.SetNextPhase` _returnvalue _currentphase)
  (set `self.CurrentPhase` _returnvalue)
  (set `self.AngryNurseCount` 3))

(event `ReStart`
  (`C_DoubtsManager.EmptyArrayfuckyou` (subsystem `C_DoubtsManager`))
  (bind _returnvalue (`GameplayStatics.GetCurrentLevelName` true))
  (`GameplayStatics.OpenLevel` (`KismetStringLibrary.Conv_StringToName` _returnvalue)))

(event `self.LoseAllLife`
  (`KismetSystemLibrary.PrintString` "죽으셨어요 시벌"))

(fn `UserConstructionScript`)