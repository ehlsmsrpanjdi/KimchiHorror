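; A Day 5 hallucination resident: a modular character that exists only on that day and reacts once when the player enters its trigger box.
; BeginPlay destroys it on other days, otherwise sets a talking face pose and stores its start position.
; Depending on State, the overlap either destroys it immediately or plays a run animation while a timeline slides the mesh to the W component's location, then destroys it.
; Clothing and hair follow the body mesh through leader pose.
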(event `self.ReceiveBeginPlay`
  (bind _asbp_game_instance (cast `/Game/BP/BP_GameInstance` (`GameplayStatics.GetGameInstance`)))
  (if (== (`C_GameInstance.DayCount` _asbp_game_instance) 5)
    (bind _asbp_entity_face_anim (cast `/Game/BP/Stage1/InteractiveEntity/AnimIns/Face/BP_EntityFaceAnim` (`SkeletalMeshComponent.GetAnimInstance` (`self.Face`))))
    (`C_AnimBPBase.SetFacePose` _asbp_entity_face_anim "Talk" "Normal" 0.0)
    (set `self.StartPosition` (`self.K2_GetActorLocation`))
    (else
      (`self.K2_DestroyActor`))))

(event `Run`
  (`SkeletalMeshComponent.PlayAnimation` (`self.Mesh`) "/Game/BP/Stage1/FaceTest/MaleBodyAnim/AN_MaleRun.AN_MaleRun" true)
  (bind (_direction `_새_트랙_0`) (`Timeline|타임라인` :!via `PlayFromStart`)
    (:`Update`
      (`SceneComponent.K2_SetWorldLocation` (`self.Mesh`) (`KismetMathLibrary.VLerp` (`self.StartPosition`) (`SceneComponent.K2_GetComponentLocation` (`self.w`)) `_새_트랙_0`) false false))
    (:`Finished`
      (`self.K2_DestroyActor`))))

(event `Turn`)

(event `Destroy`
  (`self.K2_DestroyActor`))

(event `self.Box.OnComponentBeginOverlap`
  (params (OverlappedComponent :type "PrimitiveComponent Object Reference") (OtherActor :type "Actor Object Reference") (OtherComp :type "PrimitiveComponent Object Reference") (OtherBodyIndex :type Integer) (bFromSweep :type Boolean) (SweepResult :type "HitResult Structure (by ref)"))
  (if (not (`self.Is Worked`))
    (cast `/Game/Level/Stage_1Element/BP_MainPlayer` OtherActor)
    (set `self.Is Worked` true)
    (switch `int` (`self.State`)
      (:`0`
        (`self.Destroy` :!label _label))
      (:`1`
        (goto _label))
      (:`2`
        (`self.Run`)))))

(fn `UserConstructionScript`
  (`SkinnedMeshComponent.SetLeaderPoseComponent` (`self.Clothes`) (`self.Mesh`) false false)
  (`SkinnedMeshComponent.SetLeaderPoseComponent` (`self.Gloves`) (`self.Mesh`) false false)
  (`SkinnedMeshComponent.SetLeaderPoseComponent` (`self.Pants`) (`self.Mesh`) false false)
  (`SkinnedMeshComponent.SetLeaderPoseComponent` (`self.Glasses`) (`self.Mesh`) false false)
  (`SkinnedMeshComponent.SetLeaderPoseComponent` (`self.Headphones`) (`self.Mesh`) false false)
  (`SkinnedMeshComponent.SetLeaderPoseComponent` (`self.Hair_1`) (`self.Mesh`) false false))