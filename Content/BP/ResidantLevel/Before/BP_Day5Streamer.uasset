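; Day 5 event controller that activates nurses in staged waves, destroying itself on BeginPlay if the game instance's DayCount is not 5.
; It wakes the first nurse after a short delay, while externally called events wake the second and third, the latter with a body change.
; AllWake steps through nurses registered via InitNurse on a re-armed timer, turning each into a back nurse.
; The final move to level 5 is only a debug print.
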(event `self.ReceiveBeginPlay`
  (bind _asbp_game_instance (cast `/Game/BP/BP_GameInstance` (`GameplayStatics.GetGameInstance`)))
  (if (== (`C_GameInstance.DayCount` _asbp_game_instance) 5)
    (`KismetSystemLibrary.Delay` 1.0)
    (`/Game/BP/ResidantLevel/Before/BP_EncounterHNurse.ActivateMode` (`self.FirstNurse`))
    (else
      (`self.K2_DestroyActor`))))

(event `InitNurse`
  (params (NewParam :type "/Game/BP/ResidantLevel/Before/BP_EncounterHNurse Object Reference"))
  (`KismetArrayLibrary.Array_Add` (`self.Nurses`) NewParam))

(event `SecondWake`
  (`/Game/BP/ResidantLevel/Before/BP_EncounterHNurse.ActivateMode` (`self.SecondNurse`)))

(event `Third Wake`
  (bind _thirdnuerse (`self.ThirdNuerse`))
  (`/Game/BP/ResidantLevel/Before/BP_EncounterHNurse.ActivateMode` _thirdnuerse)
  (`/Game/BP/ResidantLevel/Before/BP_EncounterHNurse.SetBody` _thirdnuerse "NewEnumerator1"))

(event `AllWake`
  (bind _nurseindex (`self.NurseIndex`))
  (bind _output (`|GetArrayItem` (`self.Nurses`) _nurseindex))
  (if (> _nurseindex (- (`KismetArrayLibrary.Array_Length` (`self.Nurses`)) 1))
    (`KismetSystemLibrary.K2_ClearAndInvalidateTimerHandle` (`self.TimerHandle`))
    (`KismetSystemLibrary.Delay` 5.0)
    (`KismetSystemLibrary.PrintString` "5레벨로 이동")
    (else
      (`/Game/BP/ResidantLevel/Before/BP_EncounterHNurse.ActivateMode` _output)
      (`/Game/BP/ResidantLevel/Before/BP_EncounterHNurse.SetBackNurse` _output)
      (bind _result (`/Engine/EditorBlueprintResources/StandardMacros.IncrementInt` (`self.NurseIndex`))
        (:`  `
          (set `self.NurseIndex` _result)
          (bind _returnvalue (`KismetSystemLibrary.K2_SetTimerDelegate` (delegate `AllWake`) 1.0))
          (set `self.TimerHandle` _returnvalue))))))

(fn `UserConstructionScript`)