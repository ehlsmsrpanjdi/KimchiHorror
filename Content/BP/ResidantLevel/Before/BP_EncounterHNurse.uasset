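; Day 5 encounter nurse that holds medicine and turns manic when the player interacts with it, destroying itself on any other day.
; It starts hidden with ticks and collision off until ActivateMode, and nurse number 0 registers with MyStream.
; Interacting once with other nurses removes the medicine, switches face, body and look-at, causes dizziness and sets doubt.
; Each number triggers its own MyStream wake stage, the third also slowing the player.
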(event `self.ReceiveBeginPlay`
  (bind _asbp_game_instance (cast `/Game/BP/BP_GameInstance` (`GameplayStatics.GetGameInstance`)))
  (if (== (`C_GameInstance.DayCount` _asbp_game_instance) 5)
    (`parent.ReceiveBeginPlay`)
    (bind _asbp_main_player (cast `/Game/Level/Stage_1Element/BP_MainPlayer` (`GameplayStatics.GetPlayerPawn` 0)))
    (set `self.Player` _asbp_main_player)
    (`self.SetBody` "NewEnumerator2")
    (`/Game/BP/Stage1/InteractiveEntity/AnimIns/BPI_EntityMoveInter.ISetFaceMove` "Idle" "MadLaugh")
    (bind _asbp_entity_face_anim (cast `/Game/BP/Stage1/InteractiveEntity/AnimIns/Face/BP_EntityFaceAnim` (`SkeletalMeshComponent.GetAnimInstance` (`self.Face`))))
    (set `/Game/BP/Stage1/InteractiveEntity/AnimIns/Face/BP_EntityFaceAnim.IsTingle` false _asbp_entity_face_anim)
    (`/Game/BP/Stage1/InteractiveEntity/AnimIns/Face/BP_EntityFaceAnim.SetMoodIntensity` _asbp_entity_face_anim 0.9)
    (`self.Eye` "NewEnumerator1")
    (`SceneComponent.K2_AttachToComponent` (`self.Medicien`) (`self.Mesh`) "ItemSocket" "KeepRelative" "KeepRelative" "KeepRelative" true)
    (`self.SleepMode`)
    (if (== (`self.MyNumber`) 0)
      (`/Game/BP/ResidantLevel/Before/BP_Day5Streamer.InitNurse` (`self.MyStream`) self))
    (else
      (`self.K2_DestroyActor`))))

(event `ActivateMode`
  (`ActorComponent.SetComponentTickEnabled` (`self.Face`) true)
  (`ActorComponent.SetComponentTickEnabled` (`self.Mesh`) true)
  (`self.SetActorHiddenInGame` false)
  (`self.SetActorEnableCollision` true)
  (`self.SetActorTickEnabled` true))

(event `SleepMode`
  (`KismetSystemLibrary.K2_ClearAndInvalidateTimerHandle` (`self.TimeHandle`))
  (`ActorComponent.SetComponentTickEnabled` (`self.Face`) false)
  (`ActorComponent.SetComponentTickEnabled` (`self.Mesh`) false)
  (`self.SetActorHiddenInGame` true)
  (`self.SetActorEnableCollision` false)
  (`self.SetActorTickEnabled` false))

(event `self.ISetFaceMove`
  (params (Pose :type "C_FacePoseEnum Enum" :default "Idle") (Mood :type "C_FaceMoodEnum Enum" :default "Normal") (Interval :type "Float (double-precision)"))
  ;[1 1 1] 기본 ㅅ
  (bind _asbp_entity_face_anim (cast `/Game/BP/Stage1/InteractiveEntity/AnimIns/Face/BP_EntityFaceAnim` (`SkeletalMeshComponent.GetAnimInstance` (`self.Face`)))
    (:`then`
      (`C_AnimBPBase.SetFacePose` _asbp_entity_face_anim Pose Mood Interval))
    (:`CastFailed`
      (`KismetSystemLibrary.PrintString` "FaceMissing"))))

(event `self.ISetHeadTilting`
  (params (DesVector :type "Vector Structure") (RotateSpeed :type "Float (double-precision)"))
  ;[1 1 1] 기본 ㅅ
  (bind _asbp_hnurse_body_anim (cast `/Game/BP/ResidantLevel/BP_HNurseBodyAnim` (`SkeletalMeshComponent.GetAnimInstance` (`self.Mesh`)))
    (:`then`
      (`C_EntityAnimBase.LerfTiltHead` _asbp_hnurse_body_anim DesVector RotateSpeed))
    (:`CastFailed`
      (`KismetSystemLibrary.PrintString` "TiltingMissing"))))

(event `Eye`
  (params (`On/Off` :type "/Game/BP/Stage1/InteractiveEntity/AnimIns/Body/BP_LookAtEnum Enum" :default "NewEnumerator0"))
  ;[1 1 1] 눈 목 돌리기
  (bind _asabp_face_post_process (cast `/Game/MetaHumans/Common/Face/ABP_Face_PostProcess` (`SkeletalMeshComponent.GetPostProcessInstance` (`self.Face`))))
  (`/Game/MetaHumans/Common/Face/ABP_Face_PostProcess.EyeMoveOnOff` _asabp_face_post_process `On/Off`))

(event `self.ISetBodyMove`
  (params (Move :type "C_EntityMoveEnum Enum" :default "Idle"))
  ;[1 1 1] 기본 ㅅ
)

(event `Look`
  (params (`On/Off` :type "/Game/BP/Stage1/InteractiveEntity/AnimIns/Body/BP_LookAtEnum Enum" :default "NewEnumerator0"))
  ;[1 1 1] 눈 목 돌리기
  (bind _asbp_hnurse_body_anim (cast `/Game/BP/ResidantLevel/BP_HNurseBodyAnim` (`SkeletalMeshComponent.GetAnimInstance` (`self.Mesh`))))
  (`/Game/BP/ResidantLevel/BP_HNurseBodyAnim.LookAtSwitch` _asbp_hnurse_body_anim `On/Off`))

(event `SetBody`
  (params (Enum :type "/Game/BP/ResidantLevel/BP_HNurseBodyEnum Enum" :default "NewEnumerator0"))
  ;[1 1 1] 기본 ㅅ
  (bind _asbp_hnurse_body_anim (cast `/Game/BP/ResidantLevel/BP_HNurseBodyAnim` (`SkeletalMeshComponent.GetAnimInstance` (`self.Mesh`))))
  (set `/Game/BP/ResidantLevel/BP_HNurseBodyAnim.Enum` Enum _asbp_hnurse_body_anim))

(event `self.OnInteract`
  (params (Interactor :type "Actor Object Reference"))
  (bind _mystream (`self.MyStream`))
  ;[1 1 1] 상호작용
  (if (== (`self.MyNumber`) 0)
    _
    (elif (not (`self.IsInteracted`))
      (`ActorComponent.K2_DestroyComponent` (`self.Medicien`))
      (set `self.IsInteracted` true)
      (`/Game/BP/Stage1/InteractiveEntity/AnimIns/BPI_EntityMoveInter.ISetHeadTilting` (1800.0 1800.0 1800.0) 4.0)
      (`/Game/BP/Stage1/InteractiveEntity/AnimIns/BPI_EntityMoveInter.ISetFaceMove` "MadLaugh" "MadLaugh")
      (`self.SetBody` "NewEnumerator4")
      (`self.Eye` "NewEnumerator0")
      (`self.Look` "NewEnumerator1")
      (for _index (range 1 3)
        (`PrimitiveComponent.SetMaterial` (`self.Face`) _index "/Game/ArtWorkOnGit/Object/MT_Hanger.MT_Hanger")
        (`/Game/Level/Stage_1Element/BP_MainPlayer.OnDizziness` (`self.Player`))
        (set `self.InteractionMassage` "")
        (`C_DoubtsManager.SetDoubt` (subsystem `C_DoubtsManager`) (+ 30 0))
        (switch `int` (`self.MyNumber`)
          (:`1`
            (`/Game/BP/ResidantLevel/Before/BP_Day5Streamer.SecondWake` _mystream))
          (:`2`
            (`/Game/BP/ResidantLevel/Before/BP_Day5Streamer.Third Wake` _mystream))
          (:`3`
            (set `CharacterMovementComponent.MaxWalkSpeed` 50.0 (`Character.CharacterMovement` (`self.Player`)))
            (`/Game/BP/ResidantLevel/Before/BP_Day5Streamer.AllWake` _mystream)))))))

(event `SetBackNurse`
  (`/Game/BP/Stage1/InteractiveEntity/AnimIns/BPI_EntityMoveInter.ISetFaceMove` "MadLaugh" "MadLaugh")
  (`self.SetBody` "NewEnumerator4")
  (`self.Eye` "NewEnumerator0")
  (`self.Look` "NewEnumerator1")
  (for _index (range 1 3)
    (`PrimitiveComponent.SetMaterial` (`self.Face`) _index "/Game/ArtWorkOnGit/Object/MT_Hanger.MT_Hanger")))

(fn `CloseEye`
  (`self.ISetHeadTilting` (-1800.0 -1800.0 -1800.0) 3.0)
  (`/Game/BP/Stage1/InteractiveEntity/AnimIns/BPI_EntityMoveInter.ISetFaceMove` "CloseEye"))

(fn `OpenEye`
  (`self.ISetHeadTilting` (1800.0 1800.0 1800.0) 3.0)
  (`/Game/BP/Stage1/InteractiveEntity/AnimIns/BPI_EntityMoveInter.ISetFaceMove` "Idle" "MadLaugh"))

(fn `UserConstructionScript`
  (`SkinnedMeshComponent.SetLeaderPoseComponent` (`self.Clothes`) (`self.Mesh`) false false)
  (`SkinnedMeshComponent.SetLeaderPoseComponent` (`self.Gloves`) (`self.Mesh`) false false)
  (`SkinnedMeshComponent.SetLeaderPoseComponent` (`self.Arms`) (`self.Mesh`) false false)
  (`SkinnedMeshComponent.SetLeaderPoseComponent` (`self.Pants`) (`self.Mesh`) false false))