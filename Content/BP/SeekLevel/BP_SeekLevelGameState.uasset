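; BP_SeekLevelGameState is the seek level's game state and handles recoloring of the level's top floor pieces.
; On BeginPlay it caches every BP_TopFloor actor in the level.
; The SetFloorColor event loops over that cached list and sets each floor's material.
; A running counter in the loop feeds a threshold branch that triggers a short Delay and resets the count.
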(event `self.ReceiveBeginPlay`
  (bind _outactors (`GameplayStatics.GetAllActorsOfClass` "/Game/BP/BP_TopFloor.BP_TopFloor_C"))
  (set `self.Out Actors` _outactors))

(event `SetFloorColor`
  (bind _returnvalue (+ (`self.Count`) 1))
  (for _array_element (`self.Out Actors`)
    (`/Game/BP/BP_TopFloor.SetMaterial` _array_element)
    (set `self.Count` _returnvalue)
    (if (< _returnvalue 10)
      (`KismetSystemLibrary.Delay` 0.2)
      (set `self.Count` 0))))

(fn `UserConstructionScript`)