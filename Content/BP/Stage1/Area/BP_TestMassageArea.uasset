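; BP_TestMassageArea is a test trigger area in Stage1 that shows a message dialog while something overlaps its Box.
; Begin overlap fetches BP_Dialog through the UI manager, calls OnUI and shows MyMassage with a fixed duration, printing a debug string if the cast fails.
; End overlap also calls OnUI, then exits the dialog.
; Neither event filters the overlapping actor.
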(event `self.ReceiveBeginPlay`)

(event `self.Box.OnComponentBeginOverlap`
  (params (OverlappedComponent :type "PrimitiveComponent Object Reference") (OtherActor :type "Actor Object Reference") (OtherComp :type "PrimitiveComponent Object Reference") (OtherBodyIndex :type Integer) (bFromSweep :type Boolean) (SweepResult :type "HitResult Structure (by ref)"))
  (bind _returnvalue (`C_UIManager.GetUIManager`))
  (bind _returnvalue_2 (`C_UIManager.GetUI` _returnvalue "/Game/BP/Stage1/UI/BP_Dialog.BP_Dialog_C"))
  (`C_UIManager.OnUI` _returnvalue null)
  (bind _asbp_dialog (cast `/Game/BP/Stage1/UI/BP_Dialog` _returnvalue_2)
    (:`then`
      (`/Game/BP/Stage1/UI/BP_Dialog.ShowDialog` _asbp_dialog (`self.MyMassage`) 3.0))
    (:`CastFailed`
      (`KismetSystemLibrary.PrintString` "Hello"))))

(event `self.Box.OnComponentEndOverlap`
  (params (OverlappedComponent :type "PrimitiveComponent Object Reference") (OtherActor :type "Actor Object Reference") (OtherComp :type "PrimitiveComponent Object Reference") (OtherBodyIndex :type Integer))
  (bind _returnvalue (`C_UIManager.GetUIManager`))
  (bind _returnvalue_2 (`C_UIManager.GetUI` _returnvalue "/Game/BP/Stage1/UI/BP_Dialog.BP_Dialog_C"))
  (`C_UIManager.OnUI` _returnvalue null)
  (bind _asbp_dialog (cast `/Game/BP/Stage1/UI/BP_Dialog` _returnvalue_2))
  (`/Game/BP/Stage1/UI/BP_Dialog.ExitDialog` _asbp_dialog))

(fn `UserConstructionScript`)