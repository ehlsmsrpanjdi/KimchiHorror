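; BP_BlinkLight is a Stage 1 light actor that can be blinked on and off through a light function material.
; On BeginPlay it creates a dynamic instance of MI_BlinkLight, assigns it to its PointLight and unhides its Box in game.
; The OnBlink and OffBlink events switch the material's Intensity parameter between full and zero.
; The Box overlap casts to BP_LightEntity but does nothing further.
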(event `self.ReceiveBeginPlay`
  (bind _returnvalue (`KismetMaterialLibrary.CreateDynamicMaterialInstance` "/Game/CustomMT/MI_BlinkLight.MI_BlinkLight"))
  (bind _output_get (set `self.BlinkMT` _returnvalue))
  (`LightComponent.SetLightFunctionMaterial` (`self.PointLight`) _output_get)
  (`SceneComponent.SetHiddenInGame` (`self.Box`) false false))

(event `OnBlink`
  (`MaterialInstanceDynamic.SetScalarParameterValue` (`self.BlinkMT`) "Intensity" 1.0))

(event `OffBlink`
  (`MaterialInstanceDynamic.SetScalarParameterValue` (`self.BlinkMT`) "Intensity" 0.0))

(event `self.Box.OnComponentBeginOverlap`
  (params (OverlappedComponent :type "PrimitiveComponent Object Reference") (OtherActor :type "Actor Object Reference") (OtherComp :type "PrimitiveComponent Object Reference") (OtherBodyIndex :type Integer) (bFromSweep :type Boolean) (SweepResult :type "HitResult Structure (by ref)"))
  (cast `/Game/BP/Stage1/Entity/BP_LightEntity` OtherActor))

(fn `UserConstructionScript`)