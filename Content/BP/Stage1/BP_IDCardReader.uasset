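; BP_IDCardReader is an interactable ID card reader for Stage 1 that triggers the last level door.
; Interact focus applies an outline overlay material to its static mesh and losing focus clears it, both with a debug print.
; Interacting forwards OnInteract to the referenced BP_LastLevelDoor if valid, with no card check in this Blueprint.
; It always reports itself as a quest object and returns its QuestName as the current quest line.
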(event `InteractionInterface.CanInteract`
  (params (Interactor :type "Actor Object Reference"))
  (`MeshComponent.SetOverlayMaterial` (`self.StaticMesh`) "/Game/BP/Material/MT_FocusActorOutLine.MT_FocusActorOutLine")
  (`KismetSystemLibrary.PrintString` "Hello"))

(event `InteractionInterface.CanNotInteract`
  (params (Interactor :type "Actor Object Reference"))
  (`MeshComponent.SetOverlayMaterial` (`self.StaticMesh`) null)
  (`KismetSystemLibrary.PrintString` "Hello"))

(event `InteractionInterface.OnInteract`
  (params (Interactor :type "Actor Object Reference"))
  (bind _as_bp_last_level_door (`self.As BP Last Level Door`))
  (if (`KismetSystemLibrary.IsValid` _as_bp_last_level_door)
    (`InteractionInterface.OnInteract` _as_bp_last_level_door null)))

(fn `GetCurrentQuestLineName`
  (params (Interactor :type "Actor Object Reference"))
  (returns (ReturnValue :type Name))
  (return (`self.QuestName`)))

(fn `IsQuestObject`
  (params (Interactor :type "Actor Object Reference"))
  (returns (ReturnValue :type Boolean))
  (return true))

(fn `UserConstructionScript`)