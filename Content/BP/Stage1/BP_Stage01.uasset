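; BP_Stage01 is a Stage 1 Blueprint that opens the stash UI at start and runs the stage's game clock.
; BeginPlay casts the game instance and adds BP_StashUI through the UI manager.
; Tick uses a Delay to throttle Minute steps, with Hour advancing every twelfth; both wrap at 360, consistent with clock-hand degrees.
; GetTime exposes both values; dialog and viewport calls are left unconnected.
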(event `self.ReceiveBeginPlay`
  (bind _asbp_game_instance (cast `/Game/BP/BP_GameInstance` (`GameplayStatics.GetGameInstance`)))
  (`C_UIManager.CreateAndAddUI` (`C_UIManager.GetUIManager`) "/Game/BP/UI/Common/Stash/BP_StashUI.BP_StashUI_C"))

(event `self.ReceiveTick`
  (params (DeltaSeconds :type "Float (single-precision)"))
  (bind _minute (`self.minute`))
  (`KismetSystemLibrary.Delay` 0.18)
  (if (>= _minute 360)
    (set `self.minute` 0)
    (else
      (bind _output_get (set `self.minute` (+ _minute 1)))
      (if (== (mod _output_get 12) 0)
        (set `self.hour` (+ (`self.hour`) 1))
        (if (>= (`self.hour`) 360)
          (set `self.hour` 0))))))

(fn `Get Time`
  (returns (Hour :type Integer) (Minute :type Integer))
  (return (`self.hour`) (`self.minute`)))

(fn `UserConstructionScript`)