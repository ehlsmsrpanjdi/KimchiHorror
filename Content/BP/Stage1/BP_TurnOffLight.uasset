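; BP_TurnOffLight is a one-shot Stage 1 trigger that briefly blacks out top-floor lights on a specific day.
; On BeginPlay it destroys itself unless the game instance's DayCount matches its own.
; When BP_MainPlayer overlaps its Box, it calls OffLight on the referenced top-floor array, then OnLight after a short Delay.
; The Delay sits inside the first loop, and DestroyActor runs inside the restore loop.
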(event `self.ReceiveBeginPlay`
  (bind _asbp_game_instance (cast `/Game/BP/BP_GameInstance` (`GameplayStatics.GetGameInstance`)))
  (if (not (== (`C_GameInstance.DayCount` _asbp_game_instance) (`self.DayCount`)))
    (`self.K2_DestroyActor`)))

(event `self.Box.OnComponentBeginOverlap`
  (params (OverlappedComponent :type "PrimitiveComponent Object Reference") (OtherActor :type "Actor Object Reference") (OtherComp :type "PrimitiveComponent Object Reference") (OtherBodyIndex :type Integer) (bFromSweep :type Boolean) (SweepResult :type "HitResult Structure (by ref)"))
  (cast `/Game/Level/Stage_1Element/BP_MainPlayer` OtherActor)
  (for _array_element (`self.As BP Top Floor`)
    (`/Game/BP/BP_TopFloor.OffLight` _array_element)
    (`KismetSystemLibrary.Delay` 2.0)
    (for _array_element_2 (`self.As BP Top Floor`)
      (`/Game/BP/BP_TopFloor.OnLight` _array_element_2)
      (`self.K2_DestroyActor`))))

(fn `UserConstructionScript`)