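; BP_HideChild is a Stage 1 entity that seeks out the player and opens doors in its way.
; Five seconds after BeginPlay, a delay-throttled Tick line-traces to the player and, on a hit, sets Find and moves toward them.
; On arrival it traces again but only prints a debug result.
; Its DoorCollision overlap calls EntityOpen on any BP_Door.
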(event `self.ReceiveBeginPlay`
  (`KismetSystemLibrary.Delay` 5.0)
  (set `self.MoveStart` true))

(event `self.ReceiveTick`
  (params (DeltaSeconds :type "Float (single-precision)"))
  (bind _player (`self.Player`))
  (bind _player_2 (`self.Player`))
  (if (`self.MoveStart`)
    (`KismetSystemLibrary.Delay` 2.0)
    (bind _returnvalue (`C_KimchiHelper.LineTraceActorToActor` self _player))
    (if (== _player (`.HitActor` (`GameplayStatics.BreakHitResult` _returnvalue)))
      (set `self.Find` true)
      (bind _returnvalue_2 (`C_KimchiHelper.MoveToActorAndCheckArrival` self (`self.Player`) 100.0 true))
      (if _returnvalue_2
        (bind _returnvalue_3 (`C_KimchiHelper.LineTraceActorToActor` self _player_2))
        (if (== (`.HitActor` (`GameplayStatics.BreakHitResult` _returnvalue_3)) _player_2)
          (`KismetSystemLibrary.PrintString` "맞음")
          (else
            (`KismetSystemLibrary.PrintString` "안맞음")))))))

(event `self.doorCollision.OnComponentBeginOverlap`
  (params (OverlappedComponent :type "PrimitiveComponent Object Reference") (OtherActor :type "Actor Object Reference") (OtherComp :type "PrimitiveComponent Object Reference") (OtherBodyIndex :type Integer) (bFromSweep :type Boolean) (SweepResult :type "HitResult Structure (by ref)"))
  (bind _asbp_door (cast `/Game/BP/Common/BP_Door` OtherActor))
  (`/Game/BP/Common/BP_DoorBase.EntityOpen` _asbp_door self))

(fn `UserConstructionScript`)