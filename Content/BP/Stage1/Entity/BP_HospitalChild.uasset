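; BP_HospitalChild is a Stage 1 hospital child entity that, five seconds after spawning, chases the player with AIMoveTo reissued in a loop.
; A looping timer runs debug-drawn line traces toward the player's target position until one hits, setting TargetFound.
; Sphere overlaps only print detection state, while DoorCollision has doors open for it.
; Tick tracks movement speed, and destruction clears the owning spawner's IsSpawn flag.
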(event `self.ReceiveBeginPlay`
  (bind _returnvalue (`GameplayStatics.GetPlayerCharacter` 0))
  (`SceneComponent.SetHiddenInGame` (`self.Sphere`) false false)
  (`KismetSystemLibrary.Delay` 5.0)
  (`self.LayPlayer`)
  (bind _asbp_main_player (cast `/Game/Level/Stage_1Element/BP_MainPlayer` _returnvalue))
  (set `self.As BP Main Player` _asbp_main_player)
  (`|AIMoveTo` self (0.0 0.0 0.0) _returnvalue :!label _label
    (:`then`
      _)
    (:`OnSuccess`
      _)
    (:`OnFail`
      _))
  (`KismetSystemLibrary.Delay` 0.2)
  (goto _label))

(event `self.ReceiveTick`
  (params (DeltaSeconds :type "Float (single-precision)"))
  (set `self.Speed` (`KismetMathLibrary.VSize` (`MovementComponent.Velocity` (`self.CharacterMovement`)))))

(event `LayPlayer`
  (bind _returnvalue (`KismetSystemLibrary.K2_SetTimerDelegate` (delegate `FindPlayer`) 0.5 true)))

(event `self.ReceiveDestroyed`
  (bind _ownerspawner (`self.OwnerSpawner`))
  (if (`KismetSystemLibrary.IsValid` _ownerspawner)
    (set `/Game/BP/Stage1/Entity/Obj/BP_HospitalChildSpawner.IsSpawn` false _ownerspawner)))

(event `FindPlayer`
  (bind _returnvalue (`self.K2_GetActorLocation`))
  (bind _returnvalue_2 (`HorrorProtoKimchiCharacter.GetTargetPos` (`self.As BP Main Player`)))
  (bind _outhit (`KismetSystemLibrary.LineTraceSingleForObjects` :`Start` _returnvalue :`End` (* (- _returnvalue_2 _returnvalue) 1000.0) :`ObjectTypes` (`self.Object Types`) :`DrawDebugType` "ForDuration"))
  (bind _asbp_main_player (cast `/Game/Level/Stage_1Element/BP_MainPlayer` (`.HitActor` (`GameplayStatics.BreakHitResult` _outhit))))
  (set `self.TargetFound` true)
  (`KismetSystemLibrary.PrintString` "차즘")
  (`KismetSystemLibrary.K2_ClearAndInvalidateTimerHandle` (stale `LayPlayer` _returnvalue)))

(event `self.Sphere.OnComponentBeginOverlap`
  (params (OverlappedComponent :type "PrimitiveComponent Object Reference") (OtherActor :type "Actor Object Reference") (OtherComp :type "PrimitiveComponent Object Reference") (OtherBodyIndex :type Integer) (bFromSweep :type Boolean) (SweepResult :type "HitResult Structure (by ref)"))
  (`KismetSystemLibrary.PrintString` (`KismetSystemLibrary.GetDisplayName` OtherActor))
  (cast `/Game/Level/Stage_1Element/BP_MainPlayer` OtherActor)
  (if (`self.TargetFound`)
    (`KismetSystemLibrary.PrintString` "찾았고 닿았움")
    (else
      (`KismetSystemLibrary.PrintString` "못찾았지만 닿았음"))))

(event `self.doorCollision.OnComponentBeginOverlap`
  (params (OverlappedComponent :type "PrimitiveComponent Object Reference") (OtherActor :type "Actor Object Reference") (OtherComp :type "PrimitiveComponent Object Reference") (OtherBodyIndex :type Integer) (bFromSweep :type Boolean) (SweepResult :type "HitResult Structure (by ref)"))
  (bind _asbp_door (cast `/Game/BP/Common/BP_Door` OtherActor))
  (`/Game/BP/Common/BP_DoorBase.EntityOpen` _asbp_door self))

(fn `UserConstructionScript`)