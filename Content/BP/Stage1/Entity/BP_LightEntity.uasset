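; BP_LightEntity is a Stage 1 entity that makes top-floor pieces blink around it and reacts to player detection.
; Its LightBox calls OnBlink on any BP_TopFloor it begins overlapping and OffBlink when that overlap ends.
; Separate DetectBox and LoseBox volumes forward begin and end overlaps, unfiltered here, to OnPlayerDetect and OnPlayerLose, whose logic lives outside these graphs.
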(event `self.ReceiveBeginPlay`)

(event `self.LightBox.OnComponentBeginOverlap`
  (params (OverlappedComponent :type "PrimitiveComponent Object Reference") (OtherActor :type "Actor Object Reference") (OtherComp :type "PrimitiveComponent Object Reference") (OtherBodyIndex :type Integer) (bFromSweep :type Boolean) (SweepResult :type "HitResult Structure (by ref)"))
  (bind _asbp_top_floor (cast `/Game/BP/BP_TopFloor` OtherActor))
  (`/Game/BP/BP_TopFloor.OnBlink` _asbp_top_floor))

(event `self.LightBox.OnComponentEndOverlap`
  (params (OverlappedComponent :type "PrimitiveComponent Object Reference") (OtherActor :type "Actor Object Reference") (OtherComp :type "PrimitiveComponent Object Reference") (OtherBodyIndex :type Integer))
  (bind _asbp_top_floor (cast `/Game/BP/BP_TopFloor` OtherActor))
  (`/Game/BP/BP_TopFloor.OffBlink` _asbp_top_floor))

(event `self.DetectBox.OnComponentBeginOverlap`
  (params (OverlappedComponent :type "PrimitiveComponent Object Reference") (OtherActor :type "Actor Object Reference") (OtherComp :type "PrimitiveComponent Object Reference") (OtherBodyIndex :type Integer) (bFromSweep :type Boolean) (SweepResult :type "HitResult Structure (by ref)"))
  (`self.OnPlayerDetect` OverlappedComponent OtherActor OtherComp OtherBodyIndex bFromSweep SweepResult))

(event `self.LoseBox.OnComponentEndOverlap`
  (params (OverlappedComponent :type "PrimitiveComponent Object Reference") (OtherActor :type "Actor Object Reference") (OtherComp :type "PrimitiveComponent Object Reference") (OtherBodyIndex :type Integer))
  (`self.OnPlayerLose` OverlappedComponent OtherActor OtherComp OtherBodyIndex))

(fn `UserConstructionScript`)