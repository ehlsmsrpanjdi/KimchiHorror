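; BP_DoubtCol is a Stage1 trigger box, shown in game, that raises the player's doubt gauge once overlapped.
; Box overlap events set IsOverlap, and Tick then adds doubt to the cached BP_MainPlayer at a frame-rate-independent rate.
; End overlap also sets IsOverlap true, so the gain never stops.
; Any actor triggers it, as the player comparison is only debug-printed, alongside the gauge value.
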(event `self.ReceiveBeginPlay`
  (bind _asbp_main_player (cast `/Game/Level/Stage_1Element/BP_MainPlayer` (`GameplayStatics.GetPlayerPawn` 0)))
  (set `self.As BP Main Player` _asbp_main_player)
  (`SceneComponent.SetHiddenInGame` (`self.Box`) false false))

(event `self.ReceiveTick`
  (params (DeltaSeconds :type "Float (single-precision)"))
  (bind _as_bp_main_player (`self.As BP Main Player`))
  (if (`self.bIsOverlap`)
    (`HorrorProtoKimchiCharacter.AddDoubt` _as_bp_main_player (* DeltaSeconds 50.0))
    (`KismetSystemLibrary.PrintString` (`KismetStringLibrary.Conv_DoubleToString` (`HorrorProtoKimchiCharacter.CurrentDoubtGauge` _as_bp_main_player)))))

(event `self.Box.OnComponentBeginOverlap`
  (params (OverlappedComponent :type "PrimitiveComponent Object Reference") (OtherActor :type "Actor Object Reference") (OtherComp :type "PrimitiveComponent Object Reference") (OtherBodyIndex :type Integer) (bFromSweep :type Boolean) (SweepResult :type "HitResult Structure (by ref)"))
  (`KismetSystemLibrary.PrintString` (`KismetStringLibrary.Conv_BoolToString` (== OtherActor (`self.As BP Main Player`))))
  (set `self.bIsOverlap` true))

(event `self.Box.OnComponentEndOverlap`
  (params (OverlappedComponent :type "PrimitiveComponent Object Reference") (OtherActor :type "Actor Object Reference") (OtherComp :type "PrimitiveComponent Object Reference") (OtherBodyIndex :type Integer))
  (`KismetSystemLibrary.PrintString` (`KismetStringLibrary.Conv_BoolToString` (== OtherActor (`self.As BP Main Player`))))
  (set `self.bIsOverlap` true))

(fn `UserConstructionScript`)