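; BP_EntitySpline is a Stage 1 actor that spawns a light entity on a spline once evening arrives.
; On BeginPlay it binds to the HorrorProtoKimchi game mode's hour-changed event.
; When the new hour is 18 or later, it spawns a BP_LightEntity at its Arrow's location, passes it its Spline, then unbinds so the spawn happens only once.
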(event `self.ReceiveBeginPlay`
  (bind _ashorror_proto_kimchi_game_mode (cast `HorrorProtoKimchiGameMode` (`GameplayStatics.GetGameMode`)))
  (add `HorrorProtoKimchiGameMode.OnHourChanged` _ashorror_proto_kimchi_game_mode (delegate `SpawnEntity`)))

(event `SpawnEntity`
  (params (NewHour :type Integer))
  (if (>= NewHour 18)
    (bind _returnvalue (`|SpawnActorFromClass` "/Game/BP/Stage1/Entity/BP_LightEntity.BP_LightEntity_C" (`KismetMathLibrary.MakeTransform` (`SceneComponent.K2_GetComponentLocation` (`self.Arrow`))) "Undefined" "MultiplyWithRoot" null null))
    (set `C_BlinkEntity.Spline` (`self.Spline`) _returnvalue)
    (remove `HorrorProtoKimchiGameMode.OnHourChanged` (stale `self.ReceiveBeginPlay` _ashorror_proto_kimchi_game_mode) (delegate `SpawnEntity`))))

(fn `UserConstructionScript`)