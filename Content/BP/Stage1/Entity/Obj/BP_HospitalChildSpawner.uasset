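; Stage 1 trigger-box spawner that randomly spawns a BP_HospitalChild near the player after an audio cue.
; While the player overlaps the box, a looping timer gives roughly even odds of starting the audio and setting IsSpawn.
; When the audio finishes, a loop tests random navmesh points for height and distance, but the spawn re-rolls its location.
; The child receives this spawner as OwnerSpawner.
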(event `self.ReceiveBeginPlay`
  (`SceneComponent.SetHiddenInGame` (`self.Box`) false false))

(event `self.ReceiveTick`
  (params (DeltaSeconds :type "Float (single-precision)")))

(event `SpawnEntity`
  (bind _audiocomp (`self.AudioComp`))
  (if (and (`self.IsOverlap`) (not (`self.IsSpawn`)))
    (if (> (`KismetMathLibrary.RandomFloat`) 0.5)
      (`KismetSystemLibrary.PrintString` "스폰함")
      (set `self.IsSpawn` true)
      (`AudioComponent.Play` _audiocomp 0.0)
      (add `AudioComponent.OnAudioFinished` _audiocomp (delegate `MusicEnd`))
      (else
        (`KismetSystemLibrary.PrintString` "스폰못함")))))

(event `self.Box.OnComponentBeginOverlap`
  (params (OverlappedComponent :type "PrimitiveComponent Object Reference") (OtherActor :type "Actor Object Reference") (OtherComp :type "PrimitiveComponent Object Reference") (OtherBodyIndex :type Integer) (bFromSweep :type Boolean) (SweepResult :type "HitResult Structure (by ref)"))
  (if (not (`self.IsOverlap`))
    (cast `/Game/Level/Stage_1Element/BP_MainPlayer` OtherActor)
    (set `self.IsOverlap` true)
    (bind _returnvalue (`KismetSystemLibrary.K2_SetTimerDelegate` (delegate `SpawnEntity`) 1.0 true))))

(event `self.Box.OnComponentEndOverlap`
  (params (OverlappedComponent :type "PrimitiveComponent Object Reference") (OtherActor :type "Actor Object Reference") (OtherComp :type "PrimitiveComponent Object Reference") (OtherBodyIndex :type Integer))
  (if (`self.IsOverlap`)
    (cast `/Game/Level/Stage_1Element/BP_MainPlayer` OtherActor)
    (set `self.IsOverlap` false)
    (`KismetSystemLibrary.K2_ClearAndInvalidateTimerHandle` (stale `self.Box.OnComponentBeginOverlap` _returnvalue))))

(event `MusicEnd`
  (bind _returnvalue (`self.K2_GetActorLocation` (`GameplayStatics.GetPlayerPawn` 0)))
  (bind _randomlocation (`NavigationSystemV1.K2_GetRandomReachablePointInRadius` _returnvalue 1000.0 null null))
  (`KismetSystemLibrary.PrintString` "노래끝남 스폰")
  (for _ (range 101)
    (`KismetSystemLibrary.Delay` 0.2)
    (if (and (< (`KismetMathLibrary.Abs` (- (.z _randomlocation) (.z _returnvalue))) 300.0) (> (`KismetMathLibrary.Vector_Distance` _randomlocation _returnvalue) 1000.0))
      (break)))
  (bind _returnvalue_2 (`|SpawnActorFromClass` "/Game/BP/Stage1/Entity/BP_HospitalChild.BP_HospitalChild_C" (`KismetMathLibrary.MakeTransform` _randomlocation) "Undefined" "MultiplyWithRoot" null null))
  (if (`KismetSystemLibrary.IsValid` _returnvalue_2)
    (set `/Game/BP/Stage1/Entity/BP_HospitalChild.OwnerSpawner` self _returnvalue_2)
    (else
      (`KismetSystemLibrary.PrintString` "Hello"))))

(fn `UserConstructionScript`)