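; Nurse character for the Stage 1 lying-down patient scene, playing a scripted walk between patient and doctor.
; BeginPlay caches both actors from BP_GameState and the start location; Tick gates a SequenceIndex switch through WaitFunction, calling Chase toward patient, doctor, then patient.
; The doctor step triggers MoveToPatient; the last casts PatientActor, not DocActor, to BP_PatientDoc before MoveToOrigin and the nurse's return.
; Construction binds modular outfit meshes to the main mesh's pose.
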(event `self.ReceiveBeginPlay`
  (bind _asbp_game_state (cast `/Game/ThirdPerson/Blueprints/BP_GameState` (`GameplayStatics.GetGameState`)))
  (set `self.PatientActor` (`/Game/ThirdPerson/Blueprints/BP_GameState.PatientActor` _asbp_game_state))
  (set `self.DocActor` (`/Game/ThirdPerson/Blueprints/BP_GameState.DocActor` _asbp_game_state))
  (set `self.OriginPos` (`self.K2_GetActorLocation`)))

(event `self.ReceiveTick`
  (params (DeltaSeconds :type "Float (single-precision)"))
  (bind _sequenceindex (`self.sequenceIndex`))
  (bind _patientactor (`self.PatientActor`))
  (bind _docactor (`self.DocActor`))
  (`KismetSystemLibrary.PrintString` (`KismetStringLibrary.Conv_DoubleToString` (`KismetMathLibrary.Conv_IntToDouble` _sequenceindex)))
  (bind _returnvalue (`self.WaitFunction` DeltaSeconds))
  (if _returnvalue
    (switch `int` _sequenceindex
      (:`0`
        (bind _returnvalue_2 (`self.Chase` (`self.PatientActor`) 5.0 200.0 5.0))
        (if _returnvalue_2
          _))
      (:`1`
        (bind _returnvalue_3 (`self.Chase` _docactor 5.0 200.0 5.0))
        (if _returnvalue_3
          (bind _asbp_patient_doc (cast `/Game/BP/Stage1/InteractiveEntity/LyingDownPatient/BP_PatientDoc` _docactor))
          (`/Game/BP/Stage1/InteractiveEntity/LyingDownPatient/BP_PatientDoc.MoveToPatient` _asbp_patient_doc 5.0)))
      (:`2`
        (bind _returnvalue_4 (`self.Chase` _patientactor 5.0 200.0 5.0))
        (if _returnvalue_4
          (bind _asbp_patient_doc_2 (cast `/Game/BP/Stage1/InteractiveEntity/LyingDownPatient/BP_PatientDoc` _patientactor))
          (`/Game/BP/Stage1/InteractiveEntity/LyingDownPatient/BP_PatientDoc.MoveToOrigin` _asbp_patient_doc_2 10.0)
          (`|AIMoveTo` self (`self.OriginPos`) null))))))

(fn `UserConstructionScript`
  (`SkinnedMeshComponent.SetLeaderPoseComponent` (`self.Clothes`) (`self.Mesh`) false false)
  (`SkinnedMeshComponent.SetLeaderPoseComponent` (`self.Backpack`) (`self.Mesh`) false false)
  (`SkinnedMeshComponent.SetLeaderPoseComponent` (`self.Armor`) (`self.Mesh`) false false)
  (`SkinnedMeshComponent.SetLeaderPoseComponent` (`self.Gloves`) (`self.Mesh`) false false)
  (`SkinnedMeshComponent.SetLeaderPoseComponent` (`self.Arm_Module_Right`) (`self.Mesh`) false false)
  (`SkinnedMeshComponent.SetLeaderPoseComponent` (`self.Patch_L_Arm`) (`self.Mesh`) false false)
  (`SkinnedMeshComponent.SetLeaderPoseComponent` (`self.Hip_Right`) (`self.Mesh`) false false)
  (`SkinnedMeshComponent.SetLeaderPoseComponent` (`self.Gasmask`) (`self.Mesh`) false false)
  (`SkinnedMeshComponent.SetLeaderPoseComponent` (`self.Balaclava`) (`self.Mesh`) false false)
  (`SkinnedMeshComponent.SetLeaderPoseComponent` (`self.Hat`) (`self.Mesh`) false false)
  (`SkinnedMeshComponent.SetLeaderPoseComponent` (`self.Hip_Left`) (`self.Mesh`) false false)
  (`SkinnedMeshComponent.SetLeaderPoseComponent` (`self.Patch_Cap`) (`self.Mesh`) false false)
  (`SkinnedMeshComponent.SetLeaderPoseComponent` (`self.Helmet_Drops`) (`self.Mesh`) false false)
  (`SkinnedMeshComponent.SetLeaderPoseComponent` (`self.Scarf`) (`self.Mesh`) false false)
  (`SkinnedMeshComponent.SetLeaderPoseComponent` (`self.Patch_Helmetn`) (`self.Mesh`) false false)
  (`SkinnedMeshComponent.SetLeaderPoseComponent` (`self.Bulletproof`) (`self.Mesh`) false false)
  (`SkinnedMeshComponent.SetLeaderPoseComponent` (`self.Arms`) (`self.Mesh`) false false)
  (`SkinnedMeshComponent.SetLeaderPoseComponent` (`self.Preset`) (`self.Mesh`) false false)
  (`SkinnedMeshComponent.SetLeaderPoseComponent` (`self.Bulletproof_Drops`) (`self.Mesh`) false false)
  (`SkinnedMeshComponent.SetLeaderPoseComponent` (`self.Helmet_Headphones`) (`self.Mesh`) false false)
  (`SkinnedMeshComponent.SetLeaderPoseComponent` (`self.Helmet_Module`) (`self.Mesh`) false false)
  (`SkinnedMeshComponent.SetLeaderPoseComponent` (`self.Tactical_Belt`) (`self.Mesh`) false false)
  (`SkinnedMeshComponent.SetLeaderPoseComponent` (`self.Pants`) (`self.Mesh`) false false)
  (`SkinnedMeshComponent.SetLeaderPoseComponent` (`self.Helmet`) (`self.Mesh`) false false)
  (`SkinnedMeshComponent.SetLeaderPoseComponent` (`self.Glasses`) (`self.Mesh`) false false)
  (`SkinnedMeshComponent.SetLeaderPoseComponent` (`self.Headphones`) (`self.Mesh`) false false)
  (`SkinnedMeshComponent.SetLeaderPoseComponent` (`self.Patch_Back`) (`self.Mesh`) false false)
  (`SkinnedMeshComponent.SetLeaderPoseComponent` (`self.Patch_R_Arm`) (`self.Mesh`) false false)
  (`SkinnedMeshComponent.SetLeaderPoseComponent` (`self.Hair`) (`self.Mesh`) false false)
  (`SkinnedMeshComponent.SetLeaderPoseComponent` (`self.Watch`) (`self.Mesh`) false false))