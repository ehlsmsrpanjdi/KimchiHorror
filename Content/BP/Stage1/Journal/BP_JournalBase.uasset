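; BP_JournalBase is a base pickup actor for journal notes in Stage 1.
; On interact it fetches the stash UI from the UI manager, passes its text and rule flag via SetJournal, then destroys itself.
; Actor overlap begin and end toggle an outline overlay material on its cube mesh to highlight it.
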(event `self.ReceiveBeginPlay`)

(event `InteractionInterface.OnInteract`
  (params (Interactor :type "Actor Object Reference"))
  (bind _returnvalue (`C_UIManager.GetUI` (`C_UIManager.GetUIManager`) "/Game/BP/UI/Common/Stash/BP_StashUI.BP_StashUI_C"))
  (bind _asbp_stash_ui (cast `/Game/BP/UI/Common/Stash/BP_StashUI` _returnvalue))
  (`/Game/BP/UI/Common/Stash/BP_StashUI.SetJournal` _asbp_stash_ui (`self.MyText`) (`self.IsRule`))
  (`self.K2_DestroyActor`))

(event `self.ReceiveActorBeginOverlap`
  (params (OtherActor :type "Actor Object Reference"))
  (`MeshComponent.SetOverlayMaterial` (`self.Cube`) (`self.OutLine`)))

(event `self.ReceiveActorEndOverlap`
  (params (OtherActor :type "Actor Object Reference"))
  (`MeshComponent.SetOverlayMaterial` (`self.Cube`) null))

(fn `UserConstructionScript`)