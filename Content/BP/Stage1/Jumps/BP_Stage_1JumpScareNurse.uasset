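; Stage 1 jump-scare nurse, a modular character that starts in a MadStand pose and forces the player's view toward it.
; Overlapping its Box calls OnlyLook on the player, then removes the trigger.
; Tick also disarms the trigger when both forward vectors roughly oppose, calling CallPlayer, which only prints.
; Interface events relay face, body and head-tilt commands to anim Blueprints; outfit parts follow the body via leader pose.
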(event `self.ISetFaceMove`
  (params (Pose :type "C_FacePoseEnum Enum" :default "Idle") (Mood :type "C_FaceMoodEnum Enum" :default "Normal") (Interval :type "Float (double-precision)"))
  (bind _asbp_entity_face_anim (cast `/Game/BP/Stage1/InteractiveEntity/AnimIns/Face/BP_EntityFaceAnim` (`SkeletalMeshComponent.GetAnimInstance` (`self.Face`)))
    (:`then`
      (`C_AnimBPBase.SetFacePose` _asbp_entity_face_anim Pose Mood Interval))
    (:`CastFailed`
      (`KismetSystemLibrary.PrintString` "FaceMissing"))))

(event `self.ReceiveBeginPlay`
  (`parent.ReceiveBeginPlay`)
  (set `self.MyFace` (`self.Face`))
  (`SceneComponent.K2_AttachToComponent` (`self.Noise`) (`self.Mesh`) "headSocket" "KeepRelative" "KeepRelative" "KeepRelative" true)
  (`self.ISetBodyMove` "MadStand"))

(event `self.ISetHeadTilting`
  (params (DesVector :type "Vector Structure") (RotateSpeed :type "Float (double-precision)"))
  (bind _asbp_female_entity_body_anim (cast `/Game/BP/Stage1/InteractiveEntity/AnimIns/Body/BP_FemaleEntityBodyAnim` (`SkeletalMeshComponent.GetAnimInstance` (`self.Mesh`)))
    (:`then`
      (`C_EntityAnimBase.LerfTiltHead` _asbp_female_entity_body_anim DesVector RotateSpeed))
    (:`CastFailed`
      (`KismetSystemLibrary.PrintString` "TiltingMissing"))))

(event `self.ISetBodyMove`
  (params (Move :type "C_EntityMoveEnum Enum" :default "Idle"))
  (bind _asbp_female_entity_body_anim (cast `/Game/BP/Stage1/InteractiveEntity/AnimIns/Body/BP_FemaleEntityBodyAnim` (`SkeletalMeshComponent.GetAnimInstance` (`self.Mesh`)))
    (:`then`
      (`C_EntityAnimBase.SetBodyMove` _asbp_female_entity_body_anim Move))
    (:`CastFailed`
      (`KismetSystemLibrary.PrintString` "BodyMissing"))))

(event `self.ReceiveTick`
  (params (DeltaSeconds :type "Float (single-precision)"))
  (if (`self.Checking`)
    _
    (elif (< (`KismetMathLibrary.Dot_VectorVector` (`self.GetActorForwardVector`) (`self.GetActorForwardVector` (`GameplayStatics.GetPlayerPawn` 0))) -0.45)
      (`self.CallPlayer`)
      (set `self.Checking` true)
      (`ActorComponent.K2_DestroyComponent` (`self.Box`)))))

(event `CallPlayer`
  (`KismetSystemLibrary.PrintString` "손님"))

(event `self.Box.OnComponentBeginOverlap`
  (params (OverlappedComponent :type "PrimitiveComponent Object Reference") (OtherActor :type "Actor Object Reference") (OtherComp :type "PrimitiveComponent Object Reference") (OtherBodyIndex :type Integer) (bFromSweep :type Boolean) (SweepResult :type "HitResult Structure (by ref)"))
  (bind _asbp_main_player (cast `/Game/Level/Stage_1Element/BP_MainPlayer` OtherActor))
  (set `self.Checking` true)
  (`/Game/Level/Stage_1Element/BP_MainPlayer.OnlyLook` _asbp_main_player (+ (`self.K2_GetActorLocation`) (0.0 0.0 80.0)))
  (`ActorComponent.K2_DestroyComponent` (`self.Box`)))

(fn `UserConstructionScript`
  (`SkinnedMeshComponent.SetLeaderPoseComponent` (`self.Clothes`) (`self.Mesh`) false false)
  (`SkinnedMeshComponent.SetLeaderPoseComponent` (`self.Gloves`) (`self.Mesh`) false false)
  (`SkinnedMeshComponent.SetLeaderPoseComponent` (`self.Gasmask`) (`self.Mesh`) false false)
  (`SkinnedMeshComponent.SetLeaderPoseComponent` (`self.Hat`) (`self.Mesh`) false false)
  (`SkinnedMeshComponent.SetLeaderPoseComponent` (`self.Arms`) (`self.Mesh`) false false)
  (`SkinnedMeshComponent.SetLeaderPoseComponent` (`self.Pants`) (`self.Mesh`) false false)
  (`SkinnedMeshComponent.SetLeaderPoseComponent` (`self.Headphones`) (`self.Mesh`) false false))