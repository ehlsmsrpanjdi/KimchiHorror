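; BP_ItemBase is the base pickup item for Stage 1, outlined while another actor overlaps it.
; On BeginPlay it looks up its data by MyIndex in the GameInstance's ItemDatabase and applies that mesh and material.
; OnInteract passes the data and itself to BP_MenuUI, then hides the actor and disables collision instead of destroying it.
; Effect, DestroyThis and the quest queries are placeholder stubs.
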(event `self.ReceiveActorBeginOverlap`
  (params (OtherActor :type "Actor Object Reference"))
  (`MeshComponent.SetOverlayMaterial` (`self.Cube`) (`self.OutLine`)))

(event `self.ReceiveBeginPlay`
  (bind _cube (`self.Cube`))
  (bind _data (`self.SetItem` (`self.myIndex`)))
  (if (`KismetSystemLibrary.IsValid` _data)
    (bind _output_get (set `self.Data` _data))
    (bind _itemmesh (`C_ItemData.ItemMesh` _output_get))
    (`StaticMeshComponent.SetStaticMesh` _cube _itemmesh)
    (`PrimitiveComponent.SetMaterial` _cube 0 (`StaticMesh.GetMaterial` _itemmesh 0))
    (else
      (`KismetSystemLibrary.PrintString` (`KismetStringLibrary.Conv_IntToString` (`self.myIndex`))))))

(event `self.ReceiveActorEndOverlap`
  (params (OtherActor :type "Actor Object Reference"))
  (`MeshComponent.SetOverlayMaterial` (`self.Cube`) null))

(event `InteractionInterface.OnInteract`
  (params (Interactor :type "Actor Object Reference"))
  (cast `/Game/BP/GameMode/BP_MainStageGameMode` (`GameplayStatics.GetGameMode`)
    (:`then`
      (bind _returnvalue (`C_UIManager.GetUI` (`C_UIManager.GetUIManager`) "/Game/BP/UI/Common/Stash/BP_MenuUI.BP_MenuUI_C"))
      (bind _asbp_menu_ui (cast `/Game/BP/UI/Common/Stash/BP_MenuUI` _returnvalue)
        (:`then`
          (`/Game/BP/UI/Common/Stash/BP_MenuUI.GetItem` _asbp_menu_ui (`self.Data`) self)
          (`self.SetActorHiddenInGame` true)
          (`self.SetActorEnableCollision` false))
        (:`CastFailed`
          (`KismetSystemLibrary.PrintString` "Hello"))))
    (:`CastFailed`
      (`KismetSystemLibrary.PrintString` "Hello"))))

(event `/Game/BP/Stage1/Stage01Item/BI_ItemEffect.Effect`
  (`KismetSystemLibrary.PrintString` "각자구현하라"))

(event `Destroy`
  (`self.DestroyThis`))

(fn `DestroyThis`)

(fn `GetCurrentQuestLineName`
  (params (Interactor :type "Actor Object Reference"))
  (returns (ReturnValue :type Name))
  (return "None"))

(fn `IsQuestObject`
  (params (Interactor :type "Actor Object Reference"))
  (returns (ReturnValue :type Boolean))
  (return false))

(fn `SetItem`
  (params (Index :type Integer))
  (returns (Data :type "C_ItemData Object Reference"))
  (bind _asbp_game_instance (cast `/Game/BP/BP_GameInstance` (`GameplayStatics.GetGameInstance`)))
  (return (`C_ItemDatabase.FindItemByID` (`C_GameInstance.ItemDatabase` _asbp_game_instance) Index)))

(fn `UserConstructionScript`)