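; BP_Mask is an interactable Stage 1 mask item that is removed from the level when used.
; On BeginPlay it looks up its data by index in the GameInstance's ItemDatabase, printing the index if the lookup fails.
; Actor overlap toggles an overlay material on its cube mesh.
; OnInteract destroys the actor if the game mode is BP_Stage01, without passing the item data on.
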(event `self.ReceiveActorBeginOverlap`
  (params (OtherActor :type "Actor Object Reference"))
  (`MeshComponent.SetOverlayMaterial` (`self.Cube`) (`self.NewVar`)))

(event `self.ReceiveBeginPlay`
  (bind _data (`self.SetItem` (`self.myIndex`)))
  (if (`KismetSystemLibrary.IsValid` _data)
    (set `self.Data` _data)
    (else
      (`KismetSystemLibrary.PrintString` (`KismetStringLibrary.Conv_IntToString` (`self.myIndex`))))))

(event `self.ReceiveActorEndOverlap`
  (params (OtherActor :type "Actor Object Reference"))
  (`MeshComponent.SetOverlayMaterial` (`self.Cube`) null))

(event `self.OnInteract`
  (params (Interactor :type "Actor Object Reference"))
  (cast `/Game/BP/Stage1/BP_Stage01` (`GameplayStatics.GetGameMode`))
  (`self.K2_DestroyActor`))

(fn `SetItem`
  (params (Index :type Integer))
  (returns (Data :type "C_ItemData Object Reference"))
  (bind _asbp_game_instance (cast `/Game/BP/BP_GameInstance` (`GameplayStatics.GetGameInstance`)))
  (return (`C_ItemDatabase.FindItemByID` (`C_GameInstance.ItemDatabase` _asbp_game_instance) Index)))

(fn `UserConstructionScript`)