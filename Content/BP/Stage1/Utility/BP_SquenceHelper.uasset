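; BP_SquenceHelper is a Stage 1 utility that plays level sequences as cutscenes and returns control to the player afterward.
; StartSequence switches the view to a given camera, hides the player, ignores input, plays the sequence and binds a caller-supplied finish event.
; StopSequence halts the current sequence, and OnFinishedSequence restores input, visibility and a blended player view.
; DoubtInsesity is an empty stub with disconnected doubt-driven post-process logic.
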(event `self.ReceiveBeginPlay`
  (set `self.Player` (`GameplayStatics.GetPlayerCharacter` 0))
  (set `self.Controller` (`GameplayStatics.GetPlayerController` 0)))

(event `OnFirstSceneFinished`
  (`self.OnFinishedSequence` 0.0))

(fn `DoubtInsesity`
  (params (Doubt :type "Float (double-precision)") (post :type "PostProcessVolume Object Reference")))

(fn `OnFinishedSequence`
  (params (Blendtype :type "Float (double-precision)"))
  (bind _player (`self.Player`))
  (bind _controller (`self.Controller`))
  (`Controller.SetIgnoreMoveInput` _controller false)
  (`Controller.SetIgnoreLookInput` _controller false)
  (`self.SetActorHiddenInGame` _player false)
  (`self.SetActorHiddenInGame` _controller false)
  (`PlayerController.SetViewTargetWithBlend` _controller _player Blendtype "VTBlend_Linear" 0.0 false)
  (set `self.CurrentActor` null))

(fn `StartSequence`
  (params (Camera :type "CineCameraActor Object Reference") (SequenceActor :type "LevelSequenceActor Object Reference") (`이벤트` :type "Delegate (by ref)"))
  (bind _controller (`self.Controller`))
  (bind _output_get (set `self.CurrentActor` SequenceActor))
  (`PlayerController.SetViewTargetWithBlend` _controller Camera 0.0 "VTBlend_Linear" 0.0 false)
  (`self.SetActorHiddenInGame` (`self.Player`) true)
  (`Controller.SetIgnoreMoveInput` _controller true)
  (`Controller.SetIgnoreLookInput` _controller true)
  (bind _sequenceplayer (`LevelSequenceActor.SequencePlayer` _output_get))
  (`MovieSceneSequencePlayer.Play` _sequenceplayer)
  (add `MovieSceneSequencePlayer.OnFinished` _sequenceplayer `이벤트`))

(fn `StopSequence`
  (params (blend :type "Float (double-precision)"))
  (bind _currentactor (`self.CurrentActor`))
  (if (`KismetSystemLibrary.IsValid` _currentactor)
    (`MovieSceneSequencePlayer.Stop` (`LevelSequenceActor.SequencePlayer` _currentactor))
    (`self.OnFinishedSequence` blend)
    (else
      (`KismetSystemLibrary.PrintString` "시네마액터비어있음"))))

(fn `UserConstructionScript`)