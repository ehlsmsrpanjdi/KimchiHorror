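; Main player character with debug keys for a controller screen fade-in, a first/third-person camera toggle, and ragdoll death.
; The camera toggle adjusts the boom and mesh visibility, while PlayerDead enables mesh physics.
; DoubtBox overlaps forward to doubt handlers, and SetDoubtPPB scales post-process dirt mask, vignette and film grain from a doubt value.
; InteractionBox overlap events are empty, and a level-sequence transform-origin snippet is left unconnected.
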(event `Key|T`
  (params (Key :type "Key Structure"))
  (:`Pressed`
    (bind _asbp_third_person_player_controller (cast `/Game/Level/Stage_1Element/BP_ThirdPersonPlayerController` (`GameplayStatics.GetPlayerController` 0)))
    (`/Game/Level/Stage_1Element/BP_ThirdPersonPlayerController.FadeIn` _asbp_third_person_player_controller 5.0)))

(event `DebugOnce`
  (bind _cameraboom (`self.CameraBoom`))
  (set `SpringArmComponent.TargetArmLength` 0.0 _cameraboom)
  (set `SpringArmComponent.TargetOffset` (0.0 0.0 70.0) _cameraboom)
  (`SceneComponent.SetHiddenInGame` (`self.Mesh`) true false))

(event `Key|O`
  (params (Key :type "Key Structure"))
  (:`Pressed`
    (if (`self.IsThird`)
      (`self.DebugOnce`)
      (set `self.IsThird` false)
      (else
        (`self.DebugThird`)
        (set `self.IsThird` true)))))

(event `DebugThird`
  (bind _cameraboom (`self.CameraBoom`))
  (set `SpringArmComponent.TargetArmLength` 400.0 _cameraboom)
  (set `SpringArmComponent.TargetOffset` (0.0 0.0 0.0) _cameraboom)
  (`SceneComponent.SetHiddenInGame` (`self.Mesh`) false false))

(event `self.ReceiveBeginPlay`
  (`SceneComponent.SetHiddenInGame` (`self.InteractionBox`) false false)
  (`SceneComponent.SetHiddenInGame` (`self.DoubtBox`) false false))

(event `Key|L`
  (params (Key :type "Key Structure"))
  (:`Pressed`
    (`self.PlayerDead`)))

(event `self.InteractionBox.OnComponentBeginOverlap`
  (params (OverlappedComponent :type "PrimitiveComponent Object Reference") (OtherActor :type "Actor Object Reference") (OtherComp :type "PrimitiveComponent Object Reference") (OtherBodyIndex :type Integer) (bFromSweep :type Boolean) (SweepResult :type "HitResult Structure (by ref)")))

(event `PlayerDead`
  (`PrimitiveComponent.SetSimulatePhysics` (`self.Mesh`) true))

(event `self.ReceiveTick`
  (params (DeltaSeconds :type "Float (single-precision)")))

(event `self.InteractionBox.OnComponentEndOverlap`
  (params (OverlappedComponent :type "PrimitiveComponent Object Reference") (OtherActor :type "Actor Object Reference") (OtherComp :type "PrimitiveComponent Object Reference") (OtherBodyIndex :type Integer)))

(event `self.DoubtBox.OnComponentBeginOverlap`
  (params (OverlappedComponent :type "PrimitiveComponent Object Reference") (OtherActor :type "Actor Object Reference") (OtherComp :type "PrimitiveComponent Object Reference") (OtherBodyIndex :type Integer) (bFromSweep :type Boolean) (SweepResult :type "HitResult Structure (by ref)"))
  (`self.OnDoubtBoxBeginOverlap` OverlappedComponent OtherActor OtherComp OtherBodyIndex bFromSweep SweepResult))

(event `self.DoubtBox.OnComponentEndOverlap`
  (params (OverlappedComponent :type "PrimitiveComponent Object Reference") (OtherActor :type "Actor Object Reference") (OtherComp :type "PrimitiveComponent Object Reference") (OtherBodyIndex :type Integer))
  (`self.OnDoubtBoxEndOverlap` OverlappedComponent OtherActor OtherComp OtherBodyIndex))

(fn `SetDoubtPPB`
  (params (CurrentDoubt :type "Float (double-precision)"))
  (setmembers `PostProcessSettings` :`StructRef` (`PostProcessComponent.Settings` (`self.PostProcess`)) :`BloomDirtMaskIntensity` (/ CurrentDoubt 12.5) :`VignetteIntensity` (/ CurrentDoubt 100.0) :`FilmGrainIntensity` (/ CurrentDoubt 300.0)))

(fn `UserConstructionScript`)