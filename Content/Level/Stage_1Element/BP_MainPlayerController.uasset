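; BP_MainPlayerController is a player controller with a FadeIn event that runs a camera fade while locking player input.
; The event removes IMC_Default and disables input, starts the fade, waits out the Duration, then restores both.
; An IsFade flag blocks re-entry during the fade.
; The fade's target alpha is derived from Duration, so it varies with the fade length.
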(event `FadeIn`
  (params (Duration :type "Float (single-precision)"))
  (if (not (`self.IsFade`))
    (`EnhancedInputSubsystemInterface.RemoveMappingContext` (subsystem `EnhancedInputLocalPlayerSubsystem`) "/Game/Input/IMC_Default.IMC_Default" (struct))
    (set `self.IsFade` true)
    (`self.DisableInput` self)
    (`PlayerCameraManager.StartCameraFade` :`self` (`GameplayStatics.GetPlayerCameraManager` 0) :`ToAlpha` (* Duration 1.0) :`Duration` Duration)
    (`KismetSystemLibrary.Delay` Duration)
    (`self.EnableInput` self)
    (set `self.IsFade` false)
    (`EnhancedInputSubsystemInterface.AddMappingContext` (subsystem `EnhancedInputLocalPlayerSubsystem`) "/Game/Input/IMC_Default.IMC_Default" 0 (struct))))

(fn `UserConstructionScript`)