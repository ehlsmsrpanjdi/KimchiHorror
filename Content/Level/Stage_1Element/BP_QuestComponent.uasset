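; Quest component that advances the game's linear quest line and refreshes the player's goal display.
; ExecuteQuest validates the given quest line, looks up its data in BP_GameInstance, then stores the next quest ID as current.
; QuestUpdate pushes that quest's description to BP_MenuUI through the UI manager and shows a Korean "goal updated" popup.
; DebugEvent sets quest state without validation or UI update, printing the IDs.
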(event `self.ExecuteQuest`
  (params (_CurrentQuestLine :type Name))
  (bind _returnvalue (`self.CheckQuestLine` _CurrentQuestLine))
  (if _returnvalue
    (bind _asbp_game_instance (cast `/Game/BP/BP_GameInstance` (`GameplayStatics.GetGameInstance`)))
    (bind _returnvalue_2 (`C_GameInstance.GetQuestData` _asbp_game_instance _CurrentQuestLine))
    (bind _output_get (set `C_GameInstance.CurrentQuestName` (`.NextQuestID` (break `C_QuestDataTable` _returnvalue_2)) _asbp_game_instance))
    (`self.SetNextQuestLine` (`.NextQuestID` (break `C_QuestDataTable` _returnvalue_2)))
    (`KismetSystemLibrary.PrintString` (`KismetStringLibrary.Conv_NameToString` _output_get))
    (`self.QuestUpdate` (`.NextQuestID` (break `C_QuestDataTable` _returnvalue_2)))))

(event `DebugEvent`
  (bind _currentquestline (`self.CurrentQuestLine`))
  (bind _asbp_game_instance (cast `/Game/BP/BP_GameInstance` (`GameplayStatics.GetGameInstance`)))
  (bind _returnvalue (`C_GameInstance.GetQuestData` _asbp_game_instance _currentquestline))
  (set `C_GameInstance.CurrentQuestName` _currentquestline _asbp_game_instance)
  (`self.SetNextQuestLine` (`.NextQuestID` (break `C_QuestDataTable` _returnvalue)))
  (`KismetSystemLibrary.PrintString` (`KismetStringLibrary.Conv_NameToString` (break `C_QuestDataTable` _returnvalue)))
  (`KismetSystemLibrary.PrintString` (`KismetStringLibrary.Conv_NameToString` (`.NextQuestID` (break `C_QuestDataTable` _returnvalue)))))

(event `QuestUpdate`
  (params (NextQuestName :type Name))
  (bind _returnvalue (`C_UIManager.GetUIManager`))
  (bind _asbp_game_instance (cast `/Game/BP/BP_GameInstance` (`GameplayStatics.GetGameInstance`)))
  (bind _returnvalue_2 (`C_GameInstance.GetQuestData` _asbp_game_instance NextQuestName))
  (bind _returnvalue_3 (`C_UIManager.GetUI` _returnvalue "/Game/BP/UI/Common/Stash/BP_MenuUI.BP_MenuUI_C"))
  (bind _asbp_menu_ui (cast `/Game/BP/UI/Common/Stash/BP_MenuUI` _returnvalue_3))
  (`/Game/BP/UI/Common/Stash/BP_MenuUI.UpdateGoal` _asbp_menu_ui (`.QuestDescription` (break `C_QuestDataTable` _returnvalue_2)))
  (bind _returnvalue_4 (`C_UIManager.GetUI` _returnvalue "/Game/BP/UI/Common/Text/BP_PopUpMassage.BP_PopUpMassage_C"))
  (bind _asbp_pop_up_massage (cast `/Game/BP/UI/Common/Text/BP_PopUpMassage` _returnvalue_4))
  (`/Game/BP/UI/Common/Text/BP_PopUpMassage.CallPopUpMassage` _asbp_pop_up_massage "목표가 갱신되었습니다."))

(event `UpdateGoal`)