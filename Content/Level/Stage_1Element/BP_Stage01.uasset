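; Stage 1 controller Blueprint that sets up the stage UI and drives the in-game clock.
; BeginPlay creates the interaction message, dialog, menu and popup widgets through the UI manager, then passes the GameInstance's current day into SetHour.
; Tick feeds delta seconds, multiplied by 1000, into CaculateTime to advance time.
; Hour printing and doubt-setting nodes are left unwired.
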(event `self.ReceiveBeginPlay`
  (bind _returnvalue (`C_UIManager.GetUIManager`))
  (cast `/Game/BP/BP_GameInstance` (`GameplayStatics.GetGameInstance`))
  (`C_UIManager.CreateAndAddUI` _returnvalue "/Game/BP/UI/Common/Text/BP_InterMassage.BP_InterMassage_C")
  (`C_UIManager.CreateAndAddUI` _returnvalue "/Game/BP/UI/Common/Text/BP_Dialog.BP_Dialog_C")
  (`C_UIManager.CreateAndAddUI` _returnvalue "/Game/BP/UI/Common/Stash/BP_MenuUI.BP_MenuUI_C")
  (`C_UIManager.CreateAndAddUI` _returnvalue "/Game/BP/UI/Common/Text/BP_PopUpMassage.BP_PopUpMassage_C")
  (bind _asbp_game_instance (cast `/Game/BP/BP_GameInstance` (`GameplayStatics.GetGameInstance`)))
  (bind _output_get (set `self.dayCount` (`/Game/BP/BP_GameInstance.CurrentDay` _asbp_game_instance)))
  (`self.SetHour` _output_get))

(event `self.ReceiveTick`
  (params (DeltaSeconds :type "Float (single-precision)"))
  (`self.CaculateTime` (* DeltaSeconds 1000.0)))

(fn `UserConstructionScript`)