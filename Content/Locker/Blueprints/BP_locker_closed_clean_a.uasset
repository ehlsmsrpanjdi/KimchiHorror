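; Interactable locker that the player can hide in and climb back out of.
; OnInteract swings the door open on a timeline, then a looping timer glides the character to the hide or exit point, turning it to match.
; On arrival a second timeline closes the door and flips BoolIsHide.
; Movement is disabled on entry and restored on exit; while hidden, the locker is the player's CurrentInteractActor.
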(event `self.ReceiveBeginPlay`
  (bind _asbp_main_player (cast `/Game/Level/Stage_1Element/BP_MainPlayer` (`GameplayStatics.GetPlayerCharacter` 0)))
  (set `self.CharacterRef` _asbp_main_player))

(event `InteractionInterface.OnInteract`
  (params (Interactor :type "Actor Object Reference"))
  (bind _characterref (`self.CharacterRef`))
  (bind (_direction _alpha) (`Timeline|타임라인` :!via `PlayFromStart`)
    (:`Update`
      (`SceneComponent.K2_SetRelativeRotation` (`self.SM_locker_0001_door`) (`KismetMathLibrary.MakeRotator` 0.0 0.0 (`KismetMathLibrary.Lerp` 0.0 -140.0 _alpha)) false false))
    (:`Finished`
      (if (`self.bool IsHide`)
        (bind _returnvalue (`KismetSystemLibrary.K2_SetTimerDelegate` (delegate `MoveCharacter`) (`GameplayStatics.GetWorldDeltaSeconds`) true))
        (else
          (`self.SetActorEnableCollision` _characterref true)
          (`CharacterMovementComponent.DisableMovement` (`Character.CharacterMovement` _characterref))
          (bind _returnvalue_2 (`KismetSystemLibrary.K2_SetTimerDelegate` (delegate `MoveCharacter`) (`GameplayStatics.GetWorldDeltaSeconds`) true)))))))

(event `MoveCharacter`
  (bind _characterref (`self.CharacterRef`))
  (`self.K2_SetActorTransform` _characterref (`KismetMathLibrary.MakeTransform` (`KismetMathLibrary.VInterpTo_Constant` (`self.K2_GetActorLocation` _characterref) (`SceneComponent.K2_GetComponentLocation` (select `bool` (`self.bool IsHide`) :`false` (`self.PlayerPosition`) :`true` (`self.ExitPosition`) :!type "SceneComponent Object Reference")) (`GameplayStatics.GetWorldDeltaSeconds`) 100.0) (`KismetMathLibrary.Conv_VectorToRotator` (`KismetMathLibrary.VInterpTo_Constant` (`self.GetActorForwardVector` (`self.CharacterRef`)) (`SceneComponent.GetForwardVector` (select `bool` (`self.bool IsHide`) :`false` (`self.PlayerPosition`) :`true` (`self.ExitPosition`) :!type "SceneComponent Object Reference")) (`GameplayStatics.GetWorldDeltaSeconds`) 100.0))) false false)
  (if (== (`self.K2_GetActorLocation` (`self.CharacterRef`)) (`SceneComponent.K2_GetComponentLocation` (select `bool` (`self.bool IsHide`) :`false` (`self.PlayerPosition`) :`true` (`self.ExitPosition`) :!type "SceneComponent Object Reference")) :`ErrorTolerance` 0.01)
    (`KismetSystemLibrary.K2_ClearAndInvalidateTimerHandle` (stale `InteractionInterface.OnInteract` _returnvalue_2))
    (`KismetSystemLibrary.K2_ClearAndInvalidateTimerHandle` (stale `InteractionInterface.OnInteract` _returnvalue))
    (`self.FinishedHide`)))

(event `FinishedHide`
  (bind _characterref (`self.CharacterRef`))
  (bind (_direction _alpha) (`Timeline|타임라인_5` :!via `PlayFromStart`)
    (:`Update`
      (`SceneComponent.K2_SetRelativeRotation` (`self.SM_locker_0001_door`) (`KismetMathLibrary.MakeRotator` 0.0 0.0 (`KismetMathLibrary.Lerp` -140.0 0.0 _alpha)) false false))
    (:`Finished`
      (if (`self.bool IsHide`)
        (set `self.bool IsHide` false)
        (`self.SetActorEnableCollision` _characterref true)
        (`CharacterMovementComponent.SetMovementMode` (`Character.CharacterMovement` _characterref) "MOVE_Walking" 0)
        (else
          (set `self.bool IsHide` true)
          (set `HorrorProtoKimchiCharacter.CurrentInteractActor` self (`self.CharacterRef`)))))))

(fn `UserConstructionScript`)