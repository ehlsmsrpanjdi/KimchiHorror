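; BP_CameraMan is a camera operator actor that carries a CineCamera on its body mesh and has collision disabled.
; On BeginPlay it attaches the camera to the mesh's CameraSocket and sets the body to Idle.
; Interface events forward head tilt and body movement to BP_MaleEntityBodyAnim, so animation can move the socketed camera.
; GetCam exposes the CineCamera to other Blueprints.
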(event `self.ReceiveBeginPlay`
  (`parent.ReceiveBeginPlay`)
  (`SceneComponent.K2_AttachToComponent` (`self.CineCamera`) (`self.Mesh`) "CameraSocket" "KeepRelative" "KeepRelative" "KeepRelative" true)
  (`self.ISetBodyMove` "Idle")
  (`self.SetActorEnableCollision` false))

(event `/Game/BP/Stage1/InteractiveEntity/AnimIns/BPI_EntityMoveInter.ISetHeadTilting`
  (params (DesVector :type "Vector Structure") (RotateSpeed :type "Float (double-precision)"))
  (bind _asbp_male_entity_body_anim (cast `/Game/BP/Stage1/InteractiveEntity/AnimIns/Body/BP_MaleEntityBodyAnim` (`SkeletalMeshComponent.GetAnimInstance` (`self.Mesh`))))
  (`C_EntityAnimBase.LerfTiltHead` _asbp_male_entity_body_anim DesVector RotateSpeed))

(event `/Game/BP/Stage1/InteractiveEntity/AnimIns/BPI_EntityMoveInter.ISetBodyMove`
  (params (Move :type "C_EntityMoveEnum Enum" :default "Idle"))
  (bind _asbp_male_entity_body_anim (cast `/Game/BP/Stage1/InteractiveEntity/AnimIns/Body/BP_MaleEntityBodyAnim` (`SkeletalMeshComponent.GetAnimInstance` (`self.Mesh`)))
    (:`then`
      (`C_EntityAnimBase.SetBodyMove` _asbp_male_entity_body_anim Move))
    (:`CastFailed`
      (`KismetSystemLibrary.PrintString` "BodyMissing"))))

(fn `GetCam`
  (returns (CineCamera :type "CineCameraComponent Object Reference"))
  (return (`self.CineCamera`)))

(fn `UserConstructionScript`
  (`parent.UserConstructionScript`))