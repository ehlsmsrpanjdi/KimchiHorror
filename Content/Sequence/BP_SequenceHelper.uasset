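; BP_SequenceHelper plays cutscene level sequences through a CameraMan view target, moving input from the player to itself.
; RunSequence guards against replays and binds completion to FIN, which restores camera and input, notifies the quest component, fires a callback and optionally opens a level.
; Q skips through the same FIN path after stopping fade and blink UI.
; CallSubscript and FadeInOut drive dialog subtitles and screen fades via the UI manager.
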(event `self.ReceiveBeginPlay`
  (set `self.Player` (`GameplayStatics.GetPlayerCharacter` 0))
  (set `self.Controller` (`GameplayStatics.GetPlayerController` 0)))

(event `self.RunSequence`
  (bind _cameraman (`self.CameraMan`))
  (if (not (`self.IsPlaying`))
    (set `self.IsPlaying` true)
    (`/Game/Sequence/BP_CameraMan.SetCol` _cameraman true)
    (`SceneComponent.SetHiddenInGame` (`Character.Mesh` _cameraman) false false)
    (`self.StartSequence` _cameraman (`self.CurrentActor`) (delegate `OnSceneFinished`))))

(event `OnSceneFinished`
  (`self.FIN`))

(event `FIN`
  (bind _returnvalue (`C_UIManager.GetUIManager`))
  (bind _level (`self.Level`))
  (`self.OnFinishedSequence` (`self.Blend`))
  (`SceneComponent.SetHiddenInGame` (`Character.Mesh` (`self.CameraMan`)) true false)
  (bind _asbp_main_player (cast `/Game/Level/Stage_1Element/BP_MainPlayer` (`self.Player`)))
  (`HorrorProtoKimchiCharacter.NotifyQuestComponent` _asbp_main_player (`self.QuestName`))
  (set `self.IsPlaying` false)
  (`self.ExecuteCallback`)
  (if (`KismetSystemLibrary.IsValidSoftObjectReference` _level)
    (`GameplayStatics.OpenLevelBySoftObjectPtr` _level)
    (`/Game/Sequence/BP_CameraMan.SetCol` (`self.CameraMan`) false)
    (bind _returnvalue_2 (`C_UIManager.GetUI` _returnvalue "/Game/BP/UI/Common/Text/BP_Dialog.BP_Dialog_C"))
    (bind _asbp_dialog (cast `/Game/BP/UI/Common/Text/BP_Dialog` _returnvalue_2))
    (bind _returnvalue_3 (`C_UIManager.GetUI` _returnvalue "/Game/BP/UI/Common/FunctionUI/BP_FadeUI.BP_FadeUI_C"))
    (bind _asbp_fade_ui (cast `/Game/BP/UI/Common/FunctionUI/BP_FadeUI` _returnvalue_3))
    (`UserWidget.StopAllAnimations` _asbp_dialog)
    (`UserWidget.StopAllAnimations` _asbp_fade_ui)
    (set `Widget.Visibility` "Collapsed" _asbp_dialog)
    (set `Widget.Visibility` "Visible" _asbp_fade_ui)))

(event `CallSubscript`
  (params (SequenceNum :type "/Game/Sequence/BP_ScriptEnum Enum" :default "NewEnumerator0") (ScriptIndex :type Integer) (Time :type "Float (double-precision)"))
  (bind _returnvalue (`C_UIManager.GetUIManager`))
  (bind _script (`/Game/Sequence/Script/BP_ScriptContainer.FindScript` (`self.Scripts`) SequenceNum ScriptIndex))
  (bind _returnvalue_2 (`C_UIManager.GetUI` _returnvalue "/Game/BP/UI/Common/Text/BP_Dialog.BP_Dialog_C"))
  (`C_UIManager.OnUI` _returnvalue "/Game/BP/UI/Common/Text/BP_Dialog.BP_Dialog_C")
  (bind _asbp_dialog (cast `/Game/BP/UI/Common/Text/BP_Dialog` _returnvalue_2)
    (:`then`
      (`/Game/BP/UI/Common/Text/BP_Dialog.CallDialog` _asbp_dialog _script Time))
    (:`CastFailed`
      (`KismetSystemLibrary.PrintString` "fuck"))))

(event `FadeInOut`
  (params (`On/Off` :type Boolean))
  (bind _returnvalue (`C_UIManager.GetUIManager`))
  (bind _returnvalue_2 (`C_UIManager.GetUI` _returnvalue "/Game/BP/UI/Common/FunctionUI/BP_FadeUI.BP_FadeUI_C"))
  (`C_UIManager.OnUI` _returnvalue "/Game/BP/UI/Common/FunctionUI/BP_FadeUI.BP_FadeUI_C")
  (bind _asbp_fade_ui (cast `/Game/BP/UI/Common/FunctionUI/BP_FadeUI` _returnvalue_2)
    (:`then`
      (if `On/Off`
        (`/Game/BP/UI/Common/FunctionUI/BP_FadeUI.CallFadeOut` _asbp_fade_ui)
        (else
          (`/Game/BP/UI/Common/FunctionUI/BP_FadeUI.CallFadein` _asbp_fade_ui))))
    (:`CastFailed`
      (`KismetSystemLibrary.PrintString` "너냐"))))

(event `나중에 시퀀스 끄는 버튼이 호출할 이벤트 함수`)

(event `Key|Q`
  (params (Key :type "Key Structure"))
  (bind _returnvalue (`C_UIManager.GetUIManager`))
  (bind _returnvalue_2 (`C_UIManager.GetUIManager`))
  (:`Pressed`
    (bind _returnvalue_3 (`C_UIManager.GetUI` _returnvalue_2 "/Game/BP/UI/Common/FunctionUI/BP_FadeUI.BP_FadeUI_C"))
    (`C_UIManager.OnUI` _returnvalue_2 "/Game/BP/UI/Common/FunctionUI/BP_FadeUI.BP_FadeUI_C")
    (bind _asbp_fade_ui (cast `/Game/BP/UI/Common/FunctionUI/BP_FadeUI` _returnvalue_3))
    (bind _returnvalue_4 (`C_UIManager.GetUI` _returnvalue "/Game/BP/UI/Common/FunctionUI/BP_BlinkEye.BP_BlinkEye_C"))
    (`C_UIManager.OnUI` _returnvalue "/Game/BP/UI/Common/FunctionUI/BP_BlinkEye.BP_BlinkEye_C")
    (bind _asbp_blink_eye (cast `/Game/BP/UI/Common/FunctionUI/BP_BlinkEye` _returnvalue_4)
      (:`then`
        (`UserWidget.StopAllAnimations` _asbp_blink_eye)
        (`UserWidget.StopAllAnimations` _asbp_fade_ui)
        (`Widget.SetVisibility` _asbp_blink_eye "Collapsed")
        (`self.StopSequence`)
        (`self.FIN`))
      (:`CastFailed`
        (`KismetSystemLibrary.PrintString` "여기야?")))))

(fn `DoubtInsesity`
  (params (Doubt :type "Float (double-precision)") (post :type "PostProcessVolume Object Reference")))

(fn `OnFinishedSequence`
  (params (Blendtime :type "Float (double-precision)"))
  (bind _player (`self.Player`))
  (bind _controller (`self.Controller`))
  (`self.DisableInput` _controller)
  (`self.EnableInput` _player _controller)
  (`PlayerController.SetViewTargetWithBlend` _controller _player Blendtime "VTBlend_Linear" 0.0 false))

(fn `StartSequence`
  (params (Camera :type "/Game/Sequence/BP_CameraMan Object Reference") (SequenceActor :type "LevelSequenceActor Object Reference") (`이벤트` :type "Delegate (by ref)") (BlendTime :type "Float (double-precision)"))
  (bind _sequenceplayer (`LevelSequenceActor.SequencePlayer` SequenceActor))
  (bind _controller (`self.Controller`))
  (set `self.Blend` BlendTime)
  (`self.EnableInput` _controller)
  (`PlayerController.SetViewTargetWithBlend` _controller Camera 0.0 "VTBlend_Linear" 0.0 false)
  (`self.DisableInput` (`self.Player`) _controller)
  (`MovieSceneSequencePlayer.Play` _sequenceplayer)
  (add `MovieSceneSequencePlayer.OnFinished` _sequenceplayer `이벤트`))

(fn `StopSequence`
  (bind _currentactor (`self.CurrentActor`))
  (if (`KismetSystemLibrary.IsValid` _currentactor)
    (`MovieSceneSequencePlayer.Stop` (`LevelSequenceActor.SequencePlayer` _currentactor))
    (else
      (`KismetSystemLibrary.PrintString` "시네마액터비어있음"))))

(fn `UserConstructionScript`)