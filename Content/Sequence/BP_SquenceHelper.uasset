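; Sequence helper actor that plays a cinematic Level Sequence and hands control back to the player when it ends.
; RunSequence guards against re-entry, switches the view to a camera, moves input from the player to this actor, then plays the sequence.
; Finishing or pressing Q to skip restores view and input, notifies BP_MainPlayer's quest component by quest name, and opens the next level if one is set.
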(event `self.ReceiveBeginPlay`
  (set `self.Player` (`GameplayStatics.GetPlayerCharacter` 0))
  (set `self.Controller` (`GameplayStatics.GetPlayerController` 0)))

(event `RunSequence`
  (if (not (`self.IsPlaying`))
    (set `self.IsPlaying` true)
    (`self.StartSequence` (`self.Camera`) (`self.CurrentActor`) (delegate `OnSceneFinished`))))

(event `FIN`
  (bind _level (`self.Level`))
  (`self.OnFinishedSequence` (`self.Blend`))
  (bind _asbp_main_player (cast `/Game/Level/Stage_1Element/BP_MainPlayer` (`GameplayStatics.GetPlayerPawn` 0)))
  (`HorrorProtoKimchiCharacter.NotifyQuestComponent` _asbp_main_player (`self.QuestName`))
  (set `self.IsPlaying` false)
  (if (`KismetSystemLibrary.IsValidSoftObjectReference` _level)
    (`GameplayStatics.OpenLevelBySoftObjectPtr` _level)))

(event `OnSceneFinished`
  (`self.FIN`))

(event `Key|Q`
  (params (Key :type "Key Structure"))
  (:`Pressed`
    (`self.StopSequence`)
    (`self.FIN`)))

(fn `DoubtInsesity`
  (params (Doubt :type "Float (double-precision)") (post :type "PostProcessVolume Object Reference")))

(fn `OnFinishedSequence`
  (params (Blendtime :type "Float (double-precision)"))
  (bind _player (`self.Player`))
  (bind _controller (`self.Controller`))
  (`self.DisableInput` _controller)
  (`self.EnableInput` _player _controller)
  (`PlayerController.SetViewTargetWithBlend` _controller _player Blendtime "VTBlend_Linear" 0.0 false))

(fn `StartSequence`
  (params (Camera :type "CineCameraActor Object Reference") (SequenceActor :type "LevelSequenceActor Object Reference") (`이벤트` :type "Delegate (by ref)") (BlendTime :type "Float (double-precision)"))
  (bind _sequenceplayer (`LevelSequenceActor.SequencePlayer` SequenceActor))
  (bind _controller (`self.Controller`))
  (set `self.Blend` BlendTime)
  (`self.EnableInput` _controller)
  (`PlayerController.SetViewTargetWithBlend` _controller Camera 0.0 "VTBlend_Linear" 0.0 false)
  (`self.DisableInput` (`self.Player`) _controller)
  (`MovieSceneSequencePlayer.Play` _sequenceplayer)
  (add `MovieSceneSequencePlayer.OnFinished` _sequenceplayer `이벤트`))

(fn `StopSequence`
  (bind _currentactor (`self.CurrentActor`))
  (if (`KismetSystemLibrary.IsValid` _currentactor)
    (`MovieSceneSequencePlayer.Stop` (`LevelSequenceActor.SequencePlayer` _currentactor))
    (else
      (`KismetSystemLibrary.PrintString` "시네마액터비어있음"))))

(fn `UserConstructionScript`)