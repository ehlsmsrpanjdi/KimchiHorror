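; BP_DeadBody is a modular dead-body character used under the Hide sequence folder.
; Its construction script makes the clothing, hip, helmet, arm and pants meshes follow the main Mesh through leader pose.
; BeginPlay runs the parent logic, then stores the Face component in MyFace.
; The face-move, head-tilt and body-move interface events are empty here.
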(event `self.ISetFaceMove`
  (params (Pose :type "C_FacePoseEnum Enum" :default "Idle") (Mood :type "C_FaceMoodEnum Enum" :default "Normal") (Interval :type "Float (double-precision)")))

(event `self.ISetHeadTilting`
  (params (DesVector :type "Vector Structure") (RotateSpeed :type "Float (double-precision)")))

(event `self.ReceiveBeginPlay`
  (`parent.ReceiveBeginPlay`)
  (set `self.MyFace` (`self.Face`)))

(event `self.ISetBodyMove`
  (params (Move :type "C_EntityMoveEnum Enum" :default "Idle")))

(fn `UserConstructionScript`
  (`SkinnedMeshComponent.SetLeaderPoseComponent` (`self.Clothes`) (`self.Mesh`) false false)
  (`SkinnedMeshComponent.SetLeaderPoseComponent` (`self.Hip_Left`) (`self.Mesh`) false false)
  (`SkinnedMeshComponent.SetLeaderPoseComponent` (`self.Helmet_Drops`) (`self.Mesh`) false false)
  (`SkinnedMeshComponent.SetLeaderPoseComponent` (`self.Arms`) (`self.Mesh`) false false)
  (`SkinnedMeshComponent.SetLeaderPoseComponent` (`self.Pants`) (`self.Mesh`) false false))