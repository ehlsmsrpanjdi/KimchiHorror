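; BP_ScriptContainer is a data-holder actor that stores dialogue script lines for the game's sequences and serves them by sequence and index.
; FindArray switches on a sequence enum to pick one of twelve numbered arrays or a None fallback array.
; FindScript returns the indexed entry from that array, printing a Korean warning instead when the index exceeds its length.
; The event graph and construction script contain no logic.
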(fn `FindArray`
  (params (Sequence :type "/Game/Sequence/BP_ScriptEnum Enum" :default "NewEnumerator0"))
  (returns (Text :type "Array of Text"))
  (switch `/Game/Sequence/BP_ScriptEnum` Sequence
    (:`NewEnumerator0`
      (return (`self.Squence1`)))
    (:`NewEnumerator1`
      (return (`self.Squence2`)))
    (:`NewEnumerator2`
      (return (`self.Squence3`)))
    (:`NewEnumerator3`
      (return (`self.Squence4`)))
    (:`NewEnumerator4`
      (return (`self.Squence5`)))
    (:`NewEnumerator5`
      (return (`self.Squence6`)))
    (:`NewEnumerator6`
      (return (`self.Squence7`)))
    (:`NewEnumerator7`
      (return (`self.Squence8`)))
    (:`NewEnumerator8`
      (return (`self.Squence9`)))
    (:`NewEnumerator9`
      (return (`self.Squence10`)))
    (:`NewEnumerator10`
      (return (`self.Squence11`)))
    (:`NewEnumerator11`
      (return (`self.Squence12`)))
    (:`NewEnumerator12`
      (return (`self.NoneSequence`)))))

(fn `FindScript`
  (params (Sequence :type "/Game/Sequence/BP_ScriptEnum Enum" :default "NewEnumerator0") (Index :type Integer))
  (returns (Script :type Text))
  (bind _text (`self.FindArray` Sequence))
  (if (>= Index (`KismetArrayLibrary.Array_Length` _text))
    (`KismetSystemLibrary.PrintString` "인덱스 초과 언리얼 터진다 대사 인덱스 다시 확인해라")
    (else
      (return (`|GetArrayItem` _text Index)))))

(fn `UserConstructionScript`)